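; Main menu pawn that doubles as a three-lane dodge minigame, where the player's lane also selects Start, About or Quit.
; Any key starts looping timers that launch and move pooled enemies, speeding up after dodge thresholds.
; Overlaps recycle passed enemies or reset the run on a hit, keeping a top score.
; Enter or clicks on 3D boxes trigger blinking text and the option; Start saves fresh equipment data before opening TestMap.
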(event `self.ReceiveBeginPlay`
  (bind _returnvalue (`GameplayStatics.GetPlayerController` 0))
  (`|ExecutionSequence`
    (:`then_0`
      (`EnhancedInputSubsystemInterface.AddMappingContext` (pcsubsystem `EnhancedInputLocalPlayerSubsystem` (`GameplayStatics.GetPlayerController` 0)) "/Game/Input/IMC_Default.IMC_Default" 0 (struct))
      (set `self.PlayerLocation` (`|MakeArray` (`self.Sphere`) (`self.Sphere1`) (`self.StaticMesh`)))
      (set `self.EnemySpawnLocation` (`|MakeArray` (`self.Sphere3`) (`self.StaticMesh1`) (`self.Sphere2`)))
      (set `self.TextLocation` (`|MakeArray` (`self.TextRender`) (`self.TextRender1`) (`self.TextRender2`)))
      (`self.SetPlayerLocation`)
      (set `self.GameIsStart` false))
    (:`then_1`
      (for _ (range 21)
        (bind _returnvalue_2 (`|SpawnActorFromClass` "/Game/MainMenu/BP_MM_Enemy.BP_MM_Enemy_C" (`KismetMathLibrary.MakeTransform` (0.0 0.0 0.0)) "Undefined" "MultiplyWithRoot" null null))
        (`KismetArrayLibrary.Array_Add` (`self.EnemyArray`) _returnvalue_2)
        (`KismetArrayLibrary.Array_Add` (`Actor.Tags` _returnvalue_2) "Enemy")))
    (:`then_2`
      (bind _output_get (set `self.CurrentScore` 0.0))
      (set `self.TopScore` _output_get)
      (set `self.Rate` 0.3))
    (:`then_3`
      (`self.Started Guide`)
      (`self.UpdateScore` true))
    (:`then_4`
      (set `PlayerController.bShowMouseCursor` true _returnvalue)
      (`WidgetBlueprintLibrary.SetInputMode_GameAndUIEx` _returnvalue null)
      (set `PlayerController.bEnableClickEvents` true _returnvalue)
      (set `PlayerController.bEnableMouseOverEvents` true _returnvalue)
      (`self.SetSubText`)
      (set `self.canPlay` true))
    (:`then_5`
      (bind _returnvalue_3 (`|CreateWidget` "/Game/UI/W_About.W_About_C"))
      (bind _output_get_2 (set `self.AboutUI` _returnvalue_3))
      (`Widget.SetVisibility` _output_get_2 "Hidden")
      (`UserWidget.AddToViewport` _output_get_2 0))))

(event `Key|AnyKey`
  (params (Key :type "Key Structure"))
  ; 按下任意键开始游戏哦
  (:`Pressed`
    (if (not (`self.GameIsStart`))
      (`self.StartGame`)
      (`KismetSystemLibrary.K2_PauseTimerHandle` (`self.GuideTimer`))
      (`SceneComponent.SetVisibility` (`self.TextRender9`) false false)
      (`AudioComponent.Play` (`self.Audio`) 0.0))))

(event `EnhancedInput|/Game/Input/IA_Move`
  (params (ActionValue :type Boolean) (ElapsedSeconds :type "Float (double-precision)") (TriggeredSeconds :type "Float (double-precision)") (InputAction :type "InputAction Object Reference" :default "/Game/Input/IA_Move.IA_Move"))
  (bind _returnvalue (- (`self.RoadIndex`) 1))
  ; 移动赛车道/选择选项
  (:`Started`
    (if (`self.canPlay`)
      (if (<= _returnvalue 0)
        (set `self.RoadIndex` 0)
        (else
          (set `self.RoadIndex` _returnvalue)))
      (`self.SetPlayerLocation` :!label _label))))

(event `StartGame`
  ; 开始主界面游戏
  ;; 随机抽取一个敌人，然后放至随机spawn点，修改布尔值让敌人可以跑
  (set `self.GameIsStart` true)
  (bind _returnvalue (`KismetSystemLibrary.K2_SetTimerDelegate` (delegate `EnemyRunning`) (* (`self.Rate`) 4.0) true))
  (set `self.SpawnEnemyTimer` _returnvalue)
  ;; 所有可以跑的敌人一起跑
  (bind _returnvalue_2 (`KismetSystemLibrary.K2_SetTimerDelegate` (delegate `MovingEnemy`) (`self.Rate`) true))
  (set `self.EnemyMovingTimer` _returnvalue_2))

(event `UpdateScore`
  (params (`isOver?` :type Boolean))
  (bind _textrender6 (`self.TextRender6`))
  (bind _currentscore (`self.CurrentScore`))
  ; 更新UI分数
  (if `isOver?`
    (`TextRenderComponent.K2_SetText` _textrender6 (`KismetTextLibrary.Conv_StringToText` "0"))
    (if (>= _currentscore (`self.TopScore`))
      (bind _output_get (set `self.TopScore` _currentscore))
      (set `self.CurrentScore` 0.0)
      (`TextRenderComponent.K2_SetText` (`self.TextRender5`) (`KismetTextLibrary.Conv_DoubleToText` _output_get "HalfToEven")))
    (else
      (`TextRenderComponent.K2_SetText` _textrender6 (`KismetTextLibrary.Conv_DoubleToText` (`self.CurrentScore`) "HalfToEven")))))

(event `SetPlayerLocation`
  (bind _textrender8 (`self.TextRender8`))
  (bind _roadindex (`self.RoadIndex`))
  (bind _textrender7 (`self.TextRender7`))
  ; 设置玩家位置
  (`self.SetSubText`)
  (`SceneComponent.K2_SetWorldLocation` (`self.Capsule`) (`SceneComponent.K2_GetComponentLocation` (`|GetArrayItem` (`self.PlayerLocation`) (`self.RoadIndex`))) false false)
  (`|ExecutionSequence`
    (:`then_0`
      (if (<= _roadindex 0)
        (`SceneComponent.SetVisibility` _textrender7 false false)
        (else
          (`SceneComponent.SetVisibility` _textrender7 true false))))
    (:`then_1`
      (if (>= _roadindex 2)
        (`SceneComponent.SetVisibility` _textrender8 false false)
        (else
          (`SceneComponent.SetVisibility` _textrender8 true false))))))

(event `EnhancedInput|/Game/Input/IA_Break`
  (params (ActionValue :type Boolean) (ElapsedSeconds :type "Float (double-precision)") (TriggeredSeconds :type "Float (double-precision)") (InputAction :type "InputAction Object Reference" :default "/Game/Input/IA_Break.IA_Break"))
  (bind _returnvalue (+ (`self.RoadIndex`) 1))
  ; 移动赛车道/选择选项
  (:`Started`
    (if (`self.canPlay`)
      (if (>= _returnvalue 2)
        (set `self.RoadIndex` 2)
        (goto _label)
        (else
          (set `self.RoadIndex` _returnvalue)
          (goto _label))))))

(event `EnemyRunning`
  ; 开始主界面游戏
  ;; 随机抽取一个敌人，然后放至随机spawn点，修改布尔值让敌人可以跑
  (bind _output_get (set `self.whichEnemy` (`KismetArrayLibrary.Array_Random` (`self.EnemyArray`))))
  (if (`/Game/MainMenu/BP_MM_Enemy.isMoving` _output_get)
    (`self.EnemyRunning`)
    (else
      (`self.K2_SetActorLocation` _output_get (`SceneComponent.K2_GetComponentLocation` (`KismetArrayLibrary.Array_Random` (`self.EnemySpawnLocation`))) false false)
      (set `/Game/MainMenu/BP_MM_Enemy.isMoving` true _output_get))))

(event `MovingEnemy`
  ; 开始主界面游戏
  ;; 所有可以跑的敌人一起跑
  (set `self.CurrentScore` (+ (`self.CurrentScore`) 1.0))
  (for _array_element (`self.EnemyArray`)
    (if (`/Game/MainMenu/BP_MM_Enemy.isMoving` _array_element)
      (bind (_returnvalue_x _returnvalue_y _returnvalue_z) (`KismetMathLibrary.BreakVector` (`self.K2_GetActorLocation` _array_element)))
      (`self.K2_SetActorLocation` _array_element (`KismetMathLibrary.MakeVector` _returnvalue_x (- _returnvalue_y 200.0) _returnvalue_z) false false)))
  (`self.UpdateScore` false))

(event `self.Capsule.OnComponentBeginOverlap`
  (params (OverlappedComponent :type "PrimitiveComponent Object Reference") (OtherActor :type "Actor Object Reference") (OtherComp :type "PrimitiveComponent Object Reference") (OtherBodyIndex :type Integer) (bFromSweep :type Boolean) (SweepResult :type "HitResult Structure (by ref)"))
  ; 撞到敌人，玩家死亡
  (if (`self.ActorHasTag` OtherActor "Enemy")
    (`self.PlayerIsDie`)))

(event `self.Box.OnComponentBeginOverlap`
  (params (OverlappedComponent :type "PrimitiveComponent Object Reference") (OtherActor :type "Actor Object Reference") (OtherComp :type "PrimitiveComponent Object Reference") (OtherBodyIndex :type Integer) (bFromSweep :type Boolean) (SweepResult :type "HitResult Structure (by ref)"))
  ; 当敌人到最后面的时候，不让跑
  (if (`self.ActorHasTag` OtherActor "Enemy")
    (`self.K2_SetActorLocation` OtherActor (0.0 0.0 0.0) false false)
    (bind _asbp_mm_enemy (cast `/Game/MainMenu/BP_MM_Enemy` OtherActor))
    (set `/Game/MainMenu/BP_MM_Enemy.isMoving` false _asbp_mm_enemy)
    (set `self.KillEnemyIndex` (+ (`self.KillEnemyIndex`) 1))
    (`self.CheckSpeed`)))

(event `PlayerIsDie`
  (`AudioComponent.Stop` (`self.Audio`))
  (`GameplayStatics.PlaySound2D` "/Game/Art/Voice/freesound_community-videogame-death-sound-43894.freesound_community-videogame-death-sound-43894" 1.0 1.0 0.0 null null)
  ; 玩家死亡
  (`self.ResetValue`)
  (`KismetSystemLibrary.PrintString` "Die")
  (`KismetSystemLibrary.K2_PauseTimerHandle` (`self.EnemyMovingTimer`))
  (`KismetSystemLibrary.K2_PauseTimerHandle` (`self.SpawnEnemyTimer`))
  (for _array_element (`self.EnemyArray`)
    (`self.K2_SetActorLocation` _array_element (0.0 0.0 0.0) false false)
    (set `/Game/MainMenu/BP_MM_Enemy.isMoving` false _array_element))
  (`self.Started Guide`)
  (`self.UpdateScore` true)
  (set `self.KillEnemyIndex` 0)
  (set `self.Rate` 0.3)
  (`KismetSystemLibrary.Delay` 0.5)
  (set `self.GameIsStart` false))

(event `Started Guide`
  (bind _returnvalue (`KismetSystemLibrary.K2_SetTimerDelegate` (delegate `Getting started guide`) 0.5 true))
  (set `self.GuideTimer` _returnvalue))

(event `CheckSpeed`
  (bind _killenemyindex (`self.KillEnemyIndex`))
  ; 修改速度（根据躲避的敌人数量
  (if (>= _killenemyindex 25)
    (`/Engine/EditorBlueprintResources/StandardMacros.DoOnce` false :!label _label_2
      (:`Completed`
        (set `self.Rate` (- (`self.Rate`) 0.1) :!label _label_3)
        (`self.StartGame`)))
    (elif (>= _killenemyindex 10)
      (`/Engine/EditorBlueprintResources/StandardMacros.DoOnce` false :!label _label_4
        (:`Completed`
          (goto _label_3))))))

(event `Key|Enter`
  (params (Key :type "Key Structure"))
  (bind _roadindex (`self.RoadIndex`))
  ; 点enter，查看是哪个按钮
  (:`Pressed`
    (if (`self.canPlay`)
      (`self.ShiningText` (`|GetArrayItem` (`self.TextLocation`) _roadindex))
      (if (== _roadindex 0)
        (`self.StartRealGame`)
        (elif (== _roadindex 1)
          (`self.CheckAbout`)
          (elif (== _roadindex 2)
            (`self.QuitThisGame`)))))))

(event `Getting started guide`
  (bind _textrender9 (`self.TextRender9`))
  (`/Engine/EditorBlueprintResources/StandardMacros.FlipFlop`
    (:`A`
      (`SceneComponent.SetVisibility` _textrender9 true false))
    (:`B`
      (`SceneComponent.SetVisibility` _textrender9 false false))))

(event `ResetValue`
  ; 修改速度（根据躲避的敌人数量
  (`|ExecutionSequence`
    (:`then_0`
      (goto _label_2 :!via `Reset`))
    (:`then_1`
      (goto _label_4 :!via `Reset`))))

(event `StartRealGame`
  (bind _returnvalue (`GameplayStatics.GetGameInstance`))
  ; 开启游戏
  (`GameplayStatics.PlaySound2D` "/Game/Art/Voice/freesound_community-gameboy-pluck-41265.freesound_community-gameboy-pluck-41265" 1.0 1.0 0.0 null null)
  (`PrimitiveComponent.SetCollisionEnabled` (`self.Box5`) "QueryOnly")
  (set `self.canPlay` false)
  (bind _savegamedata (message `/Game/Blueprint/SaveAndLoad/Utilities/BPI_SaveGame.GetGameData` _returnvalue))
  (`/Engine/EditorBlueprintResources/StandardMacros.IsValid` _savegamedata
    (:`Is Valid`
      (message `/Game/Blueprint/SaveAndLoad/Utilities/BPI_SaveGame.SaveEquipData` _returnvalue (make `/Game/Blueprint/SaveAndLoad/Utilities/S_SaveAndLoad_Equip` 0 false true 0.0 (`|MakeMap`) (`|MakeMap`) (`|MakeMap`)) false))
    (:`Is Not Valid`
      _))
  (`KismetSystemLibrary.Delay` 1.0)
  (`GameplayStatics.OpenLevelBySoftObjectPtr` "/Game/Map/TestMap.TestMap"))

(event `self.Box2.OnClicked`
  (params (TouchedComponent :type "PrimitiveComponent Object Reference") (ButtonPressed :type "Key Structure"))
  ; 按钮1
  (`self.ShiningText` (`|GetArrayItem` (`self.TextLocation`)))
  (`self.StartRealGame`))

(event `self.Box2.OnBeginCursorOver`
  (params (TouchedComponent :type "PrimitiveComponent Object Reference"))
  ; 按钮1
  (`self.SetSubText(Mouse'` 0))

(event `self.Box2.OnEndCursorOver`
  (params (TouchedComponent :type "PrimitiveComponent Object Reference"))
  ; 按钮1
  (`self.SetSubText`))

(event `self.Box3.OnBeginCursorOver`
  (params (TouchedComponent :type "PrimitiveComponent Object Reference"))
  ; 按钮2
  (`self.SetSubText(Mouse'` 1))

(event `QuitThisGame`
  ; 退出游戏
  (`GameplayStatics.PlaySound2D` "/Game/Art/Voice/freesound_community-gameboy-pluck-41265.freesound_community-gameboy-pluck-41265" 1.0 1.0 0.0 null null)
  (`PrimitiveComponent.SetCollisionEnabled` (`self.Box5`) "QueryOnly")
  (set `self.canPlay` false)
  (`KismetSystemLibrary.Delay` 1.0)
  (`KismetSystemLibrary.QuitGame` null "Quit"))

(event `SetSubText`
  ; 设置提示文本
  (`TextRenderComponent.K2_SetText` (`self.TextRender10`) (`|GetArrayItem` (`self.TextIndex`) (`self.RoadIndex`))))

(event `self.Box3.OnEndCursorOver`
  (params (TouchedComponent :type "PrimitiveComponent Object Reference"))
  ; 按钮2
  (`self.SetSubText`))

(event `self.Box3.OnClicked`
  (params (TouchedComponent :type "PrimitiveComponent Object Reference") (ButtonPressed :type "Key Structure"))
  ; 按钮2
  (`self.ShiningText` (`|GetArrayItem` (`self.TextLocation`) 1))
  (`self.CheckAbout`))

(event `CheckAbout`
  (`GameplayStatics.PlaySound2D` "/Game/Art/Voice/freesound_community-gameboy-pluck-41265.freesound_community-gameboy-pluck-41265" 1.0 1.0 0.0 null null)
  (`Widget.SetVisibility` (`self.AboutUI`) "Visible"))

(event `SetSubText(Mouse'`
  (params (index :type Integer))
  ; 设置提示文本
  (`TextRenderComponent.K2_SetText` (`self.TextRender10`) (`|GetArrayItem` (`self.TextIndex_0`) index)))

(event `ShiningText`
  (params (whichText :type "SceneComponent Object Reference"))
  ; 文本闪烁
  (for _array_element (`self.TextLocation`)
    (`SceneComponent.SetVisibility` _array_element true false)
    (set `self.TextShowIndex` 0)
    (bind _returnvalue (`KismetSystemLibrary.K2_SetTimerDelegate` (delegate `SetTextVisibility`) 0.1 true))))

(event `self.Box4.OnBeginCursorOver`
  (params (TouchedComponent :type "PrimitiveComponent Object Reference"))
  ; 按钮3
  (`self.SetSubText(Mouse'` 2))

(event `SetTextVisibility`
  (bind _returnvalue (+ (`self.TextShowIndex`) 1))
  ; 文本闪烁
  (if (>= _returnvalue 8)
    (`SceneComponent.SetVisibility` (stale `ShiningText` whichText) true false)
    (`KismetSystemLibrary.K2_PauseTimerHandle` (stale `ShiningText` _returnvalue))
    (else
      (set `self.TextShowIndex` _returnvalue)
      (`/Engine/EditorBlueprintResources/StandardMacros.FlipFlop`
        (:`A`
          (`SceneComponent.SetVisibility` (stale `ShiningText` whichText) false false))
        (:`B`
          (`SceneComponent.SetVisibility` (stale `ShiningText` whichText) true false))))))

(event `self.Box4.OnEndCursorOver`
  (params (TouchedComponent :type "PrimitiveComponent Object Reference"))
  ; 按钮3
  (`self.SetSubText`))

(event `self.Box4.OnClicked`
  (params (TouchedComponent :type "PrimitiveComponent Object Reference") (ButtonPressed :type "Key Structure"))
  ; 按钮3
  (`self.ShiningText` (`|GetArrayItem` (`self.TextLocation`) 2))
  (`self.QuitThisGame`))

(fn `UserConstructionScript`)