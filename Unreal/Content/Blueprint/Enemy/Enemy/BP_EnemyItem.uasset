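; BP_EnemyItem is the weapon loot dropped when an enemy dies, collected by the motorcycle character.
; RandomWeapon picks a random weapon type, places the physics cube and launches it along actor forward with random scatter.
; On sphere overlap with the player's capsule, it awards score, plays a sound and increments the weapon's count in the WeaponInBag map.
; The collected item is moved out of the way rather than destroyed.
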(event `RandomWeapon`
  (params (Location :type "Vector Structure") (Rotation :type "Rotator Structure"))
  (bind _cube (`self.Cube`))
  ; 敌人死亡后，爆装备，随机抽取武器属性
  (set `self.whichWeapon` (cast `/Game/Blueprint/Equipment/CubeWeapon/Utilities/E_CubeWeaponType` (`KismetMathLibrary.Conv_IntToByte` (`KismetMathLibrary.RandomIntegerInRange` 3 (- (enumcount `/Game/Blueprint/Equipment/CubeWeapon/Utilities/E_CubeWeaponType`) 1)))))
  (`SceneComponent.K2_SetWorldLocationAndRotation` _cube Location Rotation false true)
  (`PrimitiveComponent.SetSimulatePhysics` _cube true)
  (`KismetSystemLibrary.Delay` 0.0)
  (`PrimitiveComponent.AddImpulse` _cube (+ (* (`KismetMathLibrary.Normal` (`KismetMathLibrary.MakeVector` (.x (`self.GetActorForwardVector`)) (.y (`self.GetActorForwardVector`)))) 15000.0) (`KismetMathLibrary.MakeVector` (`KismetMathLibrary.RandomFloatInRange` -500.0 500.0) (`KismetMathLibrary.RandomFloatInRange` -500.0 500.0) -500.0)) "None" true)
  (`KismetSystemLibrary.Delay` 5.0)
  (`PrimitiveComponent.SetSimulatePhysics` (`self.Cube`) true))

(event `self.Sphere.OnComponentBeginOverlap`
  (params (OverlappedComponent :type "PrimitiveComponent Object Reference") (OtherActor :type "Actor Object Reference") (OtherComp :type "PrimitiveComponent Object Reference") (OtherBodyIndex :type Integer) (bFromSweep :type Boolean) (SweepResult :type "HitResult Structure (by ref)"))
  (bind _whichweapon (`self.whichWeapon`))
  (bind _asbp_motorcycle_character (cast `/Game/Blueprint/Player/BP_MotorcycleCharacter` OtherActor))
  (if (== OtherComp (`Character.CapsuleComponent` _asbp_motorcycle_character))
    (`self.K2_SetActorLocation` (0.0 0.0 5000.0))
    (`PrimitiveComponent.SetSimulatePhysics` (`self.Cube`) false)
    (message `/Game/Blueprint/Player/PlayerScoreSystem/BPI_PlayerGetScore.PlayerGetScore` _asbp_motorcycle_character "NewEnumerator0" (`KismetTextLibrary.MakeInvariantText` (`KismetStringLibrary.Concat_StrStr` "获得装备" (`|GetEnumeratorNameAsString` (`self.whichWeapon`)) "！加100分！")) 100.0)
    (`GameplayStatics.PlaySound2D` "/Game/Art/Voice/driken5482-retro-coin-1-236677.driken5482-retro-coin-1-236677" 1.0 1.0 0.0 null null)
    (bind _weaponinbag (`/Game/Blueprint/Player/BP_MotorcycleCharacter.WeaponInBag` _asbp_motorcycle_character))
    (bind _keys (`BlueprintMapLibrary.Map_Keys` _weaponinbag))
    (if (`KismetArrayLibrary.Array_Contains` _keys _whichweapon)
      (bind _output_get (set `self.WeaponNumInBag` (+ (`BlueprintMapLibrary.Map_Find` _weaponinbag _whichweapon) 1)))
      (`BlueprintMapLibrary.Map_Add` _weaponinbag (`self.whichWeapon`) _output_get)
      (else
        (`BlueprintMapLibrary.Map_Add` _weaponinbag (`self.whichWeapon`) 1)))))

(event `self.Cube.OnComponentBeginOverlap`
  (params (OverlappedComponent :type "PrimitiveComponent Object Reference") (OtherActor :type "Actor Object Reference") (OtherComp :type "PrimitiveComponent Object Reference") (OtherBodyIndex :type Integer) (bFromSweep :type Boolean) (SweepResult :type "HitResult Structure (by ref)")))

(fn `UserConstructionScript`)