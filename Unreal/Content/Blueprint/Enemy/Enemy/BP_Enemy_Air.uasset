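; Airborne enemy in a motorcycle game that flies forward, shoots at the player and awards score when destroyed.
; A manager starts and stops it; timers randomly vary speed and lateral position and fire bursts from a pre-spawned bullet pool.
; Death triggers a pre-spawned wreck actor; death or excessive player distance calls EscapePlayers, bound through manager-supplied setup.
; Obstacle traces run once per start, and their turn result is only stored here.
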(event `self.ReceiveBeginPlay`
  (`|ExecutionSequence`
    (:`then_0`
      (`self.TestMod`)
      (`self.SpawnAmmo`)
      (`self.Flying`))
    (:`then_1`
      (bind _returnvalue (`|SpawnActorFromClass` "/Game/Blueprint/Enemy/Enemy/BP_EnemyMotoSpawn.BP_EnemyMotoSpawn_C" (`KismetMathLibrary.MakeTransform` (0.0 0.0 5000.0)) "Undefined" "MultiplyWithRoot" null null))
      (set `self.DeathBody` _returnvalue))))

(event `Flying`
  (bind (_direction `_新建轨道_0`) (`Timeline|时间轴_0` :!via `PlayFromStart`)
    (:`Update`
      (`SceneComponent.K2_SetWorldRotation` (`self.flyp`) (`KismetMathLibrary.MakeRotator` 0.0 0.0 (* `_新建轨道_0` 360.0)) false false))
    (:`Finished`
      (`self.Flying`))))

(event `self.StopMovement`
  (params (`Stop?` :type Boolean))
  ; 用manager决定是否发车
  (if `Stop?`
    (set `self.isAction` false)
    ;; 停止侦测
    (`KismetSystemLibrary.K2_PauseTimerHandle` (`self.DetectorTimer`))
    (set `self.PlayerInArea?` false)
    (`self.CheckEnemyCanAction?`)
    (else
      (set `self.isAction` true)
      ;; 开始侦测环境
      (`self.StartTurn`)
      ;; 设置数值（例如速度，健康值）
      (`self.SetData`))))

(event `SpawnAmmo`
  ; 生成子弹
  (for _ (range (`self.MaxAmmo`))
    (bind _returnvalue (`|SpawnActorFromClass` "/Game/Blueprint/Enemy/Enemy/BP_Enemy_Bullet.BP_Enemy_Bullet_C" (`KismetMathLibrary.MakeTransform` (0.0 0.0 3000.0)) "Undefined" "MultiplyWithRoot" null null))
    (`KismetArrayLibrary.Array_Add` (`self.AmmoArray`) _returnvalue))
  (if (`self.isTesting?`)
    (`self.ShootingAmmo`)))

(event `StartTurn`
  ; 若开始行动，则持续性地侦测环境
  (bind _returnvalue (`KismetSystemLibrary.K2_SetTimerDelegate` (delegate `Turn`) 0.1 true))
  (set `self.DetectorTimer` _returnvalue)
  (`self.Environmental monitoring`)
  (`KismetSystemLibrary.K2_SetTimerDelegate` (delegate `RandomSpeed`) 3.0 true))

(event `RandomSpeed`
  (bind (_returnvalue_x _returnvalue_y) (`KismetMathLibrary.BreakVector` (`self.K2_GetActorLocation`)))
  (bind (_returnvalue_x_2 _returnvalue_y_2 _returnvalue_z) (`KismetMathLibrary.BreakVector` (`self.K2_GetActorLocation`)))
  (bind _basespeed (`self.BaseSpeed`))
  (set `self.RandomSpeedFloat` (`KismetMathLibrary.RandomFloatInRange` (- _basespeed 2000.0) (+ _basespeed 2000.0)))
  (bind _output_get (set `self.CurrentY` _returnvalue_y))
  (set `self.LastY` _output_get)
  (set `self.TargetY` (`KismetMathLibrary.RandomFloatInRange` -1300.0 1300.0))
  (bind (_direction `_新建轨道_0` `_新建轨道_1`) (`Timeline|时间轴` :!via `PlayFromStart`)
    (:`Update`
      (set `self.CurrentSpeed` (`KismetMathLibrary.Lerp` (`self.BaseSpeed`) (`self.RandomSpeedFloat`) `_新建轨道_0`))
      (`self.K2_SetActorLocation` (`KismetMathLibrary.MakeVector` _returnvalue_x_2 (`KismetMathLibrary.Lerp` (`self.CurrentY`) (`self.TargetY`) `_新建轨道_1`) _returnvalue_z)))))

(event `Turn`
  ; 若开始行动，则持续性地侦测环境
  (if (`self.PlayerInArea?`)
    (`self.Calculate the distance to the player`)))

(event `TestMod`
  ;[1 0.8969 0 0.5] 测试模式
  (if (`self.isTesting?`)
    (bind _asbp_motorcycle_character (cast `/Game/Blueprint/Player/BP_MotorcycleCharacter` (`GameplayStatics.GetPlayerPawn` 0)))
    (bind _output_get (set `self.Player` _asbp_motorcycle_character))
    (set `self.BaseSpeed` (`/Game/Blueprint/Player/BP_MotorcycleCharacter.BaseSpeed` _output_get))
    (set `self.isAction` true)
    (set `self.PlayerInArea?` true)
    (`self.StartTurn`)))

(event `self.ReceiveTick`
  (params (DeltaSeconds :type "Float (single-precision)"))
  ; 简单移动
  (`|ExecutionSequence`
    (:`then_0`
      (if (and (`self.isAction`) (`self.PlayerInArea?`))
        (`self.K2_AddActorWorldOffset` (* (* (`KismetMathLibrary.Vector_Forward`) (`self.CurrentSpeed`)) DeltaSeconds))))))

(event `SetData`
  ; 设置数值
  (set `self.BaseSpeed` (`/Game/Blueprint/Player/BP_MotorcycleCharacter.BaseSpeed` (`self.Player`)))
  (set `self.Health` (`self.BaseHealth`)))

(event `ShootingAmmo`
  ; 子弹射击系统
  (set `self.CurrentAmmoIndex` 0)
  (bind _returnvalue (`KismetSystemLibrary.K2_SetTimerDelegate` (delegate `ShootOnceAmmo`) 0.5 true))
  (set `self.AmmoTimer` _returnvalue))

(event `EnemyHowToTurn`
  (params (How :type "/Game/Blueprint/Enemy/E_HowToTurn Enum" :default "NewEnumerator0") (TurnValue :type "Float (double-precision)"))
  ; 侦测的结果
  (switch `/Game/Blueprint/Enemy/E_HowToTurn` How
    (:`NewEnumerator0`
      (set `self.EHowToTurn` "NewEnumerator0"))
    (:`NewEnumerator1`
      (set `self.EHowToTurn` "NewEnumerator1"))
    (:`NewEnumerator2`
      (set `self.EHowToTurn` "NewEnumerator2")))
  (set `self.Turn Value` TurnValue))

(event `ShootOnceAmmo`
  (bind _player (`self.Player`))
  (bind _returnvalue (+ (`self.CurrentAmmoIndex`) 1))
  ; 子弹射击系统
  (`/Game/Blueprint/Enemy/Enemy/BP_Enemy_Bullet.InitBullet` (`|GetArrayItem` (`self.AmmoArray`) (`self.CurrentAmmoIndex`)) (`SceneComponent.K2_GetComponentLocation` (`self.Sphere_Weapon`)) (`self.K2_GetActorLocation` _player) true (`/Game/Blueprint/Player/BP_MotorcycleCharacter.Speed` _player) (`self.CurrentSpeed`))
  (if (>= _returnvalue (- (`KismetArrayLibrary.Array_Length` (`self.AmmoArray`)) 1))
    (`KismetSystemLibrary.K2_PauseTimerHandle` (`self.AmmoTimer`))
    (else
      (set `self.CurrentAmmoIndex` _returnvalue))))

(event `self.callEnemyStartMovement`
  ; 玩家进入范围（一般在玩家碰撞盒碰撞到敌人）
  (set `self.PlayerInArea?` true)
  (`self.CheckEnemyCanAction?`))

(event `self.Enemy fled`
  ; 敌人加速逃跑（一般在游戏结束时候）
  (bind _output_get (set `self.BaseSpeed` 20000.0))
  (set `self.CurrentSpeed` _output_get)
  (`KismetSystemLibrary.PrintString` "Hello" true true (struct :`R` 0.90853 :`B` 1.0 :`A` 1.0)))

(event `CheckEnemyCanAction?`
  ; 检测敌人是否可射击（一般在玩家进入敌人action区域再开始）
  (if (and (`self.isAction`) (`self.PlayerInArea?`))
    ;; 如果条件满足，开始射击
    (`/Engine/EditorBlueprintResources/StandardMacros.DoOnce` false :!label _label
      (:`Completed`
        (bind _returnvalue (`KismetSystemLibrary.K2_SetTimerDelegate` (delegate `StartShoot`) 3.0 true))
        (set `self.ShootSystemTimer` _returnvalue)
        (`self.StartShoot`)))
    (else
      ;; 条件不满足，停止
      (`KismetSystemLibrary.K2_PauseTimerHandle` (`self.ShootSystemTimer`))
      (goto _label :!via `Reset`))))

(event `self.ReceiveAnyDamage`
  (params (Damage :type "Float (single-precision)") (DamageType :type "DamageType Object Reference") (InstigatedBy :type "Controller Object Reference") (DamageCauser :type "Actor Object Reference"))
  (bind _returnvalue (- (`self.Health`) Damage))
  (if (<= _returnvalue 0.0)
    (set `self.Health` 0.0)
    (message `/Game/Blueprint/Player/PlayerScoreSystem/BPI_PlayerGetScore.PlayerGetScore` (`self.Player`) "NewEnumerator0" "击落空中敌人！+1000分" 1000.0)
    (`self.EnemyIsDie`)
    (else
      (set `self.Health` _returnvalue))))

(event `StartShoot`
  ; 检测敌人是否可射击（一般在玩家进入敌人action区域再开始）
  ;; 如果条件满足，开始射击
  (`self.ShootingAmmo`))

(event `EnemyIsDie`
  (bind _cube (`self.Cube`))
  (`GameplayStatics.SpawnEmitterAtLocation` "/Game/InfimaGames/FreeFPSTemplate/Demo/VFX/Particles/P_Explosion.P_Explosion" (`SceneComponent.K2_GetComponentLocation` (`self.Cube`)) (struct) (3.0 3.0 3.0))
  (`/Game/Blueprint/Enemy/Enemy/BP_EnemyMotoSpawn.EnemyIsDie` (`self.DeathBody`) (`SceneComponent.K2_GetComponentLocation` _cube) (`SceneComponent.K2_GetComponentRotation` _cube))
  (`self.Escape Players` self))

(event `SetPhysics`)

(event `self.BaseInformation`
  (params (Player :type "/Game/Blueprint/Player/BP_MotorcycleCharacter Object Reference") (Manager :type "/Game/Blueprint/Manager/BP_LevelManager Object Reference"))
  ; 重点来了，因为没法直接在manager里直接bind event。我们可以通过bpi把manager引用诱骗过来，在各自的enemy蓝图当中配置，实测可行
  (set `self.isAction` false)
  (set `self.BaseSpeed` (`/Game/Blueprint/Player/BP_MotorcycleCharacter.BaseSpeed` Player))
  (set `self.Player` Player)
  (add `self.Escape Players` (`|CreateDelegate` Manager :!event `EnemyIsEscape`)))

(fn `Calculate the distance to the player`
  (`/Engine/EditorBlueprintResources/StandardMacros.IsValid` (`self.Player`)
    (:`Is Valid`
      (bind _output_get (set `self.DistanceToPlayer` (`KismetMathLibrary.Vector_Distance` (`self.K2_GetActorLocation` (`self.Player`)) (`self.K2_GetActorLocation`))))
      (if (> _output_get 50000.0)
        (`self.Escape Players` self)
        (`KismetSystemLibrary.PrintString` "Escape")))
    (:`Is Not Valid`
      (`KismetSystemLibrary.PrintString` "NONO"))))

(fn `Environmental monitoring`
  (locals (`Are there any obstacles?` :type Boolean :default false) (`Distance to obstacle on the left front` :type "Float (single-precision)" :default 0.0) (`Distance to obstacle on the right front` :type "Float (single-precision)" :default 0.0) (`Distance to obstacle on the left` :type "Float (single-precision)" :default 0.0) (`Distance to obstacle on the right` :type "Float (single-precision)" :default 0.0) (HowToTurn :type "/Game/Blueprint/Enemy/E_HowToTurn Enum") (`Front left has obstacle` :type Boolean :default false) (`Front right has obstacle` :type Boolean :default false) (`Distance to obstacle Front` :type "Float (single-precision)" :default 0.0) (LeftAvoidForce :type "Float (double-precision)") (RightAvoidForce :type "Float (double-precision)") (TurnValue :type "Float (double-precision)"))
  (bind _sphere_front (`self.Sphere_Front`))
  (bind _sphere_left (`self.Sphere_Left`))
  (bind _sphere_right (`self.Sphere_Right`))
  (bind _sphere_left1 (`self.Sphere_Left1`))
  (bind _sphere_right1 (`self.Sphere_Right1`))
  (bind _returnvalue (`SceneComponent.K2_GetComponentLocation` _sphere_right))
  (bind _returnvalue_2 (`SceneComponent.K2_GetComponentLocation` _sphere_left))
  (bind _returnvalue_3 (`SceneComponent.K2_GetComponentLocation` _sphere_left1))
  (bind _returnvalue_4 (`SceneComponent.K2_GetComponentLocation` _sphere_front))
  (bind _returnvalue_5 (`SceneComponent.K2_GetComponentLocation` _sphere_right1))
  (bind _returnvalue_6 (>= (`local.Distance to obstacle on the left front`) (`local.Distance to obstacle on the right front`)))
  ; 向前的射线，检测面前是否有障碍物
  (bind (_outhit _returnvalue_7) (`KismetSystemLibrary.LineTraceSingle` _returnvalue_4 (+ _returnvalue_4 (* (`SceneComponent.GetForwardVector` _sphere_front) 5000.0)) "TraceTypeQuery1"))
  (bind _output_get (set `local.Are there any obstacles?` _returnvalue_7))
  (set `local.Distance to obstacle Front` (`.Distance` (`GameplayStatics.BreakHitResult` _outhit)))
  ; 左前方射线
  (bind (_outhit_2 _returnvalue_8) (`KismetSystemLibrary.LineTraceSingle` _returnvalue_2 (+ _returnvalue_2 (* (`SceneComponent.GetForwardVector` _sphere_left) 5000.0)) "TraceTypeQuery1"))
  (set `local.Front left has obstacle` _returnvalue_8)
  (if _returnvalue_8
    (set `local.Distance to obstacle on the left front` (`.Distance` (`GameplayStatics.BreakHitResult` _outhit_2)))
    (else
      (set `local.Distance to obstacle on the left front` 5000.0)))
  ; 右前方射线
  (bind (_outhit_3 _returnvalue_9) (`KismetSystemLibrary.LineTraceSingle` _returnvalue (+ _returnvalue (* (`SceneComponent.GetForwardVector` _sphere_right) 5000.0)) "TraceTypeQuery1"))
  (set `local.Front right has obstacle` _returnvalue_9)
  (if _returnvalue_9
    (set `local.Distance to obstacle on the right front` (`.Distance` (`GameplayStatics.BreakHitResult` _outhit_3)))
    (else
      (set `local.Distance to obstacle on the right front` 5000.0)))
  ; 检测正左方的距离
  (bind _outhit_4 (`KismetSystemLibrary.LineTraceSingle` _returnvalue_3 (+ _returnvalue_3 (* (`SceneComponent.GetRightVector` _sphere_left1) -3000.0)) "TraceTypeQuery1"))
  (bind _output_get_2 (set `local.Distance to obstacle on the left` (`.Distance` (`GameplayStatics.BreakHitResult` _outhit_4))))
  (set `self.LeftDistance` _output_get_2)
  ; 检测正右边距离
  (bind _outhit_5 (`KismetSystemLibrary.LineTraceSingle` _returnvalue_5 (+ _returnvalue_5 (* (`SceneComponent.GetRightVector` _sphere_right1) 3000.0)) "TraceTypeQuery1"))
  (bind _output_get_3 (set `local.Distance to obstacle on the right` (`.Distance` (`GameplayStatics.BreakHitResult` _outhit_5))))
  (set `self.RightDistance` _output_get_3)
  ; 开始行为判定
  ;; 检测面前是否有障碍物，若无则正常行驶
  (if (`local.Are there any obstacles?`)
    ;; 二级判断，如果需要拐弯，看左右前方哪里可以没障碍物
    (if _returnvalue_6
      (if (`local.Front left has obstacle`)
        (if _returnvalue_6
          (bind _output_get_4 (set `local.HowToTurn` "NewEnumerator0"))
          (`self.EnemyHowToTurn` _output_get_4)
          (else
            (set `local.HowToTurn` "NewEnumerator1" :!label _label)
            ;; 三级判断，检测转弯方向是否为墙壁，避免穿墙
            (switch `/Game/Blueprint/Enemy/E_HowToTurn` (`local.HowToTurn`) :!label _label_2
              (:`NewEnumerator1`
                (if (< (`local.Distance to obstacle on the left`) 250.0)
                  (bind _output_get_5 (set `local.HowToTurn` "NewEnumerator2"))
                  (`self.EnemyHowToTurn` _output_get_5)
                  (else
                    (`self.EnemyHowToTurn` (`local.HowToTurn`)))))
              (:`NewEnumerator2`
                (if (< (`local.Distance to obstacle on the right`) 250.0)
                  (bind _output_get_6 (set `local.HowToTurn` "NewEnumerator1"))
                  (`self.EnemyHowToTurn` _output_get_6)
                  (else
                    (`self.EnemyHowToTurn` (`local.HowToTurn`))))))))
        (else
          (goto _label)))
      (elif (`local.Front right has obstacle`)
        (if (not _returnvalue_6)
          (bind _output_get_7 (set `local.HowToTurn` "NewEnumerator0"))
          (`self.EnemyHowToTurn` _output_get_7)
          (else
            (set `local.HowToTurn` "NewEnumerator2" :!label _label_3)
            (goto _label_2)))
        (else
          (goto _label_3))))
    (else
      (bind _output_get_8 (set `local.HowToTurn` "NewEnumerator0"))
      (`self.EnemyHowToTurn` _output_get_8))))

(fn `UserConstructionScript`)