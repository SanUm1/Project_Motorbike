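; Enemy motor vehicle that drives forward while dodging obstacles, started and stopped through StopMovement.
; A looping timer runs five line traces (forward, front diagonals, sides) to pick straight, left or right, which Tick applies as offset movement with sideways shifts.
; A second timer and timeline vary speed around the player's base speed.
; It calls EscapePlayers when health runs out or the player is too far away; a test mode self-starts it.
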(event `self.ReceiveBeginPlay`
  (`|ExecutionSequence`
    (:`then_0`
      (`self.TestMod`))))

(event `/Game/Blueprint/Enemy/BPI_CallItemState.StopMovement`
  (params (`Stop?` :type Boolean))
  ; 用manager决定是否发车
  (if `Stop?`
    (set `self.isAction` false)
    ;; 停止侦测
    (`KismetSystemLibrary.K2_PauseTimerHandle` (`self.DetectorTimer`))
    (set `self.PlayerInArea?` false)
    (else
      (set `self.isAction` true)
      ;; 开始侦测环境
      (`self.StartTurn`)
      ;; 设置数值（例如速度，健康值）
      (`self.SetData`))))

(event `StartTurn`
  ; 若开始行动，则持续性地侦测环境
  (bind _returnvalue (`KismetSystemLibrary.K2_SetTimerDelegate` (delegate `Turn`) 0.1 true))
  (set `self.DetectorTimer` _returnvalue)
  (`self.Environmental monitoring`)
  (`KismetSystemLibrary.K2_SetTimerDelegate` (delegate `RandomSpeed`) 3.0 true))

(event `RandomSpeed`
  (bind _basespeed (`self.BaseSpeed`))
  (set `self.RandomSpeedFloat` (`KismetMathLibrary.RandomFloatInRange` (- _basespeed 2000.0) (+ _basespeed 2000.0)))
  (bind (_direction `_新建轨道_0`) (`Timeline|时间轴` :!via `PlayFromStart`)
    (:`Update`
      (set `self.CurrentSpeed` (`KismetMathLibrary.Lerp` (`self.BaseSpeed`) (`self.RandomSpeedFloat`) `_新建轨道_0`)))))

(event `Turn`
  ; 若开始行动，则持续性地侦测环境
  (`self.Environmental monitoring`)
  (if (`self.PlayerInArea?`)
    (`self.Calculate the distance to the player`)))

(event `TestMod`
  ;[1 0.8969 0 0.5] 测试模式
  (if (`self.isTesting?`)
    (bind _asbp_motorcycle_character (cast `/Game/Blueprint/Player/BP_MotorcycleCharacter` (`GameplayStatics.GetPlayerPawn` 0)))
    (bind _output_get (set `self.Player` _asbp_motorcycle_character))
    (set `self.BaseSpeed` (`/Game/Blueprint/Player/BP_MotorcycleCharacter.BaseSpeed` _output_get))
    (set `self.isAction` true)
    (set `self.PlayerInArea?` true)
    (`self.StartTurn`)))

(event `self.ReceiveTick`
  (params (DeltaSeconds :type "Float (single-precision)"))
  (bind _returnvalue (* (* (`SceneComponent.GetRightVector` (`self.SkeletalMesh`)) 3000.0) DeltaSeconds))
  ; 简单移动
  (`|ExecutionSequence`
    (:`then_0`
      (if (and (`self.isAction`) (`self.PlayerInArea?`))
        (`self.K2_AddActorWorldOffset` (* (* (`KismetMathLibrary.Vector_Forward`) (`self.CurrentSpeed`)) DeltaSeconds))
        ;; 根据环境侦测的结果判断需不需要拐弯
        (switch `/Game/Blueprint/Enemy/E_HowToTurn` (`self.EHowToTurn`)
          (:`NewEnumerator1`
            (`self.K2_AddActorWorldOffset` (* _returnvalue -1.0)))
          (:`NewEnumerator2`
            (`self.K2_AddActorWorldOffset` _returnvalue)))))))

(event `SetData`
  ; 设置数值
  (set `self.BaseSpeed` (`/Game/Blueprint/Player/BP_MotorcycleCharacter.BaseSpeed` (`self.Player`)))
  (set `self.Health` (`self.BaseHealth`)))

(event `EnemyHowToTurn`
  (params (How :type "/Game/Blueprint/Enemy/E_HowToTurn Enum" :default "NewEnumerator0") (TurnValue :type "Float (double-precision)"))
  ; 侦测的结果
  (switch `/Game/Blueprint/Enemy/E_HowToTurn` How
    (:`NewEnumerator0`
      (set `self.EHowToTurn` "NewEnumerator0"))
    (:`NewEnumerator1`
      (set `self.EHowToTurn` "NewEnumerator1"))
    (:`NewEnumerator2`
      (set `self.EHowToTurn` "NewEnumerator2")))
  (set `self.Turn Value` TurnValue))

(event `/Game/Blueprint/Enemy/BPI_CallItemState.callEnemyStartMovement`
  (set `self.PlayerInArea?` true))

(event `/Game/Blueprint/Enemy/BPI_CallItemState.Enemy fled`
  (bind _output_get (set `self.BaseSpeed` 20000.0))
  (set `self.CurrentSpeed` _output_get)
  (`KismetSystemLibrary.PrintString` "Hello" true true (struct :`R` 0.90853 :`B` 1.0 :`A` 1.0)))

(event `self.ReceiveAnyDamage`
  (params (Damage :type "Float (single-precision)") (DamageType :type "DamageType Object Reference") (InstigatedBy :type "Controller Object Reference") (DamageCauser :type "Actor Object Reference"))
  (bind _returnvalue (- (`self.Health`) Damage))
  (if (<= _returnvalue 0.0)
    (set `self.Health` 0.0)
    (`self.Escape Players` self)
    (else
      (set `self.Health` _returnvalue))))

(fn `Calculate the distance to the player`
  (`/Engine/EditorBlueprintResources/StandardMacros.IsValid` (`self.Player`)
    (:`Is Valid`
      (bind _output_get (set `self.DistanceToPlayer` (`KismetMathLibrary.Vector_Distance` (`self.K2_GetActorLocation` (`self.Player`)) (`self.K2_GetActorLocation`))))
      (if (> _output_get 50000.0)
        (`self.Escape Players` self)
        (`KismetSystemLibrary.PrintString` "Escape")))
    (:`Is Not Valid`
      (`KismetSystemLibrary.PrintString` "NONO"))))

(fn `Environmental monitoring`
  (locals (`Are there any obstacles?` :type Boolean :default false) (`Distance to obstacle on the left front` :type "Float (single-precision)" :default 0.0) (`Distance to obstacle on the right front` :type "Float (single-precision)" :default 0.0) (`Distance to obstacle on the left` :type "Float (single-precision)" :default 0.0) (`Distance to obstacle on the right` :type "Float (single-precision)" :default 0.0) (HowToTurn :type "/Game/Blueprint/Enemy/E_HowToTurn Enum") (`Front left has obstacle` :type Boolean :default false) (`Front right has obstacle` :type Boolean :default false) (`Distance to obstacle Front` :type "Float (single-precision)" :default 0.0) (LeftAvoidForce :type "Float (double-precision)") (RightAvoidForce :type "Float (double-precision)") (TurnValue :type "Float (double-precision)"))
  (bind _sphere_front (`self.Sphere_Front`))
  (bind _sphere_left (`self.Sphere_Left`))
  (bind _sphere_right (`self.Sphere_Right`))
  (bind _sphere_left1 (`self.Sphere_Left1`))
  (bind _sphere_right1 (`self.Sphere_Right1`))
  (bind _returnvalue (`SceneComponent.K2_GetComponentLocation` _sphere_right))
  (bind _returnvalue_2 (`SceneComponent.K2_GetComponentLocation` _sphere_left))
  (bind _returnvalue_3 (`SceneComponent.K2_GetComponentLocation` _sphere_left1))
  (bind _returnvalue_4 (`SceneComponent.K2_GetComponentLocation` _sphere_front))
  (bind _returnvalue_5 (`SceneComponent.K2_GetComponentLocation` _sphere_right1))
  (bind _returnvalue_6 (>= (`local.Distance to obstacle on the left front`) (`local.Distance to obstacle on the right front`)))
  ; 向前的射线，检测面前是否有障碍物
  (bind (_outhit _returnvalue_7) (`KismetSystemLibrary.LineTraceSingle` _returnvalue_4 (+ _returnvalue_4 (* (`SceneComponent.GetForwardVector` _sphere_front) 5000.0)) "TraceTypeQuery1"))
  (bind _output_get (set `local.Are there any obstacles?` _returnvalue_7))
  (set `local.Distance to obstacle Front` (`.Distance` (`GameplayStatics.BreakHitResult` _outhit)))
  ; 左前方射线
  (bind (_outhit_2 _returnvalue_8) (`KismetSystemLibrary.LineTraceSingle` _returnvalue_2 (+ _returnvalue_2 (* (`SceneComponent.GetForwardVector` _sphere_left) 5000.0)) "TraceTypeQuery1"))
  (set `local.Front left has obstacle` _returnvalue_8)
  (if _returnvalue_8
    (set `local.Distance to obstacle on the left front` (`.Distance` (`GameplayStatics.BreakHitResult` _outhit_2)))
    (else
      (set `local.Distance to obstacle on the left front` 5000.0)))
  ; 右前方射线
  (bind (_outhit_3 _returnvalue_9) (`KismetSystemLibrary.LineTraceSingle` _returnvalue (+ _returnvalue (* (`SceneComponent.GetForwardVector` _sphere_right) 5000.0)) "TraceTypeQuery1"))
  (set `local.Front right has obstacle` _returnvalue_9)
  (if _returnvalue_9
    (set `local.Distance to obstacle on the right front` (`.Distance` (`GameplayStatics.BreakHitResult` _outhit_3)))
    (else
      (set `local.Distance to obstacle on the right front` 5000.0)))
  ; 检测正左方的距离
  (bind _outhit_4 (`KismetSystemLibrary.LineTraceSingle` _returnvalue_3 (+ _returnvalue_3 (* (`SceneComponent.GetRightVector` _sphere_left1) -3000.0)) "TraceTypeQuery1"))
  (bind _output_get_2 (set `local.Distance to obstacle on the left` (`.Distance` (`GameplayStatics.BreakHitResult` _outhit_4))))
  (set `self.LeftDistance` _output_get_2)
  ; 检测正右边距离
  (bind _outhit_5 (`KismetSystemLibrary.LineTraceSingle` _returnvalue_5 (+ _returnvalue_5 (* (`SceneComponent.GetRightVector` _sphere_right1) 3000.0)) "TraceTypeQuery1"))
  (bind _output_get_3 (set `local.Distance to obstacle on the right` (`.Distance` (`GameplayStatics.BreakHitResult` _outhit_5))))
  (set `self.RightDistance` _output_get_3)
  ; 开始行为判定
  ;; 检测面前是否有障碍物，若无则正常行驶
  (if (`local.Are there any obstacles?`)
    ;; 二级判断，如果需要拐弯，看左右前方哪里可以没障碍物
    (if _returnvalue_6
      (if (`local.Front left has obstacle`)
        (if _returnvalue_6
          (bind _output_get_4 (set `local.HowToTurn` "NewEnumerator0"))
          (`self.EnemyHowToTurn` _output_get_4)
          (else
            (set `local.HowToTurn` "NewEnumerator1" :!label _label)
            ;; 三级判断，检测转弯方向是否为墙壁，避免穿墙
            (switch `/Game/Blueprint/Enemy/E_HowToTurn` (`local.HowToTurn`) :!label _label_2
              (:`NewEnumerator1`
                (if (< (`local.Distance to obstacle on the left`) 250.0)
                  (bind _output_get_5 (set `local.HowToTurn` "NewEnumerator2"))
                  (`self.EnemyHowToTurn` _output_get_5)
                  (else
                    (`self.EnemyHowToTurn` (`local.HowToTurn`)))))
              (:`NewEnumerator2`
                (if (< (`local.Distance to obstacle on the right`) 250.0)
                  (bind _output_get_6 (set `local.HowToTurn` "NewEnumerator1"))
                  (`self.EnemyHowToTurn` _output_get_6)
                  (else
                    (`self.EnemyHowToTurn` (`local.HowToTurn`))))))))
        (else
          (goto _label)))
      (elif (`local.Front right has obstacle`)
        (if (not _returnvalue_6)
          (bind _output_get_7 (set `local.HowToTurn` "NewEnumerator0"))
          (`self.EnemyHowToTurn` _output_get_7)
          (else
            (set `local.HowToTurn` "NewEnumerator2" :!label _label_3)
            (goto _label_2)))
        (else
          (goto _label_3))))
    (else
      (bind _output_get_8 (set `local.HowToTurn` "NewEnumerator0"))
      (`self.EnemyHowToTurn` _output_get_8))))

(fn `UserConstructionScript`)