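; Motorcycle boss that drives forward once active and engaged, dodging obstacles via timed line traces.
; A looping timer fires a beam-sight gun that tracks the player, blinks, then hits the locked point relative to the boss.
; It recycles two pooled minion bikes behind a spawn progress widget.
; Dispatchers bound through BaseInformation report fight start, damage, death and escape when the player falls too far away.
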(event `self.ReceiveBeginPlay`
  (bind _returnvalue (`|CreateWidget` "/Game/UI/HolographicProjection/W_EnemySpawnEnemy.W_EnemySpawnEnemy_C"))
  (`WidgetComponent.SetWidget` (`self.Widget`) _returnvalue)
  (bind _output_get (set `self.SpawnUI` _returnvalue))
  (`Widget.SetVisibility` _output_get "Hidden")
  (bind _asbp_motorcycle_character (cast `/Game/Blueprint/Player/BP_MotorcycleCharacter` (`GameplayStatics.GetPlayerPawn` 0)))
  (set `self.Player` _asbp_motorcycle_character)
  (bind _returnvalue_2 (`|SpawnActorFromClass` "/Game/Blueprint/Enemy/Enemy/BP_EnemyMotoSpawn.BP_EnemyMotoSpawn_C" (`KismetMathLibrary.MakeTransform` (0.0 0.0 5000.0) (struct) (1.5 1.5 1.5)) "Undefined" "MultiplyWithRoot" null null))
  (set `self.DeathBody` _returnvalue_2)
  (for _ (range 2)
    (bind _returnvalue_3 (`|SpawnActorFromClass` "/Game/Blueprint/Enemy/Boss/Boss_Moto/BP_Boss_Moto_Small.BP_Boss_Moto_Small_C" (`KismetMathLibrary.MakeTransform` (0.0 0.0 5000.0)) "Undefined" "MultiplyWithRoot" null null))
    (set `/Game/Blueprint/Enemy/Boss/Boss_Moto/BP_Boss_Moto_Small.Player` (`self.Player`) _returnvalue_3)
    (add `/Game/Blueprint/Enemy/Boss/Boss_Moto/BP_Boss_Moto_Small.SmallIsDie` _returnvalue_3 (`|CreateDelegate` :!event `SmallDie`))
    (`KismetArrayLibrary.Array_Add` (`self.SmallMotoStrandbyArrayArray`) _returnvalue_3)))

(event `SmallDie`
  (params (which :type "/Game/Blueprint/Enemy/Boss/Boss_Moto/BP_Boss_Moto_Small Object Reference"))
  ; 当小弟死亡，开始生成
  (message `/Game/Blueprint/Player/PlayerScoreSystem/BPI_PlayerGetScore.PlayerGetScore` (`self.Player`) "NewEnumerator0" "击杀小弟！500分！" 500.0)
  (`self.K2_SetActorLocation` which (0.0 0.0 5000.0) false false)
  (if (`self.isAction`)
    (`KismetArrayLibrary.Array_RemoveItem` (`self.SmallMotoArray`) which)
    (`KismetArrayLibrary.Array_Add` (`self.SmallMotoStrandbyArrayArray`) which)
    (if (not (`self.isSpawningEnemy?`))
      (`self.StartSpawnEnemy`))))

(event `StartSpawnEnemy`
  (bind _spawnui (`self.SpawnUI`))
  ; 正在生成小弟
  (set `self.isSpawningEnemy?` true)
  (`Widget.SetVisibility` _spawnui "Visible")
  (`Widget.SetVisibility` (`/Game/UI/HolographicProjection/W_EnemySpawnEnemy.ProgressBar_0` _spawnui) "Visible")
  (`UserWidget.PlayAnimation` _spawnui (`/Game/UI/HolographicProjection/W_EnemySpawnEnemy.NewAnimation` _spawnui) 0.0 1 "Forward" 1.0 false)
  (bind _returnvalue (`KismetSystemLibrary.K2_SetTimerDelegate` (delegate `SpawnSmallEnemy`) 10.5))
  (set `self.SpawnTimer` _returnvalue))

(event `self.StopMovement`
  (params (`Stop?` :type Boolean))
  ; 用manager决定是否发车
  (if `Stop?`
    (set `self.isAction` false)
    ;; 停止侦测
    (`KismetSystemLibrary.K2_PauseTimerHandle` (`self.DetectorTimer`))
    (set `self.PlayerInArea?` false)
    (`self.CheckEnemyCanAction?`)
    (`KismetSystemLibrary.K2_PauseTimerHandle` (`self.SpawnTimer`))
    (`self.ResetBossCheckPlayer`)
    (for _array_element (`self.SmallMotoArray`)
      (`GameplayStatics.ApplyDamage` _array_element 1000000.0)
      (`KismetArrayLibrary.Array_Add` (`self.SmallMotoStrandbyArrayArray`) _array_element))
    (`KismetArrayLibrary.Array_Clear` (`self.SmallMotoArray`))
    (else
      (set `self.isAction` true)
      ;; 开始侦测环境
      (`self.StartTurn`)
      ;; 设置数值（例如速度，健康值）
      (`self.SetData`)
      (`self.CheckEnemyCanAction?`)
      (`SceneComponent.SetVisibility` (`self.Cube`) true false))))

(event `SpawnSmallEnemy`
  (bind _currentsmallenemy (`self.CurrentSmallEnemy`))
  (bind _returnvalue (`SceneComponent.K2_GetComponentLocation` (`self.SpawnPoint_1`)))
  ; 正在生成小弟
  (set `self.CurrentSmallEnemy` (`|GetArrayItem` (`self.SmallMotoStrandbyArrayArray`)))
  (`GameplayStatics.SpawnEmitterAtLocation` "/Game/InfimaGames/FreeFPSTemplate/Demo/VFX/Particles/P_Explosion.P_Explosion" _returnvalue (struct) (3.0 3.0 3.0))
  (`self.K2_SetActorLocationAndRotation` :`self` _currentsmallenemy :`NewLocation` _returnvalue)
  (`/Game/Blueprint/Enemy/Boss/Boss_Moto/BP_Boss_Moto_Small.SpawnSmall` _currentsmallenemy)
  (`KismetArrayLibrary.Array_Add` (`self.SmallMotoArray`) _currentsmallenemy)
  (`KismetArrayLibrary.Array_RemoveItem` (`self.SmallMotoStrandbyArrayArray`) _currentsmallenemy)
  (if (< (`KismetArrayLibrary.Array_Length` (`self.SmallMotoArray`)) 2)
    (`self.StartSpawnEnemy`)
    (else
      (`Widget.SetVisibility` (`self.SpawnUI`) "Hidden")
      (set `self.isSpawningEnemy?` false))))

(event `StartTurn`
  ; 若开始行动，则持续性地侦测环境
  (bind _returnvalue (`KismetSystemLibrary.K2_SetTimerDelegate` (delegate `Turn`) 0.1 true))
  (set `self.DetectorTimer` _returnvalue)
  (`self.Environmental monitoring`))

(event `Turn`
  ; 若开始行动，则持续性地侦测环境
  (`self.Environmental monitoring`)
  (if (`self.PlayerInArea?`)
    (`self.Calculate the distance to the player`)))

(event `MechinGunShooting`
  ; 简单子弹射击系统
  (set `self.GunAttackTime` 0.0)
  (bind _returnvalue (`KismetSystemLibrary.K2_SetTimerDelegate` (delegate `BulletShooting`) 0.05 true))
  (set `self.ShootTimer` _returnvalue)
  (`SceneComponent.SetVisibility` (`self.Sphere`) true false)
  (`SceneComponent.SetVisibility` (`self.Cylinder6`) true false))

(event `self.ReceiveTick`
  (params (DeltaSeconds :type "Float (single-precision)"))
  (bind _returnvalue (* (* (`SceneComponent.GetRightVector` (`self.SkeletalMesh`)) 3000.0) DeltaSeconds))
  ; 简单移动
  (`|ExecutionSequence`
    (:`then_0`
      (if (and (`self.isAction`) (`self.PlayerInArea?`))
        (`self.K2_AddActorWorldOffset` (* (* (`KismetMathLibrary.Vector_Forward`) (`self.CurrentSpeed`)) DeltaSeconds))
        ;; 根据环境侦测的结果判断需不需要拐弯
        (switch `/Game/Blueprint/Enemy/E_HowToTurn` (`self.EHowToTurn`)
          (:`NewEnumerator1`
            (`self.K2_AddActorWorldOffset` (* _returnvalue -1.0) true))
          (:`NewEnumerator2`
            (`self.K2_AddActorWorldOffset` _returnvalue true)))))))

(event `SetData`
  ; 设置数值
  (set `self.BaseSpeed` (`/Game/Blueprint/Player/BP_MotorcycleCharacter.BaseSpeed` (`self.Player`)))
  (set `self.Health` (`self.BaseHealth`)))

(event `BulletShooting`
  (bind _cylinder6 (`self.Cylinder6`))
  (bind _returnvalue (`SceneComponent.K2_GetComponentLocation` (`self.Sphere_Weapon`)))
  (bind _returnvalue_2 (`SceneComponent.K2_GetComponentLocation` (`self.Sphere_Weapon`)))
  (bind (_returnvalue_x _returnvalue_y) (`KismetMathLibrary.BreakVector` (`SceneComponent.K2_GetComponentScale` _cylinder6)))
  (bind _returnvalue_3 (+ (`self.GunAttackTime`) 0.05))
  (bind _returnvalue_4 (+ _returnvalue (* (`KismetMathLibrary.Normal` (- (`self.K2_GetActorLocation` (`self.Player`)) (`SceneComponent.K2_GetComponentLocation` (`self.Sphere_Weapon`)))) 20000.0)))
  ; 简单子弹射击系统
  (if true
    (if (>= _returnvalue_3 2.0)
      ;; 造成伤害
      (`KismetSystemLibrary.K2_PauseTimerHandle` (`self.ShootTimer`))
      (bind _outhit (`KismetSystemLibrary.LineTraceSingle` :`Start` _returnvalue_2 :`End` (+ _returnvalue_2 (* (`KismetMathLibrary.Normal` (- (`KismetMathLibrary.TransformLocation` (`self.GetTransform` self) (`self.LockedLocation`)) _returnvalue_2)) 20000.0)) :`TraceChannel` "TraceTypeQuery1" :`DrawDebugType` "ForDuration"))
      (bind (_bblockinghit _binitialoverlap _time _distance _location _impactpoint _normal _impactnormal _physmat _hitactor) (`GameplayStatics.BreakHitResult` _outhit))
      (`GameplayStatics.ApplyDamage` _hitactor 30.0)
      (if (== _hitactor (`self.Player`))
        (message `/Game/Blueprint/Player/PlayerScoreSystem/BPI_PlayerGetScore.PlayerGetScore` (`self.Player`) "NewEnumerator2" "被Boss武器击中" 0.0))
      (`SceneComponent.SetVisibility` (`self.Sphere`) false false)
      (`SceneComponent.SetVisibility` (`self.Cylinder6`) false false)
      (else
        (set `self.GunAttackTime` _returnvalue_3)
        (if (>= (`self.GunAttackTime`) 1.5)
          (`/Engine/EditorBlueprintResources/StandardMacros.FlipFlop`
            (:`A`
              (`SceneComponent.SetVisibility` (`self.Cylinder6`) false false)
              (`SceneComponent.SetVisibility` (`self.Sphere`) false false))
            (:`B`
              (`SceneComponent.SetVisibility` (`self.Sphere`) true false)
              (`SceneComponent.SetVisibility` (`self.Cylinder6`) true false)))
          (else
            ;; 瞄准阶段
            (bind _outhit_2 (`KismetSystemLibrary.LineTraceSingle` _returnvalue _returnvalue_4 "TraceTypeQuery1"))
            (bind (_bblockinghit_2 _binitialoverlap_2 _time_2 _distance_2 _location_2) (`GameplayStatics.BreakHitResult` _outhit_2))
            (`SceneComponent.K2_SetWorldLocation` (`self.Sphere`) _location_2 false false)
            (bind _returnvalue_5 (`KismetMathLibrary.VLerp` _returnvalue _returnvalue_4 _time_2))
            (`SceneComponent.K2_SetWorldLocation` _cylinder6 (/ (+ _returnvalue _returnvalue_5) 2.0) false false)
            (`SceneComponent.K2_SetWorldRotation` _cylinder6 (`KismetMathLibrary.MakeRotFromZ` (`KismetMathLibrary.Normal` (- _returnvalue_5 _returnvalue))) false false)
            (`SceneComponent.SetWorldScale3D` _cylinder6 (`KismetMathLibrary.MakeVector` _returnvalue_x _returnvalue_y (/ _distance_2 100.0)))
            (set `self.AimLocation` _returnvalue_5)
            (set `self.LockedLocation` (`KismetMathLibrary.InverseTransformLocation` (`self.GetTransform` self) (`self.AimLocation`)))))))))

(event `EnemyHowToTurn`
  (params (How :type "/Game/Blueprint/Enemy/E_HowToTurn Enum" :default "NewEnumerator0") (TurnValue :type "Float (double-precision)"))
  ; 侦测的结果
  (switch `/Game/Blueprint/Enemy/E_HowToTurn` How
    (:`NewEnumerator0`
      (set `self.EHowToTurn` "NewEnumerator0"))
    (:`NewEnumerator1`
      (set `self.EHowToTurn` "NewEnumerator1"))
    (:`NewEnumerator2`
      (set `self.EHowToTurn` "NewEnumerator2")))
  (set `self.Turn Value` TurnValue))

(event `/Game/Blueprint/Enemy/BPI_CallItemState.callEnemyStartMovement`
  ; 玩家进入范围（一般在玩家碰撞盒碰撞到敌人）
  (`/Engine/EditorBlueprintResources/StandardMacros.DoOnce` false :!label _label
    (:`Completed`
      (set `self.PlayerInArea?` true)
      (`self.CheckEnemyCanAction?`)
      (`self.ReadyTooFight`)
      (`self.StartSpawnEnemy`))))

(event `ResetBossCheckPlayer`
  (goto _label :!via `Reset`))

(event `self.Enemy fled`
  ; 敌人加速逃跑（一般在游戏结束时候）
  (bind _output_get (set `self.BaseSpeed` 20000.0))
  (set `self.CurrentSpeed` _output_get)
  (`KismetSystemLibrary.PrintString` "Hello" true true (struct :`R` 0.90853 :`B` 1.0 :`A` 1.0)))

(event `CheckEnemyCanAction?`
  ; 检测敌人是否可射击（一般在玩家进入敌人action区域再开始）
  (if (and (`self.isAction`) (`self.PlayerInArea?`))
    ;; 如果条件满足，开始射击
    (`/Engine/EditorBlueprintResources/StandardMacros.DoOnce` false :!label _label_2
      (:`Completed`
        (bind _returnvalue (`KismetSystemLibrary.K2_SetTimerDelegate` (delegate `StartShoot`) 8.0 true))
        (set `self.ShootSystemTimer` _returnvalue)))
    (else
      ;; 条件不满足，停止
      (`KismetSystemLibrary.K2_PauseTimerHandle` (`self.ShootSystemTimer`))
      (goto _label_2 :!via `Reset`))))

(event `self.ReceiveAnyDamage`
  (params (Damage :type "Float (single-precision)") (DamageType :type "DamageType Object Reference") (InstigatedBy :type "Controller Object Reference") (DamageCauser :type "Actor Object Reference"))
  (bind _returnvalue (- (`self.Health`) Damage))
  (if (<= _returnvalue 0.0)
    (set `self.Health` 0.0)
    (`self.EnemyIsDie`)
    (message `/Game/Blueprint/Player/PlayerScoreSystem/BPI_PlayerGetScore.PlayerGetScore` (`self.Player`) "NewEnumerator0" "击杀Boss！+10000分" 10000.0)
    (else
      (set `self.Health` _returnvalue)))
  (`self.BossDamage` (`self.Health`) (`self.BaseHealth`)))

(event `StartShoot`
  ; 检测敌人是否可射击（一般在玩家进入敌人action区域再开始）
  ;; 如果条件满足，开始射击
  (`self.MechinGunShooting`))

(event `EnemyIsDie`
  (bind _returnvalue (`self.K2_GetActorLocation`))
  ; 敌人死亡
  (`KismetSystemLibrary.K2_PauseTimerHandle` (`self.SpawnTimer`))
  (`GameplayStatics.SpawnEmitterAtLocation` "/Game/InfimaGames/FreeFPSTemplate/Demo/VFX/Particles/P_Explosion.P_Explosion" _returnvalue (struct) (3.0 3.0 3.0))
  (set `self.MotoLocation` (`self.K2_GetActorLocation`))
  (set `self.MotoRotation` (`self.K2_GetActorRotation`))
  (`/Game/Blueprint/Enemy/Enemy/BP_EnemyMotoSpawn.EnemyIsDie` (`self.DeathBody`) _returnvalue (`self.MotoRotation`))
  (`GameplayStatics.PlaySoundAtLocation` "/Game/Art/Voice/explosion.explosion" _returnvalue (struct) 1.0 1.0 0.0 null null null null)
  (`self.EndEvent`)
  (`self.Escape Players` self))

(event `self.BaseInformation`
  (params (Player :type "/Game/Blueprint/Player/BP_MotorcycleCharacter Object Reference") (Manager :type "/Game/Blueprint/Manager/BP_LevelManager Object Reference"))
  ; 重点来了，因为没法直接在manager里直接bind event。我们可以通过bpi把manager引用诱骗过来，在各自的enemy蓝图当中配置，实测可行
  (set `self.isAction` false)
  (set `self.BaseSpeed` (`/Game/Blueprint/Player/BP_MotorcycleCharacter.BaseSpeed` Player))
  (set `self.Player` Player)
  (add `self.Escape Players` (`|CreateDelegate` Manager :!event `EnemyIsEscape`))
  (add `self.EndEvent` (`|CreateDelegate` Manager :!event `EndGameEvent`))
  (add `self.BossDamage` (`|CreateDelegate` Manager :!event `UpdateBossHealth`))
  (add `self.ReadyTooFight` (`|CreateDelegate` Manager :!event `StartToFight`))
  (add `self.BossIsToFar` (`|CreateDelegate` Manager :!event `EventIsFailure`)))

(event `self.Sphere1.OnComponentBeginOverlap`
  (params (OverlappedComponent :type "PrimitiveComponent Object Reference") (OtherActor :type "Actor Object Reference") (OtherComp :type "PrimitiveComponent Object Reference") (OtherBodyIndex :type Integer) (bFromSweep :type Boolean) (SweepResult :type "HitResult Structure (by ref)"))
  (bind _player (`self.Player`))
  (if (== OtherComp (`Character.CapsuleComponent` _player))
    (`GameplayStatics.ApplyDamage` _player 10.0)
    (message `/Game/Blueprint/Player/PlayerScoreSystem/BPI_PlayerGetScore.PlayerGetScore` (`self.Player`) "NewEnumerator2" "与Boss撞车！离Boss太近啦！" 0.0)
    (`Character.LaunchCharacter` _player (* (`self.GetActorForwardVector` _player) -5000.0) false false)))

(fn `Calculate the distance to the player`
  (`/Engine/EditorBlueprintResources/StandardMacros.IsValid` (`self.Player`)
    (:`Is Valid`
      (bind _output_get (set `self.DistanceToPlayer` (`KismetMathLibrary.Vector_Distance` (`self.K2_GetActorLocation` (`self.Player`)) (`self.K2_GetActorLocation`))))
      (if (> _output_get 40000.0)
        (`self.BossIsToFar`)
        (`self.Escape Players` self)
        (message `/Game/Blueprint/Player/PlayerScoreSystem/BPI_PlayerGetScore.PlayerGetScore` (`self.Player`) "NewEnumerator2" "任务失败！Boss逃走了！" 0.0)
        (`KismetSystemLibrary.PrintString` "Escape")))
    (:`Is Not Valid`
      (`KismetSystemLibrary.PrintString` "NONO"))))

(fn `Environmental monitoring`
  (locals (`Are there any obstacles?` :type Boolean :default false) (`Distance to obstacle on the left front` :type "Float (single-precision)" :default 0.0) (`Distance to obstacle on the right front` :type "Float (single-precision)" :default 0.0) (`Distance to obstacle on the left` :type "Float (single-precision)" :default 0.0) (`Distance to obstacle on the right` :type "Float (single-precision)" :default 0.0) (HowToTurn :type "/Game/Blueprint/Enemy/E_HowToTurn Enum") (`Front left has obstacle` :type Boolean :default false) (`Front right has obstacle` :type Boolean :default false) (`Distance to obstacle Front` :type "Float (single-precision)" :default 0.0) (LeftAvoidForce :type "Float (double-precision)") (RightAvoidForce :type "Float (double-precision)") (TurnValue :type "Float (double-precision)"))
  (bind _sphere_front (`self.Sphere_Front`))
  (bind _sphere_left (`self.Sphere_Left`))
  (bind _sphere_right (`self.Sphere_Right`))
  (bind _sphere_left1 (`self.Sphere_Left1`))
  (bind _sphere_right1 (`self.Sphere_Right1`))
  (bind _returnvalue (`SceneComponent.K2_GetComponentLocation` _sphere_right))
  (bind _returnvalue_2 (`SceneComponent.K2_GetComponentLocation` _sphere_left))
  (bind _returnvalue_3 (`SceneComponent.K2_GetComponentLocation` _sphere_left1))
  (bind _returnvalue_4 (`SceneComponent.K2_GetComponentLocation` _sphere_front))
  (bind _returnvalue_5 (`SceneComponent.K2_GetComponentLocation` _sphere_right1))
  (bind _returnvalue_6 (>= (`local.Distance to obstacle on the left front`) (`local.Distance to obstacle on the right front`)))
  ; 向前的射线，检测面前是否有障碍物
  (bind (_outhit _returnvalue_7) (`KismetSystemLibrary.LineTraceSingle` _returnvalue_4 (+ _returnvalue_4 (* (`SceneComponent.GetForwardVector` _sphere_front) 5000.0)) "TraceTypeQuery1"))
  (bind _output_get (set `local.Are there any obstacles?` _returnvalue_7))
  (set `local.Distance to obstacle Front` (`.Distance` (`GameplayStatics.BreakHitResult` _outhit)))
  ; 左前方射线
  (bind (_outhit_2 _returnvalue_8) (`KismetSystemLibrary.LineTraceSingle` _returnvalue_2 (+ _returnvalue_2 (* (`SceneComponent.GetForwardVector` _sphere_left) 5000.0)) "TraceTypeQuery1"))
  (set `local.Front left has obstacle` _returnvalue_8)
  (if _returnvalue_8
    (set `local.Distance to obstacle on the left front` (`.Distance` (`GameplayStatics.BreakHitResult` _outhit_2)))
    (else
      (set `local.Distance to obstacle on the left front` 5000.0)))
  ; 右前方射线
  (bind (_outhit_3 _returnvalue_9) (`KismetSystemLibrary.LineTraceSingle` _returnvalue (+ _returnvalue (* (`SceneComponent.GetForwardVector` _sphere_right) 5000.0)) "TraceTypeQuery1"))
  (set `local.Front right has obstacle` _returnvalue_9)
  (if _returnvalue_9
    (set `local.Distance to obstacle on the right front` (`.Distance` (`GameplayStatics.BreakHitResult` _outhit_3)))
    (else
      (set `local.Distance to obstacle on the right front` 5000.0)))
  ; 检测正左方的距离
  (bind _outhit_4 (`KismetSystemLibrary.LineTraceSingle` _returnvalue_3 (+ _returnvalue_3 (* (`SceneComponent.GetRightVector` _sphere_left1) -3000.0)) "TraceTypeQuery1"))
  (bind _output_get_2 (set `local.Distance to obstacle on the left` (`.Distance` (`GameplayStatics.BreakHitResult` _outhit_4))))
  (set `self.LeftDistance` _output_get_2)
  ; 检测正右边距离
  (bind _outhit_5 (`KismetSystemLibrary.LineTraceSingle` _returnvalue_5 (+ _returnvalue_5 (* (`SceneComponent.GetRightVector` _sphere_right1) 3000.0)) "TraceTypeQuery1"))
  (bind _output_get_3 (set `local.Distance to obstacle on the right` (`.Distance` (`GameplayStatics.BreakHitResult` _outhit_5))))
  (set `self.RightDistance` _output_get_3)
  ; 开始行为判定
  ;; 检测面前是否有障碍物，若无则正常行驶
  (if (`local.Are there any obstacles?`)
    ;; 二级判断，如果需要拐弯，看左右前方哪里可以没障碍物
    (if _returnvalue_6
      (if (`local.Front left has obstacle`)
        (if _returnvalue_6
          (bind _output_get_4 (set `local.HowToTurn` "NewEnumerator0"))
          (`self.EnemyHowToTurn` _output_get_4)
          (else
            (set `local.HowToTurn` "NewEnumerator1" :!label _label)
            ;; 三级判断，检测转弯方向是否为墙壁，避免穿墙
            (switch `/Game/Blueprint/Enemy/E_HowToTurn` (`local.HowToTurn`) :!label _label_2
              (:`NewEnumerator1`
                (if (< (`local.Distance to obstacle on the left`) 250.0)
                  (bind _output_get_5 (set `local.HowToTurn` "NewEnumerator2"))
                  (`self.EnemyHowToTurn` _output_get_5)
                  (else
                    (`self.EnemyHowToTurn` (`local.HowToTurn`)))))
              (:`NewEnumerator2`
                (if (< (`local.Distance to obstacle on the right`) 250.0)
                  (bind _output_get_6 (set `local.HowToTurn` "NewEnumerator1"))
                  (`self.EnemyHowToTurn` _output_get_6)
                  (else
                    (`self.EnemyHowToTurn` (`local.HowToTurn`))))))))
        (else
          (goto _label)))
      (elif (`local.Front right has obstacle`)
        (if (not _returnvalue_6)
          (bind _output_get_7 (set `local.HowToTurn` "NewEnumerator0"))
          (`self.EnemyHowToTurn` _output_get_7)
          (else
            (set `local.HowToTurn` "NewEnumerator2" :!label _label_3)
            (goto _label_2)))
        (else
          (goto _label_3))))
    (else
      (bind _output_get_8 (set `local.HowToTurn` "NewEnumerator0"))
      (`self.EnemyHowToTurn` _output_get_8))))

(fn `UserConstructionScript`)