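; Bus boss for a motorcycle chase that drives forward after a timeline entrance, deploys manager-supplied obstacle items and punishes player collisions.
; Looping timers drive its attacks: blinking danger zones sized by box traces before dealing overlap damage, and two machine guns that track, lock, then fire line traces.
; Health thresholds knock off each gun and trigger a tumbling death, with dispatchers reporting damage, item requests and the fight's end.
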(event `BossStart`
  (bind _player (`self.Player`))
  (bind _baselocation (`self.BaseLocation`))
  ; 启动
  (`GameplayStatics.PlaySoundAtLocation` "/Game/Art/Voice/出场2.出场2" (`SceneComponent.K2_GetComponentLocation` (`self.BaseLocation`)) (struct) 1.0 1.0 0.0 null null null null)
  (`/Game/Blueprint/Player/BP_MotorcycleCharacter.PlayBossAnim` _player)
  (set `/Game/Blueprint/Player/BP_MotorcycleCharacter.isStartToPlay` false _player)
  (bind (_direction `_新建轨道_1` `_新建轨道_2`) (`Timeline|时间轴` :!via `PlayFromStart`)
    (:`Update`
      (`SceneComponent.K2_SetWorldLocation` _baselocation (`KismetMathLibrary.TransformLocation` (`self.GetTransform` self) (`KismetMathLibrary.VLerp` (-8000.0 1500.0 0.0) (0.0 0.0 0.0) `_新建轨道_1`)) false false)
      (`SceneComponent.K2_SetWorldRotation` _baselocation (`KismetMathLibrary.MakeRotator` 0.0 0.0 (`KismetMathLibrary.Lerp` 90.0 0.0 `_新建轨道_2`)) false false))
    (:`Finished`
      (`self.GameIsStart`)
      (set `/Game/Blueprint/Player/BP_MotorcycleCharacter.isStartToPlay` true _player)
      (set `self.Preparations complete` true))))

(event `/Game/Blueprint/Enemy/BPI_CallItemState.SetActor`
  (params (Item :type "Actor Object Reference"))
  (set `self.AttachActor` Item))

(event `/Game/Blueprint/Enemy/BPI_CallItemState.StopMovement`
  (params (`Stop?` :type Boolean))
  (if `Stop?`
    (set `self.isAction` false)
    (`KismetSystemLibrary.K2_PauseTimerHandle` (`self.PutRandomItemTimer`))
    (`KismetSystemLibrary.K2_PauseTimerHandle` (`self.AttackTimer`))
    (`self.ResetBoss`)
    (else
      (set `self.isAction` true)
      (set `self.Health` (`self.MaxHealth`))
      (set `self.Speed` (`self.MaxSpeed`))
      (`self.BossStart`)
      (`PrimitiveComponent.SetCollisionEnabled` (`self.Box`) "QueryOnly"))))

(event `GameIsStart`
  (bind _returnvalue (`KismetSystemLibrary.K2_SetTimerDelegate` (`|CreateDelegate` :!event `Attack`) 20.0 true))
  (set `self.AttackTimer` _returnvalue)
  (bind _returnvalue_2 (`KismetSystemLibrary.K2_SetTimerDelegate` (`|CreateDelegate` :!event `MechinGunShooting`) 5.0 true))
  (set `self.MechingunAttackTimer` _returnvalue_2)
  (`self.RandomPutItem`))

(event `self.ReceiveBeginPlay`
  (`parent.ReceiveBeginPlay`)
  (`|ExecutionSequence`
    (:`then_0`
      (bind _asbp_motorcycle_character (cast `/Game/Blueprint/Player/BP_MotorcycleCharacter` (`GameplayStatics.GetPlayerPawn` 0)))
      (set `self.Player` _asbp_motorcycle_character)
      (set `self.DamageAreaLocationArray` (`|MakeArray` (`self.DAL_1`) (`self.DAL_2`) (`self.DAL_3`)))
      (set `self.GoodLocatioArray` (`|MakeArray` (`self.GoodL_1`) (`self.GoodL_2`) (`self.GoodL_3`)))
      (set `self.SpawnPointLocationArray` (`|MakeArray` (`self.SP_1`) (`self.SP_2`) (`self.SP_3`)))
      (set `self.TargetPointLocationArray` (`|MakeArray` (`self.SP_6`) (`self.SP_4`) (`self.SP_5`)))
      (set `self.MechinGunArray` (`|MakeArray` (`self.train__1`) (`self.train__`)))
      (bind _output_get (set `self.DamageAreaArray` (`|MakeArray` (`self.DA_1`) (`self.DA_2`) (`self.DA_3`))))
      (for _array_element _output_get
        (`SceneComponent.SetVisibility` _array_element false false)))))

(event `self.ReceiveTick`
  (params (DeltaSeconds :type "Float (single-precision)"))
  (`parent.ReceiveTick` DeltaSeconds)
  (if (`self.isAction`)
    (`self.K2_AddActorWorldOffset` (* (* (`KismetMathLibrary.Vector_Forward`) (`self.Speed`)) DeltaSeconds))))

(event `Attack`
  ; 开始攻击
  (set `self.DMTime` 0.0)
  (set `self.isAlpha` false)
  (`self.DANote`)
  (bind _returnvalue (`KismetSystemLibrary.K2_SetTimerDelegate` (delegate `CheckDangerArea`) 0.1 true))
  (set `self.DangerAreaAttackTimer` _returnvalue)
  (`self.ResetDangerNote#`))

(event `RandomPutItem`
  ; 获取物品，从boss下面运出，然后放置在场景当中作为玩家的障碍物
  (bind _returnvalue (`KismetSystemLibrary.K2_SetTimerDelegate` (delegate `SetGoodLocation`) 1.5 true))
  (set `self.PutRandomItemTimer` _returnvalue))

(event `CheckDangerArea`
  (bind _returnvalue (+ (`self.DMTime`) 0.1))
  ; 每0.1s的时候，检测一次发射点到设定距离，有没有遮挡，若有遮挡，就缩短距离
  ;; 检测是否到时间，到时间就造成伤害，取消显示危险区域
  (if (>= _returnvalue (`self.MaxsDMTime`))
    (`KismetSystemLibrary.K2_PauseTimerHandle` (`self.DangerAreaAttackTimer`))
    (`KismetSystemLibrary.K2_PauseTimerHandle` (`self.DangerNoteTimer`))
    (`self.DMStartAttack`)
    (else
      (set `self.DMTime` _returnvalue)
      ;; 检测是否到了闪烁警告时间，到了就开始闪烁警告
      (if (>= _returnvalue (- (`self.MaxsDMTime`) 1.0))
        (`self.DangerNote`))
      ;; 这俩是记录每一个警告区域的中心位置和尺寸，在开始检查时候先清除
      (`KismetArrayLibrary.Array_Clear` (`self.DMLocation`))
      (`KismetArrayLibrary.Array_Clear` (`self.DMScaleVector`))
      (for (_array_element _array_index) (`self.DamageAreaLocationArray`)
        (bind _output_get (set `self.CurrentDamageAreaLocation` _array_element))
        (bind _returnvalue_2 (`SceneComponent.K2_GetComponentLocation` _output_get))
        (bind _returnvalue_3 (+ _returnvalue_2 (* (`SceneComponent.GetForwardVector` _output_get) -20000.0)))
        ;; 从发射点开始，朝-20000的位置发射盒体检测
        (bind _outhit (`KismetSystemLibrary.BoxTraceSingle` _returnvalue_2 _returnvalue_3 (100.0 500.0 50.0) (struct) "TraceTypeQuery1" false (`|MakeArray` (`self.Player`) :!type "Actor Object Reference")))
        (bind _output (`|GetArrayItem` (`self.DamageAreaArray`) _array_index))
        (bind (_bblockinghit _binitialoverlap _time _distance _location _impactpoint _normal _impactnormal _physmat _hitactor _hitcomponent _hitbonename _bonename _hititem _elementindex _faceindex _tracestart) (`GameplayStatics.BreakHitResult` _outhit))
        (bind _returnvalue_4 (`KismetMathLibrary.VLerp` _returnvalue_2 _returnvalue_3 _time))
        (bind _returnvalue_5 (/ (+ _tracestart _returnvalue_4) 2.0))
        ;; 用发射点与命中点相加然后除2，计算中心点位置
        (`SceneComponent.K2_SetWorldLocation` _output _returnvalue_5 false false)
        (`KismetArrayLibrary.Array_Add` (`self.DMLocation`) _returnvalue_5)
        (`SceneComponent.K2_SetWorldRotation` _output (`KismetMathLibrary.FindLookAtRotation` _tracestart _returnvalue_4) false false)
        (bind _returnvalue_6 (/ (`KismetMathLibrary.VSize` (- _returnvalue_4 _tracestart)) 100.0))
        (bind (_returnvalue_x _returnvalue_y _returnvalue_z) (`KismetMathLibrary.BreakVector` (`SceneComponent.K2_GetComponentScale` _output)))
        (`SceneComponent.SetWorldScale3D` _output (`KismetMathLibrary.MakeVector` _returnvalue_6 _returnvalue_y _returnvalue_z))
        (`KismetArrayLibrary.Array_Add` (`self.DMScaleVector`) (`KismetMathLibrary.MakeVector` _returnvalue_6 _returnvalue_y _returnvalue_z))))))

(event `SetGoodLocation`
  (bind _randomgoodlocationindex (`self.RandomGoodLocationIndex`))
  (bind _attachactor (`self.AttachActor`))
  (bind (_returnvalue_x _returnvalue_y _returnvalue_z) (`KismetMathLibrary.BreakVector` (`SceneComponent.K2_GetComponentLocation` (`|GetArrayItem` (`self.TargetPointLocationArray`) _randomgoodlocationindex))))
  (bind (_returnvalue_x_2 _returnvalue_y_2 _returnvalue_z_2) (`KismetMathLibrary.BreakVector` (`SceneComponent.K2_GetComponentLocation` (`|GetArrayItem` (`self.SpawnPointLocationArray`) _randomgoodlocationindex))))
  ; 获取物品，从boss下面运出，然后放置在场景当中作为玩家的障碍物
  ;; 随机获取三个点位的其中一个，然后告知manager，获取随机物品附加
  (set `self.RandomGoodLocationIndex` (`KismetMathLibrary.RandomIntegerInRange` 0 2))
  (`self.AttachItemToGoodLocation` (`|GetArrayItem` (`self.GoodLocatioArray`) (`self.RandomGoodLocationIndex`)))
  (bind (_direction _newtrack_0) (`Timeline|Timeline` :!via `PlayFromStart`)
    (:`Update`
      (`SceneComponent.K2_SetWorldLocation` (`|GetArrayItem` (`self.GoodLocatioArray`) (`self.RandomGoodLocationIndex`)) (`KismetMathLibrary.MakeVector` (`KismetMathLibrary.Lerp` _returnvalue_x_2 _returnvalue_x (.x _newtrack_0)) (`KismetMathLibrary.Lerp` _returnvalue_y_2 _returnvalue_y (.y _newtrack_0)) (`KismetMathLibrary.Lerp` _returnvalue_z_2 _returnvalue_z (.z _newtrack_0))) false false))
    (:`Finished`
      (`/Engine/EditorBlueprintResources/StandardMacros.IsValid` _attachactor
        (:`Is Valid`
          (`self.K2_DetachFromActor` _attachactor "KeepWorld" "KeepWorld" "KeepWorld"))))))

(event `DangerNote`
  ; 开始提示危险区域的时候激活，危险区域会闪烁
  (`/Engine/EditorBlueprintResources/StandardMacros.DoOnce` false :!label _label
    (:`Completed`
      (bind _returnvalue (`KismetSystemLibrary.K2_SetTimerDelegate` (delegate `DANote`) 0.1 true))
      (set `self.DangerNoteTimer` _returnvalue))))

(event `ResetDangerNote#`
  ; 开始提示危险区域的时候激活，危险区域会闪烁
  (goto _label :!via `Reset`))

(event `MechinGunShooting`
  ; 简单子弹射击系统
  (set `self.mechingunAimmingValue` 0.0)
  (bind _returnvalue (`KismetSystemLibrary.K2_SetTimerDelegate` (delegate `BulletShooting`) 0.05 true))
  (set `self.ShootingTimer` _returnvalue)
  (`self.ShowAimming` true))

(event `DANote`
  ; 开始提示危险区域的时候激活，危险区域会闪烁
  (if (`self.isAlpha`)
    (set `self.isAlpha` false)
    (else
      (set `self.isAlpha` true)))
  (for _array_element (`self.DamageAreaArray`)
    (`SceneComponent.SetVisibility` _array_element (`self.isAlpha`) false)))

(event `DMStartAttack`
  ; 在时间结束后，三个危险区域开始轮流对区域内生物造成伤害
  (for (_array_element _array_index) (`self.DamageAreaArray`)
    (bind _output (`|GetArrayItem` (`self.DMLocation`) _array_index))
    (bind _output_x (`KismetMathLibrary.BreakVector` (`|GetArrayItem` (`self.DMScaleVector`) _array_index)))
    (bind _returnvalue (* _output_x 50.0))
    (bind _outactors (`KismetSystemLibrary.BoxOverlapActors` _output (`KismetMathLibrary.MakeVector` _returnvalue 500.0 50.0) (`|MakeArray` "ObjectTypeQuery3" :!type "EObjectTypeQuery Enum") null (`|MakeArray` self :!type "Actor Object Reference")))
    (`KismetSystemLibrary.DrawDebugBox` _output (`KismetMathLibrary.MakeVector` _returnvalue 500.0 50.0) (struct :`R` 1.0 :`A` 1.0) (struct) 10.0 10.0)
    (`SceneComponent.SetVisibility` _array_element false false)
    (for _array_element_2 _outactors
      (`GameplayStatics.ApplyDamage` _array_element_2 30.0)
      (if (== _array_element_2 (`self.Player`))
        (message `/Game/Blueprint/Player/PlayerScoreSystem/BPI_PlayerGetScore.PlayerGetScore` (`self.Player`) "NewEnumerator2" "遭遇区域攻击" 0.0)))))

(event `BulletShooting`
  (bind _cylinder6 (`self.Cylinder6`))
  (bind (_returnvalue_x _returnvalue_y) (`KismetMathLibrary.BreakVector` (`SceneComponent.K2_GetComponentScale` _cylinder6)))
  (bind _returnvalue (+ (`self.mechingunAimmingValue`) 0.05))
  (bind _returnvalue_2 (`SceneComponent.K2_GetComponentLocation` (`|GetArrayItem` (`self.MechinGunArray`) (`self.MechinGunIndex`))))
  (bind _returnvalue_3 (`SceneComponent.K2_GetComponentLocation` (`|GetArrayItem` (`self.MechinGunArray`) (`self.MechinGunIndex`))))
  (bind _returnvalue_4 (+ _returnvalue_2 (* (`KismetMathLibrary.Normal` (- (`self.K2_GetActorLocation` (`self.Player`)) (`SceneComponent.K2_GetComponentLocation` (`|GetArrayItem` (`self.MechinGunArray`) (`self.MechinGunIndex`))))) 20000.0)))
  ; 简单子弹射击系统
  (if (`self.isBMechinGun?`)
    (set `self.MechinGunIndex` 1)
    (if (`self.weaponBCanShoot?`)
      (if (>= _returnvalue 2.0) :!label _label_2
        ;; 造成伤害
        (`KismetSystemLibrary.K2_PauseTimerHandle` (`self.ShootingTimer`))
        (bind _outhit (`KismetSystemLibrary.LineTraceSingle` :`Start` _returnvalue_3 :`End` (+ _returnvalue_3 (* (`KismetMathLibrary.Normal` (- (`KismetMathLibrary.TransformLocation` (`self.GetTransform` self) (`self.LockedRelativeLocation`)) _returnvalue_3)) 20000.0)) :`TraceChannel` "TraceTypeQuery1" :`DrawDebugType` "ForDuration"))
        (bind (_bblockinghit _binitialoverlap _time _distance _location _impactpoint _normal _impactnormal _physmat _hitactor) (`GameplayStatics.BreakHitResult` _outhit))
        (`GameplayStatics.ApplyDamage` _hitactor 30.0)
        (if (== _hitactor (`self.Player`))
          (message `/Game/Blueprint/Player/PlayerScoreSystem/BPI_PlayerGetScore.PlayerGetScore` (`self.Player`) "NewEnumerator2" "被Boss武器击中" 0.0))
        (if (`self.isBMechinGun?`)
          (set `self.isBMechinGun?` false)
          (`self.ShowAimming` false)
          (else
            (set `self.isBMechinGun?` true)
            (`self.MechinGunShooting`)))
        (else
          (set `self.mechingunAimmingValue` _returnvalue)
          (if (>= (`self.mechingunAimmingValue`) 1.5)
            (`self.AimmingLocking`)
            (else
              ;; 瞄准阶段
              (bind _outhit_2 (`KismetSystemLibrary.LineTraceSingle` _returnvalue_2 _returnvalue_4 "TraceTypeQuery1"))
              (bind (_bblockinghit_2 _binitialoverlap_2 _time_2 _distance_2 _location_2) (`GameplayStatics.BreakHitResult` _outhit_2))
              (`SceneComponent.K2_SetWorldLocation` (`self.Sphere`) _location_2 false false)
              (bind _returnvalue_5 (`KismetMathLibrary.VLerp` _returnvalue_2 _returnvalue_4 _time_2))
              (`SceneComponent.K2_SetWorldLocation` _cylinder6 (/ (+ _returnvalue_2 _returnvalue_5) 2.0) false false)
              (`SceneComponent.K2_SetWorldRotation` _cylinder6 (`KismetMathLibrary.MakeRotFromZ` (`KismetMathLibrary.Normal` (- _returnvalue_5 _returnvalue_2))) false false)
              (`SceneComponent.SetWorldScale3D` _cylinder6 (`KismetMathLibrary.MakeVector` _returnvalue_x _returnvalue_y (/ _distance_2 100.0)))
              (set `self.AimmingLocation` _returnvalue_5)
              (set `self.LockedRelativeLocation` (`KismetMathLibrary.InverseTransformLocation` (`self.GetTransform` self) (`self.AimmingLocation`)))))))
      (else
        (`KismetSystemLibrary.K2_PauseTimerHandle` (`self.ShootingTimer`))
        (`self.ShowAimming` false)))
    (else
      (set `self.MechinGunIndex` 0)
      (if (`self.weaponACanShoot?`)
        (goto _label_2)
        (else
          (set `self.isBMechinGun?` true)
          (`self.MechinGunShooting`))))))

(event `/Game/Blueprint/Enemy/Base/BPI_PutInformation.BaseInformation`
  (params (Player :type "/Game/Blueprint/Player/BP_MotorcycleCharacter Object Reference") (Manager :type "/Game/Blueprint/Manager/BP_LevelManager Object Reference"))
  ; bind event给manager
  ;; 每次运输item的时候，从manager的item array里随机获取一个物品
  (add `self.AttachItemToGoodLocation` (`|CreateDelegate` Manager :!event `AttackItemToBus`))
  ;; 当boss每次造成伤害时，告知manager，再由manager告知玩家的UI
  (add `self.BossDamage` (`|CreateDelegate` Manager :!event `UpdateBossHealth`))
  (add `self.isEndEvent` (`|CreateDelegate` Manager :!event `EndGameEvent`))
  (add `self.Escape Players` (`|CreateDelegate` Manager :!event `EnemyIsEscape`)))

(event `ResetBoss`
  (bind _train__ (`self.train__`))
  (bind _train___2 (`self.train__`))
  (bind _train__1 (`self.train__1`))
  (bind _train__1_2 (`self.train__1`))
  (`|ExecutionSequence`
    (:`then_0`
      (`|ExecutionSequence`
        (:`then_0`
          (goto _label_3 :!via `Reset`))
        (:`then_1`
          (goto _label_4 :!via `Reset`))
        (:`then_2`
          (goto _label_5 :!via `Reset`))))
    (:`then_1`
      (`SceneComponent.K2_SetWorldLocationAndRotation` :`self` (`self.BaseLocation`) :`NewLocation` (`KismetMathLibrary.TransformLocation` (`self.GetTransform` self))))
    (:`then_2`
      (`SceneComponent.K2_AttachToComponent` _train___2 (`self.BaseLocation`) "None" "KeepWorld" "KeepWorld" "KeepWorld" true)
      (`SceneComponent.K2_SetWorldLocationAndRotation` :`self` _train___2 :`NewLocation` (`SceneComponent.K2_GetComponentLocation` (`self.WBL`)))
      (`SceneComponent.K2_AttachToComponent` _train__1_2 (`self.BaseLocation`) "None" "KeepWorld" "KeepWorld" "KeepWorld" true)
      (`SceneComponent.K2_SetWorldLocationAndRotation` :`self` _train__1_2 :`NewLocation` (`SceneComponent.K2_GetComponentLocation` (`self.WAL`))))
    (:`then_3`
      (set `self.weaponACanShoot?` true)
      (set `self.weaponBCanShoot?` true))
    (:`then_4`
      (`PrimitiveComponent.SetCollisionEnabled` (`self.Box`) "QueryOnly"))))

(event `AimmingLocking`
  (if (`self.showAim`)
    (set `self.showAim` false)
    (else
      (set `self.showAim` true)))
  (`self.ShowAimming` (`self.showAim`)))

(event `BossIsDie`
  (bind _baselocation (`self.BaseLocation`))
  ; boss死亡效果
  (set `self.Preparations complete` false)
  (`PrimitiveComponent.SetCollisionEnabled` (`self.Box`) "NoCollision")
  (`KismetSystemLibrary.K2_PauseTimerHandle` (`self.AttackTimer`))
  (`KismetSystemLibrary.K2_PauseTimerHandle` (`self.MechingunAttackTimer`))
  (`KismetSystemLibrary.K2_PauseTimerHandle` (`self.PutRandomItemTimer`))
  (bind (_direction _l_z _rx _ry _rz) (`Timeline|时间轴_0` :!via `PlayFromStart`)
    (:`Update`
      (`SceneComponent.K2_SetWorldLocation` _baselocation (`KismetMathLibrary.TransformLocation` (`self.GetTransform` self) (`KismetMathLibrary.MakeVector` 0.0 0.0 (`KismetMathLibrary.Lerp` 0.0 217.0 _l_z))) false false)
      (`SceneComponent.K2_SetWorldRotation` _baselocation (`KismetMathLibrary.MakeRotator` (`KismetMathLibrary.Lerp` 0.0 142.0 _rx) (`KismetMathLibrary.Lerp` 0.0 80.0 _ry) (`KismetMathLibrary.Lerp` 0.0 180.0 _rz)) false false))
    (:`Finished`
      (bind (_direction_2 `_新建轨道_0`) (`Timeline|时间轴_1` :!via `PlayFromStart`)
        (:`Update`
          (set `self.Speed` (`KismetMathLibrary.Lerp` 10000.0 0.0 `_新建轨道_0`)))
        (:`Finished`
          (`self.isEndEvent`)
          (`self.Escape Players` self))))))

(event `ShowAimming`
  (params (`show?` :type Boolean))
  (bind _sphere (`self.Sphere`))
  (if `show?`
    (`SceneComponent.SetVisibility` _sphere true false)
    (`SceneComponent.SetVisibility` (`self.Cylinder6`) true false)
    (else
      (`SceneComponent.SetVisibility` _sphere false false)
      (`SceneComponent.SetVisibility` (`self.Cylinder6`) false false))))

(event `self.ReceiveAnyDamage`
  (params (Damage :type "Float (single-precision)") (DamageType :type "DamageType Object Reference") (InstigatedBy :type "Controller Object Reference") (DamageCauser :type "Actor Object Reference"))
  (bind _train__ (`self.train__`))
  (bind _train__1 (`self.train__1`))
  (bind _health (`self.Health`))
  (bind _returnvalue (/ _health (`self.MaxHealth`)))
  ; 受到伤害
  (bind _output_get (set `self.Health` (- (`self.Health`) Damage)))
  (`self.BossDamage` _output_get (`self.MaxHealth`))
  (if (<= _health 0.0)
    (`/Engine/EditorBlueprintResources/StandardMacros.DoOnce` false :!label _label_3
      (:`Completed`
        (`self.BossIsDie`)
        (message `/Game/Blueprint/Player/PlayerScoreSystem/BPI_PlayerGetScore.PlayerGetScore` (`self.Player`) "NewEnumerator0" "击杀Boss！+10000分" 10000.0)))
    (elif (<= _returnvalue 0.3)
      (`/Engine/EditorBlueprintResources/StandardMacros.DoOnce` false :!label _label_4
        (:`Completed`
          (`SceneComponent.K2_DetachFromComponent` _train__ "KeepWorld" "KeepWorld" "KeepWorld" true)
          (set `self.weaponBCanShoot?` false)
          (`PrimitiveComponent.SetSimulatePhysics` _train__ true)
          (message `/Game/Blueprint/Player/PlayerScoreSystem/BPI_PlayerGetScore.PlayerGetScore` (`self.Player`) "NewEnumerator0" "将Boss武器打落！+2000分" 2000.0)))
      (elif (<= _returnvalue 0.6)
        (`/Engine/EditorBlueprintResources/StandardMacros.DoOnce` false :!label _label_5
          (:`Completed`
            (`SceneComponent.K2_DetachFromComponent` _train__1 "KeepWorld" "KeepWorld" "KeepWorld" true)
            (set `self.weaponACanShoot?` false)
            (`PrimitiveComponent.SetSimulatePhysics` _train__1 true)
            (message `/Game/Blueprint/Player/PlayerScoreSystem/BPI_PlayerGetScore.PlayerGetScore` (`self.Player`) "NewEnumerator0" "将Boss武器打落！+2000分" 2000.0)))))))

(event `self.Box1.OnComponentBeginOverlap`
  (params (OverlappedComponent :type "PrimitiveComponent Object Reference") (OtherActor :type "Actor Object Reference") (OtherComp :type "PrimitiveComponent Object Reference") (OtherBodyIndex :type Integer) (bFromSweep :type Boolean) (SweepResult :type "HitResult Structure (by ref)"))
  (bind _player (`self.Player`))
  (if (== OtherComp (`Character.CapsuleComponent` _player))
    (`GameplayStatics.ApplyDamage` _player 10.0)
    (message `/Game/Blueprint/Player/PlayerScoreSystem/BPI_PlayerGetScore.PlayerGetScore` (`self.Player`) "NewEnumerator2" "被Boss追尾！离后面的Boss太近啦！" 0.0)
    (`Character.LaunchCharacter` _player (* (`self.GetActorForwardVector` _player) 10000.0) false false)))

(event `self.Box2.OnComponentBeginOverlap`
  (params (OverlappedComponent :type "PrimitiveComponent Object Reference") (OtherActor :type "Actor Object Reference") (OtherComp :type "PrimitiveComponent Object Reference") (OtherBodyIndex :type Integer) (bFromSweep :type Boolean) (SweepResult :type "HitResult Structure (by ref)"))
  (bind _player (`self.Player`))
  (if (`self.Preparations complete`)
    (if (== OtherComp (`Character.CapsuleComponent` _player))
      (`GameplayStatics.ApplyDamage` _player 10.0)
      (message `/Game/Blueprint/Player/PlayerScoreSystem/BPI_PlayerGetScore.PlayerGetScore` (`self.Player`) "NewEnumerator2" "与Boss撞车！离前面的Boss太近啦！" 0.0)
      (`Character.LaunchCharacter` _player (* (`self.GetActorForwardVector` _player) -5000.0) false false))))

(fn `UserConstructionScript`
  (`parent.UserConstructionScript`))