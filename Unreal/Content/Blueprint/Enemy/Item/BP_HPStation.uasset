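; BP_HPStation is a repair-zone pickup that restores health and awards score when the motorcycle character passes through it.
; Its Box overlap casts the other actor to BP_MotorcycleCharacter and responds only when the capsule component is what overlapped.
; It then calls AddHealth and sends a Chinese score message announcing the repair bonus.
; Nothing disables or destroys the station, so each new overlap grants the reward again.
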(event `self.Box.OnComponentBeginOverlap`
  (params (OverlappedComponent :type "PrimitiveComponent Object Reference") (OtherActor :type "Actor Object Reference") (OtherComp :type "PrimitiveComponent Object Reference") (OtherBodyIndex :type Integer) (bFromSweep :type Boolean) (SweepResult :type "HitResult Structure (by ref)"))
  (bind _asbp_motorcycle_character (cast `/Game/Blueprint/Player/BP_MotorcycleCharacter` OtherActor))
  (if (== OtherComp (`Character.CapsuleComponent` _asbp_motorcycle_character))
    (`/Game/Blueprint/Player/BP_MotorcycleCharacter.AddHealth` _asbp_motorcycle_character 20.0)
    (message `/Game/Blueprint/Player/PlayerScoreSystem/BPI_PlayerGetScore.PlayerGetScore` OtherActor "NewEnumerator1" "经过维修区！加100分！加20健康值！" 100.0)))

(fn `UserConstructionScript`
  (`parent.UserConstructionScript`))