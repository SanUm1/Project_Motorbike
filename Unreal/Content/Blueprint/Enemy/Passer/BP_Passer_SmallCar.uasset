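; Passing small-car obstacle that deals damage when it hits the motorcycle player and awards points for near misses.
; While IsAction is set, Tick moves it along world -X at constant, frame-rate-independent speed; a manager toggles this through the StopMovement interface event.
; The front Box applies damage behind a DoOnce that resets after a short delay.
; Box1 and Box2 send near-miss score messages when the player's capsule enters.
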(event `self.ReceiveTick`
  (params (DeltaSeconds :type "Float (single-precision)"))
  ; 简单行驶
  (if (`self.isAction`)
    (`self.K2_AddActorWorldOffset` (* (* (`KismetMathLibrary.Vector_Forward`) -8000.0) DeltaSeconds))))

(event `self.StopMovement`
  (params (`Stop?` :type Boolean))
  ; 开始或结束行驶（由Manager用BPI传递）
  (if `Stop?`
    (set `self.isAction` false)
    (else
      (set `self.isAction` true))))

(event `self.Box.OnComponentBeginOverlap`
  (params (OverlappedComponent :type "PrimitiveComponent Object Reference") (OtherActor :type "Actor Object Reference") (OtherComp :type "PrimitiveComponent Object Reference") (OtherBodyIndex :type Integer) (bFromSweep :type Boolean) (SweepResult :type "HitResult Structure (by ref)"))
  ; 头部撞击玩家
  (bind _asbp_motorcycle_character (cast `/Game/Blueprint/Player/BP_MotorcycleCharacter` OtherActor))
  (if (== OtherComp (`Character.CapsuleComponent` _asbp_motorcycle_character))
    (`/Engine/EditorBlueprintResources/StandardMacros.DoOnce` false :!label _label
      (:`Completed`
        (`KismetSystemLibrary.PrintString` "Hurt")
        (`GameplayStatics.ApplyDamage` OtherActor 10.0)
        (message `/Game/Blueprint/Player/PlayerScoreSystem/BPI_PlayerGetScore.PlayerGetScore` OtherActor "NewEnumerator2" "撞车！" 0.0)
        (`KismetSystemLibrary.Delay` 0.1)
        (`self.ResetDamage`)))))

(event `ResetDamage`
  ; 头部撞击玩家
  (goto _label :!via `Reset`))

(event `self.BaseInformation`
  (params (Player :type "/Game/Blueprint/Player/BP_MotorcycleCharacter Object Reference") (Manager :type "/Game/Blueprint/Manager/BP_LevelManager Object Reference"))
  (set `self.isAction` false))

(event `self.Box1.OnComponentBeginOverlap`
  (params (OverlappedComponent :type "PrimitiveComponent Object Reference") (OtherActor :type "Actor Object Reference") (OtherComp :type "PrimitiveComponent Object Reference") (OtherBodyIndex :type Integer) (bFromSweep :type Boolean) (SweepResult :type "HitResult Structure (by ref)"))
  (bind _asbp_motorcycle_character (cast `/Game/Blueprint/Player/BP_MotorcycleCharacter` OtherActor))
  (if (== OtherComp (`Character.CapsuleComponent` _asbp_motorcycle_character))
    (message `/Game/Blueprint/Player/PlayerScoreSystem/BPI_PlayerGetScore.PlayerGetScore` OtherActor "NewEnumerator1" "擦肩而过！+1000分" 1000.0)))

(event `self.Box2.OnComponentBeginOverlap`
  (params (OverlappedComponent :type "PrimitiveComponent Object Reference") (OtherActor :type "Actor Object Reference") (OtherComp :type "PrimitiveComponent Object Reference") (OtherBodyIndex :type Integer) (bFromSweep :type Boolean) (SweepResult :type "HitResult Structure (by ref)"))
  (bind _asbp_motorcycle_character (cast `/Game/Blueprint/Player/BP_MotorcycleCharacter` OtherActor))
  (if (== OtherComp (`Character.CapsuleComponent` _asbp_motorcycle_character))
    (message `/Game/Blueprint/Player/PlayerScoreSystem/BPI_PlayerGetScore.PlayerGetScore` OtherActor "NewEnumerator1" "擦肩而过！+1000分" 1000.0)))

(fn `UserConstructionScript`)