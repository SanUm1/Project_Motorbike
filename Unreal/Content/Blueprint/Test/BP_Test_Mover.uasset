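; BP_Test_Mover is a test actor that moves its Cube between the positions of two marker components, Sphere and Sphere1.
; From BeginPlay, the PP flag selects whether a timeline plays from the start or reverses from the end, and its track drives a world-location lerp without sweep.
; On finish, a zero-second Delay loops back to the PP check, repeating the motion; this graph never changes PP.
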(event `self.ReceiveBeginPlay`
  (if (`self.PP`) :!label _label
    (bind (_direction `_新建轨道_0`) (`Timeline|时间轴` :!via `PlayFromStart` :!label _label_2)
      (:`Update`
        (`SceneComponent.K2_SetWorldLocation` (`self.Cube`) (`KismetMathLibrary.VLerp` (`SceneComponent.K2_GetComponentLocation` (`self.Sphere`)) (`SceneComponent.K2_GetComponentLocation` (`self.Sphere1`)) `_新建轨道_0`) false false))
      (:`Finished`
        (`KismetSystemLibrary.Delay` 0.0)
        (goto _label)))
    (else
      (goto _label_2 :!via `ReverseFromEnd`))))

(fn `UserConstructionScript`)