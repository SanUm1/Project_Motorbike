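; BP_Truck_Test is a test truck actor that loops an animation alongside a moving sphere.
; BeginPlay calls the Anim event, which plays the close-door wait montage on the Kache1 mesh and calls itself again when the montage completes.
; Each cycle also snaps Sphere to Sphere2 and restarts a timeline that lerps it toward Sphere1, so the motion restarts with the montage.
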(event `self.ReceiveBeginPlay`
  (`self.Anim`))

(event `Anim`
  (`|ExecutionSequence`
    (:`then_0`
      (`|PlayMontage` (`self.kache_1`) "/Game/Art/Animation/Truck/Truck_Ainm_CloseDoor_Wait_Montage.Truck_Ainm_CloseDoor_Wait_Montage"
        (:`OnCompleted`
          (`self.Anim`))))
    (:`then_1`
      (`SceneComponent.K2_SetWorldLocation` (`self.Sphere`) (`SceneComponent.K2_GetComponentLocation` (`self.Sphere2`)) false false)
      (bind (_direction `_新建轨道_0`) (`Timeline|时间轴` :!via `PlayFromStart`)
        (:`Update`
          (`SceneComponent.K2_SetWorldLocation` (`self.Sphere`) (`KismetMathLibrary.VLerp` (`SceneComponent.K2_GetComponentLocation` (`self.Sphere2`)) (`SceneComponent.K2_GetComponentLocation` (`self.Sphere1`)) `_新建轨道_0`) false false))))))

(fn `UserConstructionScript`)