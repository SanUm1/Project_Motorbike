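; Level manager for a motorcycle tunnel run, controlling the truck launch, timed events and rest breaks.
; Pre-spawns data-table actors into tag-sorted standby pools, recycling them instead of destroying them.
; Tunnel segments leapfrog forward, placing pooled actors according to the current Normal, Special, Survival or Boss event.
; When an event ends, the base truck appears and enemies flee; recycling the truck starts the next random event, periodically a boss.
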(event `self.ReceiveBeginPlay`
  (`|ExecutionSequence`
    (:`then_0`
      (bind _asbp_motorcycle_character (cast `/Game/Blueprint/Player/BP_MotorcycleCharacter` (`GameplayStatics.GetPlayerPawn` 0)))
      (bind _output_get (set `self.Player` _asbp_motorcycle_character))
      (add `/Game/Blueprint/Player/BP_MotorcycleCharacter.GetSpawnItemAndMoveToStandbyArea` _output_get (`|CreateDelegate` :!event `MoveItemToStandbyArea`))
      (add `/Game/Blueprint/Player/BP_MotorcycleCharacter.isStart` _output_get (delegate `StartTheGame`))
      (add `/Game/Blueprint/Player/BP_MotorcycleCharacter.AllReady` _output_get (delegate `PlayerIsReady`))
      (`self.SpawnTunnel`)
      (`self.SpawnAllItem`))
    (:`then_1`
      ; 筛选事件（正常与boss
      (bind _outrownames (`DataTableFunctionLibrary.GetDataTableRowNames` "/Game/Blueprint/Enemy/Base/RandomEvent/DT_RandomEventList.DT_RandomEventList"))
      (for _array_element _outrownames
        (bind _returnvalue (`|GetDataTableRow` "/Game/Blueprint/Enemy/Base/RandomEvent/DT_RandomEventList.DT_RandomEventList" _array_element)
          (:`then`
            (if (`|EnumEquality` (`.EventType_5_239FC33741374B9A3CE9488B24289CE1` (break `/Game/Blueprint/Enemy/Base/RandomEvent/S_RandomEventList` _returnvalue)) "NewEnumerator3")
              (`KismetArrayLibrary.Array_Add` (`self.BossEventArray`) _array_element)
              (else
                (`KismetArrayLibrary.Array_Add` (`self.NormalEventArray`) _array_element)))))))))

(event `PlayerIsReady`
  ; 在玩家创建好一切物品后，才允许开始流程（否则会比UI先创建，导致无索引
  (`self.Tutorial`)
  (add `/Game/UI/W_PlayerScoreUI.ReadyToPlay` (`/Game/Blueprint/Player/BP_MotorcycleCharacter.ScoreUI` (`self.Player`)) (delegate `Ready`)))

(event `Ready`
  (bind _basevehicle (`self.BaseVehicle`))
  ; 准备开始（一般在卡车开门时候【在教程到结束的时候，或者测试】才允许玩家操作）
  (`|ExecutionSequence`
    (:`then_0`
      (`self.ResetAndReadyToStart`)
      (`/Game/Blueprint/Player/BP_BaseVehicle.StartCar` _basevehicle)
      (`/Game/Blueprint/Player/BP_BaseVehicle.ResetCarDoor` _basevehicle)
      (set `/Game/Blueprint/Player/BP_MotorcycleCharacter.isStartToPlay` true (`self.Player`))
      (`/Game/UI/W_PlayerScoreUI.TutorialSystem` (`/Game/Blueprint/Player/BP_MotorcycleCharacter.ScoreUI` (`self.Player`)) 6))
    (:`then_1`
      (goto _label :!via `Reset`))))

(event `StartTheGame`
  ; 按下E才开始游戏（在关卡流程允许的情况下才可以）
  (`/Engine/EditorBlueprintResources/StandardMacros.DoOnce` false :!label _label
    (:`Completed`
      (`self.MotoStart`))))

(event `SpawnAllItem`
  ; 新一代创建敌人结构
  ;; 从data table读取数据，然后开始创建
  (bind _outrownames (`DataTableFunctionLibrary.GetDataTableRowNames` "/Game/Blueprint/Enemy/Base/DT_SpawerList.DT_SpawerList"))
  (for _array_element _outrownames
    (bind _returnvalue (`|GetDataTableRow` "/Game/Blueprint/Enemy/Base/DT_SpawerList.DT_SpawerList" _array_element)
      (:`then`
        (bind (_name _type _whichbp _number _tag) (break `/Game/Blueprint/Enemy/Base/S_SpawnerList` _returnvalue))
        (for _ (range _number)
          (bind _returnvalue_2 (`|SpawnActorFromClass` _whichbp (`KismetMathLibrary.MakeTransform` (0.0 0.0 5000.0)) "Undefined" "MultiplyWithRoot" null null))
          (`KismetArrayLibrary.Array_Add` (`Actor.Tags` _returnvalue_2) _tag)
          ;; 重点！！因为这个方法没法直接用bind event，所以需要用bpi把自己传过去。至于如何操作，可以看enemy_1里是怎么操作的。
          (message `/Game/Blueprint/Enemy/Base/BPI_PutInformation.BaseInformation` _returnvalue_2 (`self.Player`) self)
          (switch `/Game/Blueprint/Enemy/Base/E_SpawerType` _type
            (:`NewEnumerator0`
              (bind _tags (`Actor.Tags` _returnvalue_2))
              (`KismetArrayLibrary.Array_Add` _tags "Item")
              (`KismetArrayLibrary.Array_Add` (`self.ItemStandbyArray`) _returnvalue_2))
            (:`NewEnumerator1`
              (`KismetArrayLibrary.Array_Add` _tags "Passer")
              (`KismetArrayLibrary.Array_Add` (`self.PasserStandbyArray`) _returnvalue_2))
            (:`NewEnumerator2`
              (`KismetArrayLibrary.Array_Add` _tags "Enemy")
              (`KismetArrayLibrary.Array_Add` (`self.EnemyStandbyArray`) _returnvalue_2))
            (:`NewEnumerator3`
              (`KismetArrayLibrary.Array_Add` _tags "Boss")
              (`KismetArrayLibrary.Array_Add` (`self.BossStandbyArray`) _returnvalue_2)))))))
  ;; 最后创建基地车，非常完美，毫无bug
  (bind _returnvalue_3 (`|SpawnActorFromClass` "/Game/Blueprint/Player/BP_BaseVehicle.BP_BaseVehicle_C" (`KismetMathLibrary.MakeTransform` (0.0 0.0 5000.0)) "Undefined" "MultiplyWithRoot" null null))
  (bind _output_get (set `self.BaseVehicle` _returnvalue_3))
  (set `/Game/Blueprint/Player/BP_BaseVehicle.isAction` false _output_get)
  (`KismetArrayLibrary.Array_Add` (`Actor.Tags` _output_get) "Base")
  (`self.PlayerInVehicle`))

(event `Tutorial`
  (bind _player (`self.Player`))
  (bind _basevehicle (`self.BaseVehicle`))
  ; 是否需要教程（一般都需要，下面的是直接开卡车门进行游玩，一般用于测试
  (if (`self.needTutorial?`)
    (set `/Game/Blueprint/Player/BP_MotorcycleCharacter.isStartToPlay` false _player)
    (`/Game/Blueprint/Player/BP_MotorcycleCharacter.PlayerTutorial` _player)
    (else
      ;; 测试用
      (`/Game/Blueprint/Player/BP_BaseVehicle.StartCar` _basevehicle)
      (`/Game/Blueprint/Player/BP_BaseVehicle.ResetCarDoor` _basevehicle)
      (set `/Game/Blueprint/Player/BP_MotorcycleCharacter.isStartToPlay` true (`self.Player`)))))

(event `PlayerInVehicle`
  (bind _basevehicle (`self.BaseVehicle`))
  (bind _player (`self.Player`))
  ; 在所有物品都创建好后，先把卡车传送到玩家位置，再把玩家卡在车内，准备出发
  (set `/Game/Blueprint/Player/BP_BaseVehicle.isAction` true _basevehicle)
  (set `/Game/Blueprint/Player/BP_BaseVehicle.isInAnim` true _basevehicle)
  (set `/Game/Blueprint/Player/BP_MotorcycleCharacter.isInVehicle` true _player)
  (`CharacterMovementComponent.SetMovementMode` (`Character.CharacterMovement` _player) "MOVE_None" 0)
  (`self.K2_SetActorLocation` (`self.BaseVehicle`) (`self.K2_GetActorLocation` (`self.Player`)) false false)
  (`self.K2_SetActorLocation` (`self.Player`) (`SceneComponent.K2_GetComponentLocation` (`/Game/Blueprint/Player/BP_BaseVehicle.MotoLocation` (`self.BaseVehicle`))) false false)
  (`self.K2_AttachToComponent` (`self.Player`) (`/Game/Blueprint/Player/BP_BaseVehicle.MotoLocation` (`self.BaseVehicle`)) "None" "KeepWorld" "KeepWorld" "KeepWorld" true)
  (`KismetArrayLibrary.Array_Add` (`Actor.Tags` (`self.BaseVehicle`)) "Spawn"))

(event `MotoStart`
  (bind _player (`self.Player`))
  (bind _player_2 (`self.Player`))
  ; 摩托车开始（按下e开始，一般在流程允许摩托车启动之后才可以
  (`/Engine/EditorBlueprintResources/StandardMacros.DoOnce` false :!label _label_2
    (:`Completed`
      (`|ExecutionSequence`
        (:`then_0`
          (`PlayerController.ClientStartCameraShake` :`self` (`GameplayStatics.GetPlayerController` 0) :`Shake` "/Game/Blueprint/Player/CameraShake/BP_SpeedUpCameraShake.BP_SpeedUpCameraShake_C")
          ;; 从卡车解除attach，开始行驶
          (set `/Game/Blueprint/Player/BP_MotorcycleCharacter.isInVehicle` false _player)
          (`CharacterMovementComponent.SetMovementMode` (`Character.CharacterMovement` _player) "MOVE_Walking" 0)
          (`self.K2_DetachFromActor` _player "KeepWorld" "KeepWorld" "KeepWorld")
          (bind (_direction `_新建轨道_0`) (`Timeline|时间轴` :!via `PlayFromStart`)
            (:`Update`
              (`Character.LaunchCharacter` _player_2 (* (`SceneComponent.GetForwardVector` (`Actor.RootComponent` _player_2)) (`KismetMathLibrary.Lerp` 5000.0 8000.0 `_新建轨道_0`)) true false))))
        (:`then_1`
          (`/Engine/EditorBlueprintResources/StandardMacros.DoOnce` false
            (:`Completed`
              (`AudioComponent.Play` (`/Game/Blueprint/Player/BP_MotorcycleCharacter.BGM` (`self.Player`)) 0.0))))))))

(event `ResetAndReadyToStart`
  ; 摩托车开始（按下e开始，一般在流程允许摩托车启动之后才可以
  (goto _label_2 :!via `Reset`))

(event `MoveItemToStandbyArea`
  (params (whichItem :type "Actor Object Reference") (`isBoss?` :type Boolean))
  (bind _basevehicle (`self.BaseVehicle`))
  (bind _remove_actor (`self.Remove Actor`))
  (bind _remove_actor_2 (`self.Remove Actor`))
  (bind _tags (`Actor.Tags` (`self.Remove Actor`)))
  ; 将（单个）物品转移回Standby位置（由玩家的BoxCollision控制
  (set `self.Remove Actor` whichItem)
  (`self.K2_SetActorLocation` _remove_actor (0.0 0.0 5000.0) false false :!label _label)
  (`KismetArrayLibrary.Array_RemoveItem` _tags "Spawn")
  (`KismetSystemLibrary.PrintString` (`KismetSystemLibrary.GetDisplayName` _remove_actor) true true (struct :`R` 1.0 :`G` 0.151192 :`A` 1.0))
  ;; 看Tag是谁家的，就各回各家
  (for _array_element _tags
    (if (== _array_element "Item")
      (`KismetArrayLibrary.Array_Add` (`self.ItemStandbyArray`) _remove_actor_2)
      (elif (== _array_element "Passer")
        (`KismetArrayLibrary.Array_Add` (`self.PasserStandbyArray`) _remove_actor_2)
        (elif (== _array_element "Enemy")
          (`KismetArrayLibrary.Array_Add` (`self.EnemyStandbyArray`) _remove_actor_2)
          (`KismetArrayLibrary.Array_RemoveItem` (`self.EnemyActionArray`) _remove_actor_2)
          (elif (== _array_element "Boss")
            (`KismetArrayLibrary.Array_Add` (`self.BossStandbyArray`) _remove_actor_2)
            (elif (== _array_element "Base")
              (`self.GameIsStart`)
              (set `/Game/Blueprint/Player/BP_BaseVehicle.isAction` false _basevehicle)
              (set `/Game/Blueprint/Player/BP_BaseVehicle.isInAnim` false _basevehicle)))))))
  ;; 停止进行行为，一般用于会动的物品
  (message `/Game/Blueprint/Enemy/BPI_CallItemState.StopMovement` (`self.Remove Actor`) true))

(event `EnemyIsEscape`
  (params (who :type "Actor Object Reference"))
  ; 将（单个）物品转移回Standby位置（由玩家的BoxCollision控制
  (set `self.Remove Actor` who)
  (goto _label))

(event `RemoveFromArray`
  (bind _temporary_actor (`self.Temporary Actor`))
  ; 看Tag是谁家的就从谁家赶出去
  (for _array_element (`Actor.Tags` (`self.Temporary Actor`)) :!label _label_2
    (if (== _array_element "Item")
      (`KismetArrayLibrary.Array_RemoveItem` (`self.ItemStandbyArray`) _temporary_actor)
      (elif (== _array_element "Passer")
        (`KismetArrayLibrary.Array_RemoveItem` (`self.PasserStandbyArray`) _temporary_actor)
        (elif (== _array_element "Enemy")
          (`KismetArrayLibrary.Array_RemoveItem` (`self.EnemyStandbyArray`) _temporary_actor)
          (`KismetArrayLibrary.Array_Add` (`self.EnemyActionArray`) _temporary_actor)
          (elif (== _array_element "Boss")
            (`KismetArrayLibrary.Array_RemoveItem` (`self.BossStandbyArray`) _temporary_actor))))))
  ; 需要布尔来设置启动（例如车，敌人）
  (message `/Game/Blueprint/Enemy/BPI_CallItemState.StopMovement` (`self.Temporary Actor`) false))

(event `SpawnTunnel`
  ; 创建所有隧道
  (for _index (range (+ (`self.MaxTunnelIndex`) 1))
    (bind _returnvalue (`|SpawnActorFromClass` "/Game/Blueprint/Tunnel/BP_SingleTunnel.BP_SingleTunnel_C" (`KismetMathLibrary.MakeTransform` (`KismetMathLibrary.MakeVector` (`KismetMathLibrary.Conv_IntToDouble` (* _index 5000)))) "Undefined" "MultiplyWithRoot" null null))
    (add `/Game/Blueprint/Tunnel/BP_SingleTunnel.MovingTunnel` _returnvalue (`|CreateDelegate` :!event `MoveTunnelToTop`))))

(event `NormalEvent`
  ; 普通事件
  ;; 此次意为：当场地敌人刷新超过上限，就控制RandomIntegerInRange的max值（控制需不需要刷新敌人）
  (if (>= (`KismetArrayLibrary.Array_Length` (`self.EnemyActionArray`)) (`self.MaxEnemyInAreaAtTheSameTime`))
    (set `self.MaxInteger (ForEnemySpawner)` 1)
    (else
      (set `self.MaxInteger (ForEnemySpawner)` 2)))
  ;; 随机抽取一个类型的数组、
  (switch `int` (`KismetMathLibrary.RandomIntegerInRange` 0 (`self.MaxInteger (ForEnemySpawner)`))
    (:`0`
      (set `self.Temporary Array` (`self.ItemStandbyArray`)))
    (:`1`
      (set `self.Temporary Array` (`self.PasserStandbyArray`)))
    (:`2`
      (set `self.Temporary Array` (`self.EnemyStandbyArray`)))
    (:`3`
      (set `self.Temporary Array` (`self.BossStandbyArray`))))
  ;; 打上Tag
  (bind _output_get (set `self.Temporary Actor` (`KismetArrayLibrary.Array_Random` (`self.Temporary Array`))))
  (`KismetArrayLibrary.Array_Add` (`Actor.Tags` _output_get) "Spawn")
  ; 把抽取的物品设置位置
  (`self.K2_SetActorLocation` (`self.Temporary Actor`) (`SceneComponent.K2_GetComponentLocation` (`KismetArrayLibrary.Array_Random` (`/Game/Blueprint/Tunnel/BP_SingleTunnel.SpawnPoint` (`self.Which Tunnel`)))) false false :!label _label_3)
  (goto _label_2))

(event `MoveTunnelToTop`
  (params (whichTunnel :type "/Game/Blueprint/Tunnel/BP_SingleTunnel Object Reference"))
  (bind _returnvalue_x (`KismetMathLibrary.BreakVector` (`self.K2_GetActorLocation` whichTunnel)))
  ; 当玩家走到隧道checkpoint，就把隧道移动到前面（暂时写的是不动的物品，例如路人车，障碍物）
  (set `self.Which Tunnel` whichTunnel)
  (`self.K2_SetActorLocation` whichTunnel (`KismetMathLibrary.MakeVector` (+ (* (`self.MaxTunnelIndex`) 5000) _returnvalue_x)) true false)
  ;; 控制流程，如果不需要刷新敌人，这里就为否
  (if (`self.shouldSpanwItem`)
    (bind _returnvalue (`|GetDataTableRow` "/Game/Blueprint/Enemy/Base/RandomEvent/DT_RandomEventList.DT_RandomEventList" (`self.RandomEventName`))
      (:`then`
        (bind (_eventname _eventdescription _eventtype _iteminevent _maxenemynum) (break `/Game/Blueprint/Enemy/Base/RandomEvent/S_RandomEventList` _returnvalue))
        (set `self.MaxEnemyInAreaAtTheSameTime` _maxenemynum)
        (switch `/Game/Blueprint/Enemy/Base/RandomEvent/E_EventType` _eventtype
          (:`NewEnumerator2`
            (`self.NormalEvent`))
          (:`NewEnumerator0`
            (`self.SpecialEvent`))
          (:`NewEnumerator1`
            (`self.SurvivalEvent`))
          (:`NewEnumerator3`
            (`self.BossEvent`)))))
    (else
      (`self.AddBaseCar`))))

(event `SurvivalEvent`
  ; 生存事件
  (bind _returnvalue (`|GetDataTableRow` "/Game/Blueprint/Enemy/Base/RandomEvent/DT_RandomEventList.DT_RandomEventList" (`self.RandomEventName`))
    (:`then`
      (for (_array_element _array_index) (`/Game/Blueprint/Tunnel/BP_SingleTunnel.SpawnPoint` (`self.Which Tunnel`))
        (if (== _array_index (`KismetMathLibrary.RandomIntegerInRange` 0 4))
          (bind (_itemtype0123itempasserenemyboss _itemtag) (break `/Game/Blueprint/Enemy/Base/RandomEvent/S_SingleItemInfo` (`KismetArrayLibrary.Array_Random` (`.ItemInEvent_12_B002A4DB4ACF8AE54FE9AE92943C8ADF` (break `/Game/Blueprint/Enemy/Base/RandomEvent/S_RandomEventList` _returnvalue)))))
          (switch `int` _itemtype0123itempasserenemyboss
            (:`0`
              (set `self.Temporary Array` (`self.ItemStandbyArray`)))
            (:`1`
              (set `self.Temporary Array` (`self.PasserStandbyArray`)))
            (:`2`
              (set `self.Temporary Array` (`self.EnemyStandbyArray`)))
            (:`3`
              (set `self.Temporary Array` (`self.BossStandbyArray`))))
          (for _array_element_2 (`self.Temporary Array`)
            (if (`self.ActorHasTag` _array_element_2 _itemtag)
              (bind _output_get (set `self.Temporary Actor` _array_element_2))
              (`KismetArrayLibrary.Array_Add` (`Actor.Tags` _output_get) "Spawn")
              (`self.K2_SetActorLocation` (`self.Temporary Actor`) (`SceneComponent.K2_GetComponentLocation` _array_element) false false)
              (`|ExecutionSequence`
                (:`then_0`
                  (goto _label_2))
                (:`then_1`
                  (break))))))))))

(event `SpecialEvent`
  ; 特殊事件
  (bind _returnvalue (`|GetDataTableRow` "/Game/Blueprint/Enemy/Base/RandomEvent/DT_RandomEventList.DT_RandomEventList" (`self.RandomEventName`))
    (:`then`
      (bind (_itemtype0123itempasserenemyboss _itemtag) (break `/Game/Blueprint/Enemy/Base/RandomEvent/S_SingleItemInfo` (`KismetArrayLibrary.Array_Random` (`.ItemInEvent_12_B002A4DB4ACF8AE54FE9AE92943C8ADF` (break `/Game/Blueprint/Enemy/Base/RandomEvent/S_RandomEventList` _returnvalue)))))
      (switch `int` _itemtype0123itempasserenemyboss
        (:`0`
          (set `self.Temporary Array` (`self.ItemStandbyArray`))
          (for _array_element (`self.Temporary Array`) :!label _label_4
            (if (`self.ActorHasTag` _array_element _itemtag)
              (bind _output_get (set `self.Temporary Actor` _array_element))
              (`KismetArrayLibrary.Array_Add` (`Actor.Tags` _output_get) "Spawn")
              (break)))
          (goto _label_3))
        (:`1`
          (set `self.Temporary Array` (`self.PasserStandbyArray`))
          (goto _label_4))
        (:`2`
          (set `self.Temporary Array` (`self.EnemyStandbyArray`))
          (if (not (>= (`KismetArrayLibrary.Array_Length` (`self.EnemyActionArray`)) (`self.MaxEnemyInAreaAtTheSameTime`)))
            (goto _label_4)))
        (:`3`
          (set `self.Temporary Array` (`self.BossStandbyArray`))
          (goto _label_4))))))

(event `GameIsStart`
  (bind _output_get (set `self.canEscape?` false))
  (set `/Game/Blueprint/Player/BP_MotorcycleCharacter.canEscape?` _output_get (`self.Player`))
  (bind _time (`self.ProcessControl` false))
  ; 设定该关卡的时间，一旦时间结束，则停止刷新敌人
  (message `/Game/Blueprint/Player/PlayerScoreSystem/BPI_PlayerGetScore.GameIsOver/Start` (`self.Player`) false)
  (`KismetSystemLibrary.K2_SetTimerDelegate` (delegate `GameCountdown`) (`KismetMathLibrary.Conv_IntToDouble` _time))
  (`self.ResetBaseCar`))

(event `GameCountdown`
  (bind _player (`self.Player`))
  ; 设定该关卡的时间，一旦时间结束，则停止刷新敌人
  (`self.ProcessControl` true :!label _label_5)
  (`/Game/UI/W_PlayerScoreUI.SubSystem` (`/Game/Blueprint/Player/BP_MotorcycleCharacter.ScoreUI` _player) (`KismetArrayLibrary.Array_Random` (`/Game/Blueprint/Player/BP_MotorcycleCharacter.RelaxSubIndexArray` _player)))
  (`self.ResetBossEvent`))

(event `EndGameEvent`
  (bind _player (`self.Player`))
  (bind _output_get (set `self.canEscape?` true))
  (set `/Game/Blueprint/Player/BP_MotorcycleCharacter.canEscape?` _output_get _player)
  (`/Game/Blueprint/Player/BP_MotorcycleCharacter.EndCaculate` _player)
  (goto _label_5))

(event `BossEvent`
  (bind _temporary_actor (`self.Temporary Actor`))
  (bind (_returnvalue_x _returnvalue_y _returnvalue_z) (`KismetMathLibrary.BreakVector` (`self.K2_GetActorLocation` (`self.Player`))))
  ; Boss
  (`/Engine/EditorBlueprintResources/StandardMacros.DoOnce` false :!label _label_6
    (:`Completed`
      (bind _returnvalue (`|GetDataTableRow` "/Game/Blueprint/Enemy/Base/RandomEvent/DT_RandomEventList.DT_RandomEventList" (`self.RandomEventName`))
        (:`then`
          (bind (_itemtype0123itempasserenemyboss _itemtag) (break `/Game/Blueprint/Enemy/Base/RandomEvent/S_SingleItemInfo` (`KismetArrayLibrary.Array_Random` (`.ItemInEvent_12_B002A4DB4ACF8AE54FE9AE92943C8ADF` (break `/Game/Blueprint/Enemy/Base/RandomEvent/S_RandomEventList` _returnvalue)))))
          (switch `int` _itemtype0123itempasserenemyboss
            (:`3`
              (bind _output_get (set `self.Temporary Array` (`self.BossStandbyArray`)))
              (for _array_element _output_get
                (if (`self.ActorHasTag` _array_element _itemtag)
                  (set `self.Temporary Actor` _array_element)
                  (set `self.Boss Actor` _array_element)
                  (break)))
              (`self.K2_SetActorLocation` _temporary_actor (`KismetMathLibrary.MakeVector` (+ _returnvalue_x 5000.0) 0.0 (- _returnvalue_z 100.0)) false false)
              (`/Game/Blueprint/Player/BP_MotorcycleCharacter.StartToCaculateDistination` (`self.Player`) (`self.Boss Actor`))
              (message `/Game/Blueprint/Enemy/BPI_CallItemState.StopMovement` _temporary_actor false)
              (goto _label_2))))))))

(event `ResetBossEvent`
  ; Boss
  (goto _label_6 :!via `Reset`))

(event `UpdateBossHealth`
  (params (Health :type "Float (double-precision)") (MaxHealth :type "Float (double-precision)"))
  ; Boss
  (`/Game/UI/W_PlayerScoreUI.UpdateBoss` (`/Game/Blueprint/Player/BP_MotorcycleCharacter.ScoreUI` (`self.Player`)) (/ Health MaxHealth)))

(event `AddBaseCar`
  (bind _basevehicle (`self.BaseVehicle`))
  (bind _widget2 (`/Game/Blueprint/Player/BP_BaseVehicle.Widget2` _basevehicle))
  ; 加基地车，并且所有敌人逃逸
  (`/Engine/EditorBlueprintResources/StandardMacros.DoOnce` false :!label _label_7
    (:`Completed`
      (set `self.EventIndex` (+ (`self.EventIndex`) 1))
      (`self.CheckEventIndex`)
      (message `/Game/Blueprint/Player/PlayerScoreSystem/BPI_PlayerGetScore.GameIsOver/Start` (`self.Player`) true)
      (`/Game/Blueprint/Player/BP_BaseVehicle.ResetPlayerGetScore` _basevehicle)
      (set `/Game/Blueprint/Player/BP_BaseVehicle.isAction` true _basevehicle)
      (set `/Game/Blueprint/Player/BP_BaseVehicle.isInAnim` false _basevehicle)
      (`|PlayMontage` (`/Game/Blueprint/Player/BP_BaseVehicle.kache_1` _basevehicle) "/Game/Art/Animation/Truck/Truck_Ainm_OpenDoor_Montage.Truck_Ainm_OpenDoor_Montage"
        (:`then`
          (`SceneComponent.SetVisibility` (`/Game/Blueprint/Player/BP_BaseVehicle.RectLight` _basevehicle) true false)
          (`KismetArrayLibrary.Array_Add` (`Actor.Tags` _basevehicle) "Spawn")
          (`self.K2_SetActorLocation` _basevehicle (`SceneComponent.K2_GetComponentLocation` (`KismetArrayLibrary.Array_Random` (`/Game/Blueprint/Tunnel/BP_SingleTunnel.SpawnPoint` (`self.Which Tunnel`)))) false false)
          (if (`self.canEscape?`)
            (`SceneComponent.SetVisibility` _widget2 true false)
            (`SceneComponent.SetVisibility` (`/Game/Blueprint/Player/BP_BaseVehicle.Widget3` _basevehicle) true false)
            (else
              (`SceneComponent.SetVisibility` _widget2 false false)
              (`SceneComponent.SetVisibility` (`/Game/Blueprint/Player/BP_BaseVehicle.Widget3` _basevehicle) false false)))
          (for _array_element (`self.EnemyActionArray`)
            (if (`self.ActorHasTag` _array_element "Spawn")
              (message `/Game/Blueprint/Enemy/BPI_CallItemState.Enemy fled` _array_element))))))))

(event `ResetBaseCar`
  ; 加基地车，并且所有敌人逃逸
  (goto _label_7 :!via `Reset`))

(event `CheckEventIndex`
  (if (> (`self.EventIndex`) 4)
    (set `self.EventIndex` 0)
    (set `self.isBossEvent?` true)))

(event `AttackItemToBus`
  (params (Location :type "SceneComponent Object Reference"))
  (bind _output_get (set `self.Temporary Actor` (`KismetArrayLibrary.Array_Random` (`self.ItemStandbyArray`))))
  (`KismetArrayLibrary.Array_Add` (`Actor.Tags` _output_get) "Spawn")
  (`self.K2_SetActorLocation` (`self.Temporary Actor`) (`SceneComponent.K2_GetComponentLocation` Location) false false)
  (message `/Game/Blueprint/Enemy/BPI_CallItemState.SetActor` (`self.Boss Actor`) _output_get)
  (`self.K2_AttachToComponent` _output_get Location "None" "KeepWorld" "KeepWorld" "KeepWorld" true)
  (`self.RemoveFromArray`))

(fn `ProcessControl`
  (params (`isOver?` :type Boolean))
  (returns (Time :type Integer))
  (locals (RandomRestDescription :type "Array of Text"))
  (bind _scoreui (`/Game/Blueprint/Player/BP_MotorcycleCharacter.ScoreUI` (`self.Player`)))
  (bind _scoreui_2 (`/Game/Blueprint/Player/BP_MotorcycleCharacter.ScoreUI` (`self.Player`)))
  (if `isOver?`
    (set `self.shouldSpanwItem` false)
    (`UserWidget.PlayAnimation` _scoreui (`/Game/UI/W_PlayerScoreUI.NewEvent` _scoreui) 0.0 1 "Forward" 1.0 false)
    (`/Game/UI/W_PlayerScoreUI.EventInfor` _scoreui "中场休息" (`KismetArrayLibrary.Array_Random` (`local.RandomRestDescription`)) 0.0)
    (`/Game/UI/W_PlayerScoreUI.EndCountdown` _scoreui)
    (else
      (set `self.shouldSpanwItem` true)
      (if (`self.isBossEvent?`)
        (set `self.isBossEvent?` false)
        (set `self.RandomEventName` (`KismetArrayLibrary.Array_Random` (`self.BossEventArray`)))
        (else
          (set `self.RandomEventName` (`KismetArrayLibrary.Array_Random` (`self.NormalEventArray`)))))
      (bind _returnvalue (`|GetDataTableRow` "/Game/Blueprint/Enemy/Base/RandomEvent/DT_RandomEventList.DT_RandomEventList" (`self.RandomEventName`))
        (:`then`
          (`UserWidget.PlayAnimation` _scoreui_2 (`/Game/UI/W_PlayerScoreUI.NewEvent` _scoreui_2) 0.0 1 "Forward" 1.0 false)
          (bind (_eventname _eventdescription _eventtype _iteminevent _maxenemynum _eventtime) (break `/Game/Blueprint/Enemy/Base/RandomEvent/S_RandomEventList` _returnvalue))
          (bind _returnvalue_2 (`KismetMathLibrary.Conv_IntToDouble` _eventtime))
          (`/Game/UI/W_PlayerScoreUI.EventInfor` _scoreui_2 _eventname (`KismetArrayLibrary.Array_Random` _eventdescription) _returnvalue_2)
          (`/Game/UI/W_PlayerScoreUI.SetCountdown` _scoreui _returnvalue_2 (`|EnumEquality` _eventtype "NewEnumerator3"))
          (return _eventtime))))))

(fn `UserConstructionScript`)