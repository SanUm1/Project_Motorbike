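; Player controller actor for the motorcycle equipment screen, handling camera view, rotation input, cursor hover and weapon placement.
; A looping timer traces under the cursor, converting hits into cube index and face on BP_CubeWeaponUnit to highlight tiles.
; A selected equipment slot spawns a snapped, adjustable preview weapon and sets the add-weapon action.
; Clicks execute swappable action actors on the hovered tile; another timer applies yaw input to the equipment camera.
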(event `self.ReceiveBeginPlay`
  (bind _returnvalue (`GameplayStatics.GetPlayerController` 0))
  (bind _returnvalue_2 (`GameplayStatics.GetPlayerController` 0))
  (bind _returnvalue_3 (`self.K2_GetActorRotation` (`self.BP_EquipCamera`)))
  (bind _returnvalue_4 (pcsubsystem `EnhancedInputLocalPlayerSubsystem` _returnvalue_2))
  (`|ExecutionSequence`
    (:`then_0`
      ; Comment
      (bind _returnvalue_5 (`GameplayStatics.GetActorOfClass` "/Game/Blueprint/Equipment/BP_CameraInEquipment.BP_CameraInEquipment_C"))
      (set `self.BP_EquipCamera` _returnvalue_5)
      (bind _returnvalue_6 (`GameplayStatics.GetActorOfClass` "/Game/Blueprint/Player/BP_MotorcycleCharacter_Child.BP_MotorcycleCharacter_Child_C"))
      (set `self.BP_Motorcycle_Child` _returnvalue_6)
      (bind _returnvalue_7 (`GameplayStatics.GetActorOfClass` "/Game/Blueprint/Equipment/BP_EquipmentSystem.BP_EquipmentSystem_C"))
      (bind _output_get (set `self.EquipmentSystem` _returnvalue_7))
      (set `/Game/Blueprint/Equipment/BP_EquipmentSystem.PlayerActionInEquip` self _output_get))
    (:`then_1`
      ; Comment
      (set `self.MotorcycleStartRotation` _returnvalue_3)
      (set `self.RotationDesiredZ` (.yaw _returnvalue_3))
      (`self.StartEquipMotocycleTimer`)
      ; Comment
      (set `PlayerController.bShowMouseCursor` true _returnvalue)
      (`self.EnableInput` _returnvalue)
      (`PlayerController.SetViewTargetWithBlend` _returnvalue (`self.BP_EquipCamera`) 0.0 "VTBlend_Linear" 0.0 false))
    (:`then_2`
      ; Comment
      (`/Engine/EditorBlueprintResources/StandardMacros.IsValid` _returnvalue_2
        (:`Is Valid`
          (`/Engine/EditorBlueprintResources/StandardMacros.IsValid` _returnvalue_4
            (:`Is Valid`
              (`EnhancedInputSubsystemInterface.AddMappingContext` _returnvalue_4 "/Game/Input/IMC_EquipementMenu.IMC_EquipementMenu" 0 (struct)))))))
    (:`then_3`
      (`self.StartTimerToCheckLocationUnderCursor`))))

(event `StartEquipMotocycleTimer`
  ;[0 0 0 0.5] A&D 控制场景中的摩托车左右旋转，E重置初始的摩托车旋转视角
  (bind _returnvalue (`KismetSystemLibrary.K2_SetTimerDelegate` (delegate `UpdateMotocycleTransform`) (`self.MotocycleUpdateDeltaSecond`) true))
  (set `self.MotocycleUpdateTimer` _returnvalue))

(event `UpdateMotocycleTransform`
  (bind _returnvalue (- (`self.RotationDesiredZ`) (.yaw (`self.K2_GetActorRotation` (`self.BP_Motorcycle_Child`)))))
  ;[0 0 0 0.5] A&D 控制场景中的摩托车左右旋转，E重置初始的摩托车旋转视角
  (if (!= (.yaw (`self.K2_GetActorRotation` (`self.BP_Motorcycle_Child`))) (`self.RotationDesiredZ`))
    (`self.K2_AddActorWorldRotation` (`self.BP_EquipCamera`) (`KismetMathLibrary.MakeRotator` 0.0 0.0 _returnvalue) false false)
    (set `self.RotationDesiredZ` (- (`self.RotationDesiredZ`) _returnvalue))))

(event `EnhancedInput|/Game/Input/IA_Rotation_LeftOrRight`
  (params (ActionValue :type "Float (double-precision)") (ElapsedSeconds :type "Float (double-precision)") (TriggeredSeconds :type "Float (double-precision)") (InputAction :type "InputAction Object Reference" :default "/Game/Input/IA_Rotation_LeftOrRight.IA_Rotation_LeftOrRight"))
  ;[0 0 0 0.5] A&D 控制场景中的摩托车左右旋转，E重置初始的摩托车旋转视角
  (:`Triggered`
    (if (!= ActionValue 0.0)
      (if (> ActionValue 0.0)
        (set `self.RotationDesiredZ` (+ (`self.RotationDesiredZ`) (* (`self.RotateAngle`) -1.0)))
        (else
          (set `self.RotationDesiredZ` (+ (`self.RotationDesiredZ`) (`self.RotateAngle`))))))))

(event `EnhancedInput|/Game/Input/IA_ResetRotation`
  (params (ActionValue :type Boolean) (ElapsedSeconds :type "Float (double-precision)") (TriggeredSeconds :type "Float (double-precision)") (InputAction :type "InputAction Object Reference" :default "/Game/Input/IA_ResetRotation.IA_ResetRotation"))
  ;[0 0 0 0.5] A&D 控制场景中的摩托车左右旋转，E重置初始的摩托车旋转视角
  (:`Started`
    (`/Engine/EditorBlueprintResources/StandardMacros.DoOnce` false :!label _label
      (:`Completed`
        (`KismetSystemLibrary.PrintString` "ResetRotation")
        (if (!= (`self.K2_GetActorRotation` (`self.BP_Motorcycle_Child`)) (`self.MotorcycleStartRotation`))
          (set `self.RotationDesiredZ` (.yaw (`self.MotorcycleStartRotation`)))))))
  (:`Completed`
    (goto _label :!via `Reset`)))

(event `StartTimerToCheckLocationUnderCursor`
  (bind _returnvalue (`KismetSystemLibrary.K2_SetTimerDelegate` (delegate `UpdateLocationUnderCursor`) 0.02 true))
  (set `self.CursorLocCheckingTimer` _returnvalue))

(event `UpdateLocationUnderCursor`
  (bind _previewweapon (`self.PreviewWeapon`))
  (bind _hoveredtileindexandcubeweapon (`self.HoveredTileIndexAndCubeWeapon`))
  (bind _currentselectedequipslot (`/Game/Blueprint/Equipment/Widget/WBP_EquipmentScreen.CurrentSelectedEquipSlot` (`/Game/Blueprint/Equipment/BP_EquipmentSystem.WBP_EquipScreen` (`self.EquipmentSystem`))))
  (bind (_location _hitcubeweapon) (`self.GetCursorLocationAndWeaponOnTile` 0))
  (bind (_linkingweapon _indexonweapon _direction) (`self.GetTileIndexAndDirectIndexOfWeaponFromLoc` _location _hitcubeweapon))
  (`self.SetHoveredTileIndexAndWeapon` _linkingweapon _indexonweapon _direction)
  ; Comment
  (`/Engine/EditorBlueprintResources/StandardMacros.IsValid` _currentselectedequipslot
    (:`Is Valid`
      (if (`|EnumInequality` (`/Game/Blueprint/Equipment/Widget/WBP_EquipSlot.WeaponType` _currentselectedequipslot) "NewEnumerator0")
        (`|ExecutionSequence`
          (:`then_0`
            (`/Engine/EditorBlueprintResources/StandardMacros.DoOnce` false :!label _label_2
              (:`Completed`
                (`self.SetSelectedAction` "/Game/Blueprint/Equipment/Action/BP_Action_Child_AddRemoveWeaponToHoveredTile.BP_Action_Child_AddRemoveWeaponToHoveredTile_C")
                (bind _asbp_action_child_add_remove_weapon_to_hovered_tile (cast `/Game/Blueprint/Equipment/Action/BP_Action_Child_AddRemoveWeaponToHoveredTile` (`self.SelectedActionLeftClick`)))
                (set `/Game/Blueprint/Equipment/Action/BP_Action_Child_AddRemoveWeaponToHoveredTile.IsAddingWeapon` true _asbp_action_child_add_remove_weapon_to_hovered_tile))))
          (:`then_1`
            (if (> (`BlueprintMapLibrary.Map_Length` _hoveredtileindexandcubeweapon) 0)
              (bind _values (`BlueprintMapLibrary.Map_Values` _hoveredtileindexandcubeweapon))
              (`/Engine/EditorBlueprintResources/StandardMacros.IsValid` (`|GetArrayItem` _values)
                (:`Is Valid`
                  (`/Engine/EditorBlueprintResources/StandardMacros.IsValid` (`self.PreviewWeapon`)
                    (:`Is Valid`
                      _)
                    (:`Is Not Valid`
                      (bind _returnvalue (`|SpawnActorFromClass` "/Game/Blueprint/Equipment/CubeWeapon/BP_CubeWeaponUnit.BP_CubeWeaponUnit_C" (`KismetMathLibrary.MakeTransform` (0.0 0.0 0.0)) "AlwaysSpawn" "MultiplyWithRoot" null (`/Game/Blueprint/Equipment/Widget/WBP_EquipSlot.WeaponType` (`/Game/Blueprint/Equipment/Widget/WBP_EquipmentScreen.CurrentSelectedEquipSlot` (`/Game/Blueprint/Equipment/BP_EquipmentSystem.WBP_EquipScreen` (`self.EquipmentSystem`)))) true null))
                      (set `self.PreviewWeapon` _returnvalue)))
                  (`/Game/Blueprint/Equipment/BP_EquipmentSystem.ShowPreviewWeaponDisplay` (`self.EquipmentSystem`) (`self.PreviewWeapon`) (`self.HoveredTileIndexAndCubeWeapon`) true (`self.HorizontalAdjustNum`) (`self.VerticalAdjustNum`)))
                (:`Is Not Valid`
                  (`|ExecutionSequence` :!label _label_3
                    (:`then_0`
                      (goto _label_2 :!via `Reset`))
                    (:`then_1`
                      (`self.SetSelectedAction` null)
                      (`/Engine/EditorBlueprintResources/StandardMacros.IsValid` _previewweapon
                        (:`Is Valid`
                          (`self.K2_DestroyActor` _previewweapon)
                          (set `self.PreviewWeapon` null)
                          (set `self.HorizontalAdjustNum` 0)
                          (set `self.VerticalAdjustNum` 0)))))))
              (else
                (goto _label_3)))))
        (else
          (goto _label_3))))
    (:`Is Not Valid`
      (goto _label_3))))

(event `EnhancedInput|/Game/Input/IA_LeftClickInEquipment`
  (params (ActionValue :type Boolean) (ElapsedSeconds :type "Float (double-precision)") (TriggeredSeconds :type "Float (double-precision)") (InputAction :type "InputAction Object Reference" :default "/Game/Input/IA_LeftClickInEquipment.IA_LeftClickInEquipment"))
  (bind _selectedactionleftclick (`self.SelectedActionLeftClick`))
  ; Comment
  (:`Triggered`
    (if ActionValue
      (`/Engine/EditorBlueprintResources/StandardMacros.DoOnce` false :!label _label_4
        (:`Completed`
          (`/Engine/EditorBlueprintResources/StandardMacros.IsValid` _selectedactionleftclick
            (:`Is Valid`
              (`/Game/Blueprint/Equipment/Action/BP_Action.ExecuteAction` _selectedactionleftclick (`self.HoveredTileIndexAndCubeWeapon`))))))))
  (:`Completed`
    (goto _label_4 :!via `Reset`)))

(event `EnhancedInput|/Game/Input/IA_RightClickInEquipment`
  (params (ActionValue :type Boolean) (ElapsedSeconds :type "Float (double-precision)") (TriggeredSeconds :type "Float (double-precision)") (InputAction :type "InputAction Object Reference" :default "/Game/Input/IA_RightClickInEquipment.IA_RightClickInEquipment"))
  (bind _selectedactionrightclick (`self.SelectedActionRightClick`))
  ; Comment
  (:`Triggered`
    (if ActionValue
      (`/Engine/EditorBlueprintResources/StandardMacros.DoOnce` false :!label _label_5
        (:`Completed`
          (`/Engine/EditorBlueprintResources/StandardMacros.IsValid` _selectedactionrightclick
            (:`Is Valid`
              (`/Game/Blueprint/Equipment/Action/BP_Action.ExecuteAction` _selectedactionrightclick (`self.HoveredTileIndexAndCubeWeapon`))))))))
  (:`Completed`
    (goto _label_5 :!via `Reset`)))

(event `EnhancedInput|/Game/Input/IA_EquipHorizontalAdjust`
  (params (ActionValue :type "Float (double-precision)") (ElapsedSeconds :type "Float (double-precision)") (TriggeredSeconds :type "Float (double-precision)") (InputAction :type "InputAction Object Reference" :default "/Game/Input/IA_EquipHorizontalAdjust.IA_EquipHorizontalAdjust"))
  ; Comment
  (:`Triggered`
    (`/Engine/EditorBlueprintResources/StandardMacros.IsValid` (`self.PreviewWeapon`)
      (:`Is Valid`
        (if (!= ActionValue 0.0)
          (`/Engine/EditorBlueprintResources/StandardMacros.DoOnce` false :!label _label_6
            (:`Completed`
              (bind _keys (`BlueprintMapLibrary.Map_Keys` (`self.HoveredTileIndexAndCubeWeapon`)))
              (bind (_x _y) (break `IntPoint` (`/Game/Blueprint/Equipment/BP_EquipmentSystem.GetWeaponAdjustNumRangeBaseOnDirect` (`self.EquipmentSystem`) (`self.PreviewWeapon`) (`.DirectIndex_4_404E2F104352FAD9B748E5B3D95D45D4` (break `/Game/Blueprint/Equipment/CubeWeapon/Utilities/S_CubeIndexWithDirectIndex` (`|GetArrayItem` _keys))))))
              (set `self.HorizontalAdjustNum` (`KismetMathLibrary.Clamp` (+ (`self.HorizontalAdjustNum`) (select `bool` (> ActionValue 0.0) :`false` -1 :`true` 1)) _x _y))))))))
  (:`Completed`
    (goto _label_6 :!via `Reset`)))

(event `EnhancedInput|/Game/Input/IA_EquipVerticalAdjust`
  (params (ActionValue :type "Float (double-precision)") (ElapsedSeconds :type "Float (double-precision)") (TriggeredSeconds :type "Float (double-precision)") (InputAction :type "InputAction Object Reference" :default "/Game/Input/IA_EquipVerticalAdjust.IA_EquipVerticalAdjust"))
  ; Comment
  (:`Triggered`
    (`/Engine/EditorBlueprintResources/StandardMacros.IsValid` (`self.PreviewWeapon`)
      (:`Is Valid`
        (if (!= ActionValue 0.0)
          (`/Engine/EditorBlueprintResources/StandardMacros.DoOnce` false :!label _label_7
            (:`Completed`
              (bind _keys (`BlueprintMapLibrary.Map_Keys` (`self.HoveredTileIndexAndCubeWeapon`)))
              (bind (_x _y) (break `IntPoint` (`.VerticalAdjustClamp` (`/Game/Blueprint/Equipment/BP_EquipmentSystem.GetWeaponAdjustNumRangeBaseOnDirect` (`self.EquipmentSystem`) (`self.PreviewWeapon`) (`.DirectIndex_4_404E2F104352FAD9B748E5B3D95D45D4` (break `/Game/Blueprint/Equipment/CubeWeapon/Utilities/S_CubeIndexWithDirectIndex` (`|GetArrayItem` _keys)))))))
              (set `self.VerticalAdjustNum` (`KismetMathLibrary.Clamp` (+ (`self.VerticalAdjustNum`) (select `bool` (> ActionValue 0.0) :`false` -1 :`true` 1)) _x _y))))))))
  (:`Completed`
    (goto _label_7 :!via `Reset`)))

(fn `GetCursorLocationAndWeaponOnTile`
  (params (PlayerIndex :type Integer))
  (returns (Location :type "Vector Structure") (HitCubeWeapon :type "/Game/Blueprint/Equipment/CubeWeapon/BP_CubeWeaponUnit Object Reference"))
  (bind _returnvalue (`GameplayStatics.GetPlayerController` PlayerIndex))
  (bind (_locationx _locationy) (`PlayerController.GetMousePosition` _returnvalue))
  (bind (_worldposition _worlddirection) (`GameplayStatics.DeprojectScreenToWorld` _returnvalue (`KismetMathLibrary.MakeVector2D` _locationx _locationy)))
  (bind (_outhit _returnvalue_2) (`KismetSystemLibrary.LineTraceSingle` _worldposition (+ _worldposition (* _worlddirection 999999.0)) "TraceTypeQuery3"))
  (if _returnvalue_2
    (bind (_bblockinghit _binitialoverlap _time _distance _location _impactpoint _normal _impactnormal _physmat _hitactor) (`GameplayStatics.BreakHitResult` _outhit))
    (bind _asbp_cube_weapon_unit (cast `/Game/Blueprint/Equipment/CubeWeapon/BP_CubeWeaponUnit` _hitactor)
      (:`then`
        (return _location _asbp_cube_weapon_unit))
      (:`CastFailed`
        _)))
  (return (-999999.0 -999999.0 -999999.0) null))

(fn `GetTileIndexAndDirectIndexOfWeaponFromLoc`
  (params (Location :type "Vector Structure") (TargetWeapon :type "/Game/Blueprint/Equipment/CubeWeapon/BP_CubeWeaponUnit Object Reference"))
  (returns (LinkingWeapon :type "/Game/Blueprint/Equipment/CubeWeapon/BP_CubeWeaponUnit Object Reference") (IndexOnWeapon :type "IntVector Structure") (Direction :type Integer))
  (locals (LocRelativeToWeapon :type "Vector Structure") (CubeIndex :type "IntVector Structure") (CubeCenterLoc :type "Vector Structure") (I :type Integer) (IsGreaterThanZero :type Boolean) (RetDirect :type Integer :default 0))
  (bind _isgreaterthanzero (`local.IsGreaterThanZero`))
  (bind _x (.x (- (`local.LocRelativeToWeapon`) (* (`KismetMathLibrary.Conv_IntVectorToVector` (`local.CubeIndex`)) (50.0 50.0 50.0)))))
  (bind _y (.y (- (`local.LocRelativeToWeapon`) (* (`KismetMathLibrary.Conv_IntVectorToVector` (`local.CubeIndex`)) (50.0 50.0 50.0)))))
  (bind _z (.z (- (`local.LocRelativeToWeapon`) (* (`KismetMathLibrary.Conv_IntVectorToVector` (`local.CubeIndex`)) (50.0 50.0 50.0)))))
  (`/Engine/EditorBlueprintResources/StandardMacros.IsValid` TargetWeapon
    (:`Is Valid`
      (if (!= (`local.Location`) (-999999.0 -999999.0 -999999.0))
        (bind _output_get (set `local.LocRelativeToWeapon` (- (+ (`local.Location`) (25.0 25.0 25.0)) (+ (`self.K2_GetActorLocation` (`local.TargetWeapon`)) (25.0 25.0 25.0)))))
        (set `local.CubeIndex` (make `IntVector` (`KismetMathLibrary.FTrunc` (.x (/ (`/Game/Blueprint/Equipment/CubeWeapon/Utilities/BFL_CubeWeaponData.SnapVectorToCriterion` _output_get (50.0 50.0 50.0)) (50.0 50.0 50.0)))) (`KismetMathLibrary.FTrunc` (.y (/ (`/Game/Blueprint/Equipment/CubeWeapon/Utilities/BFL_CubeWeaponData.SnapVectorToCriterion` _output_get (50.0 50.0 50.0)) (50.0 50.0 50.0)))) (`KismetMathLibrary.FTrunc` (.z (/ (`/Game/Blueprint/Equipment/CubeWeapon/Utilities/BFL_CubeWeaponData.SnapVectorToCriterion` _output_get (50.0 50.0 50.0)) (50.0 50.0 50.0))))))
        (bind _output_get_2 (set `local.I` (`KismetMathLibrary.MaxOfFloatArray` (`|MakeArray` (`KismetMathLibrary.Abs` _x) (`KismetMathLibrary.Abs` _y) (`KismetMathLibrary.Abs` _z) :!type "Float (single-precision)"))))
        (set `local.IsGreaterThanZero` (> (`|GetArrayItem` (`|MakeArray` _x _y _z) _output_get_2) 0.0))
        (set `local.RetDirect` (select `int` (`local.I`) :`0` (`KismetMathLibrary.SelectInt` 2 3 _isgreaterthanzero) :`1` (`KismetMathLibrary.SelectInt` 5 4 _isgreaterthanzero) :`2` (`KismetMathLibrary.SelectInt` 0 1 _isgreaterthanzero)))
        (return (`local.TargetWeapon`) (`local.CubeIndex`) (`local.RetDirect`))
        (else
          _)))
    (:`Is Not Valid`
      _))
  (return null (make `IntVector` -999 -999 -999) -999))

(fn `SetHoveredTileIndexAndWeapon`
  (params (Weapon :type "/Game/Blueprint/Equipment/CubeWeapon/BP_CubeWeaponUnit Object Reference") (CubeIndex :type "IntVector Structure") (DirectIndex :type Integer))
  (if (> (`BlueprintMapLibrary.Map_Length` (`self.HoveredTileIndexAndCubeWeapon`)) 0)
    (bind _keys (`BlueprintMapLibrary.Map_Keys` (`self.HoveredTileIndexAndCubeWeapon`)))
    (bind (_cubeindex _directindex) (break `/Game/Blueprint/Equipment/CubeWeapon/Utilities/S_CubeIndexWithDirectIndex` (`|GetArrayItem` _keys)))
    (if (or (not (== (`KismetMathLibrary.Conv_IntVectorToVector` _cubeindex) (`KismetMathLibrary.Conv_IntVectorToVector` (`local.CubeIndex`)))) (!= _directindex (`local.DirectIndex`)))
      (bind _values (`BlueprintMapLibrary.Map_Values` (`self.HoveredTileIndexAndCubeWeapon`)))
      (for (_array_element _array_index) _values
        (`/Engine/EditorBlueprintResources/StandardMacros.IsValid` _array_element
          (:`Is Valid`
            (bind _keys_2 (`BlueprintMapLibrary.Map_Keys` (`self.HoveredTileIndexAndCubeWeapon`)))
            (bind (_cubeindex_2 _directindex_2) (break `/Game/Blueprint/Equipment/CubeWeapon/Utilities/S_CubeIndexWithDirectIndex` (`|GetArrayItem` _keys_2 _array_index)))
            (`/Game/Blueprint/Equipment/CubeWeapon/BP_CubeWeaponUnit.RemoveStateFromTile` _array_element _cubeindex_2 _directindex_2 "NewEnumerator1")
            (`KismetSystemLibrary.PrintString` (`KismetStringLibrary.Concat_StrStr` "旧的   " (select `int` _directindex_2 :`0` "上" :`1` "下" :`2` "前" :`3` "后" :`4` "左" :`5` "右")) true true (struct :`R` 0.079895 :`B` 1.0 :`A` 1.0)))))
      (`BlueprintMapLibrary.Map_Clear` (`self.HoveredTileIndexAndCubeWeapon`))
      (`/Engine/EditorBlueprintResources/StandardMacros.IsValid` (`local.Weapon`) :!label _label
        (:`Is Valid`
          (if (`KismetArrayLibrary.Array_Contains` (`/Game/Blueprint/Equipment/CubeWeapon/BP_CubeWeaponUnit.WeaponCubeIndex` (`local.Weapon`)) (`local.CubeIndex`))
            (`/Game/Blueprint/Equipment/CubeWeapon/BP_CubeWeaponUnit.AddStateToTile` (`local.Weapon`) (`local.CubeIndex`) (`local.DirectIndex`) "NewEnumerator1")
            (`KismetSystemLibrary.PrintString` (`KismetStringLibrary.Concat_StrStr` "新的的   " (select `int` (`local.DirectIndex`) :`0` "上" :`1` "下" :`2` "前" :`3` "后" :`4` "左" :`5` "右")) true true (struct :`G` 1.0 :`B` 0.91453 :`A` 1.0))
            (`BlueprintMapLibrary.Map_Add` (`self.HoveredTileIndexAndCubeWeapon`) (make `/Game/Blueprint/Equipment/CubeWeapon/Utilities/S_CubeIndexWithDirectIndex` (`local.CubeIndex`) (`local.DirectIndex`)) (`local.Weapon`))))
        (:`Is Not Valid`
          (set `self.HoveredTileIndexAndCubeWeapon` (`|MakeMap` (make `/Game/Blueprint/Equipment/CubeWeapon/Utilities/S_CubeIndexWithDirectIndex` (make `IntVector` -999 -999 -999)) :!valuetype "/Game/Blueprint/Equipment/CubeWeapon/BP_CubeWeaponUnit Object Reference")))))
    (else
      (goto _label))))

(fn `SetSelectedAction`
  (params (LeftAction :type "/Game/Blueprint/Equipment/Action/BP_Action Class Reference") (RightAction :type "/Game/Blueprint/Equipment/Action/BP_Action Class Reference"))
  (bind _selectedactionleftclick (`self.SelectedActionLeftClick`))
  (bind _selectedactionrightclick (`self.SelectedActionRightClick`))
  (`|ExecutionSequence`
    (:`then_0`
      (`/Engine/EditorBlueprintResources/StandardMacros.IsValid` _selectedactionleftclick
        (:`Is Valid`
          (`self.K2_DestroyActor` _selectedactionleftclick)
          (set `self.SelectedActionLeftClick` null))
        (:`Is Not Valid`
          _))
      (if (`KismetSystemLibrary.IsValidClass` (`local.LeftAction`))
        (bind _returnvalue (`|SpawnActorFromClass` (`local.LeftAction`) (`KismetMathLibrary.MakeTransform` (0.0 0.0 0.0)) "AlwaysSpawn" "MultiplyWithRoot" null self null))
        (set `self.SelectedActionLeftClick` _returnvalue)))
    (:`then_1`
      (`/Engine/EditorBlueprintResources/StandardMacros.IsValid` _selectedactionrightclick
        (:`Is Valid`
          (`self.K2_DestroyActor` _selectedactionrightclick)
          (set `self.SelectedActionRightClick` null))
        (:`Is Not Valid`
          _))
      (if (`KismetSystemLibrary.IsValidClass` (`local.RightAction`))
        (bind _returnvalue_2 (`|SpawnActorFromClass` (`local.RightAction`) (`KismetMathLibrary.MakeTransform` (0.0 0.0 0.0)) "AlwaysSpawn" "MultiplyWithRoot" null self null))
        (set `self.SelectedActionRightClick` _returnvalue_2)))
    (:`then_2`
      (`self.OnSelectedActionsChanged` (`self.SelectedActionLeftClick`) (`self.SelectedActionRightClick`)))))

(fn `SetSelectedTileIndexAndWeapon`
  (params (InputCubeIndexAndDirectIndex_CubeWeapon :type "Map of /Game/Blueprint/Equipment/CubeWeapon/Utilities/S_CubeIndexWithDirectIndex Structure to /Game/Blueprint/Equipment/CubeWeapon/BP_CubeWeaponUnit Object Reference") (Force :type Boolean))
  (bind _selectedtileindexandcubeweapon (`self.SelectedTileIndexAndCubeWeapon`))
  (bind _inputcubeindexanddirectindex_cubeweapon (`local.InputCubeIndexAndDirectIndex_CubeWeapon`))
  (bind _selectedtileindexandcubeweapon_2 (`self.SelectedTileIndexAndCubeWeapon`))
  (bind _inputcubeindexanddirectindex_cubeweapon_2 (`local.InputCubeIndexAndDirectIndex_CubeWeapon`))
  (bind _selectedtileindexandcubeweapon_3 (`self.SelectedTileIndexAndCubeWeapon`))
  (bind _selectedtileindexandcubeweapon_4 (`self.SelectedTileIndexAndCubeWeapon`))
  (`|ExecutionSequence`
    (:`then_0`
      (if (> (`BlueprintMapLibrary.Map_Length` (`local.InputCubeIndexAndDirectIndex_CubeWeapon`)) 0)
        (if (> (`BlueprintMapLibrary.Map_Length` (`self.SelectedTileIndexAndCubeWeapon`)) 0)
          (bind _keys (`BlueprintMapLibrary.Map_Keys` _inputcubeindexanddirectindex_cubeweapon_2))
          (bind _values (`BlueprintMapLibrary.Map_Values` _inputcubeindexanddirectindex_cubeweapon_2))
          (bind _keys_2 (`BlueprintMapLibrary.Map_Keys` _selectedtileindexandcubeweapon))
          (bind _values_2 (`BlueprintMapLibrary.Map_Values` _selectedtileindexandcubeweapon))
          (bind (_cubeindex _directindex) (break `/Game/Blueprint/Equipment/CubeWeapon/Utilities/S_CubeIndexWithDirectIndex` (`|GetArrayItem` _keys_2)))
          (bind (_cubeindex_2 _directindex_2) (break `/Game/Blueprint/Equipment/CubeWeapon/Utilities/S_CubeIndexWithDirectIndex` (`|GetArrayItem` _keys)))
          (if (or (!= (`|GetArrayItem` _values) (`|GetArrayItem` _values_2)) (not (== (`KismetMathLibrary.Conv_IntVectorToVector` _cubeindex) (`KismetMathLibrary.Conv_IntVectorToVector` _cubeindex_2))) (!= _directindex _directindex_2) (`local.Force`))
            ; Comment
            (if (> (`BlueprintMapLibrary.Map_Length` _selectedtileindexandcubeweapon_4) 0) :!label _label
              (bind _values_3 (`BlueprintMapLibrary.Map_Values` _selectedtileindexandcubeweapon_4))
              (for (_array_element _array_index) _values_3
                (`/Engine/EditorBlueprintResources/StandardMacros.IsValid` _array_element
                  (:`Is Valid`
                    (bind _keys_3 (`BlueprintMapLibrary.Map_Keys` (`self.SelectedTileIndexAndCubeWeapon`)))
                    (bind (_cubeindex_3 _directindex_3) (break `/Game/Blueprint/Equipment/CubeWeapon/Utilities/S_CubeIndexWithDirectIndex` (`|GetArrayItem` _keys_3 _array_index)))
                    (`/Game/Blueprint/Equipment/CubeWeapon/BP_CubeWeaponUnit.RemoveStateFromTile` _array_element _cubeindex_3 _directindex_3 "NewEnumerator2")))))
            (bind _values_4 (`BlueprintMapLibrary.Map_Values` _inputcubeindexanddirectindex_cubeweapon))
            (`/Engine/EditorBlueprintResources/StandardMacros.IsValid` (`|GetArrayItem` _values_4)
              (:`Is Valid`
                (set `self.SelectedTileIndexAndCubeWeapon` _inputcubeindexanddirectindex_cubeweapon)
                (if (> (`BlueprintMapLibrary.Map_Length` _selectedtileindexandcubeweapon_2) 0)
                  (bind _values_5 (`BlueprintMapLibrary.Map_Values` _selectedtileindexandcubeweapon_2))
                  (for (_array_element_2 _array_index_2) _values_5
                    (`/Engine/EditorBlueprintResources/StandardMacros.IsValid` _array_element_2
                      (:`Is Valid`
                        (bind _keys_4 (`BlueprintMapLibrary.Map_Keys` (`self.SelectedTileIndexAndCubeWeapon`)))
                        (bind (_cubeindex_4 _directindex_4) (break `/Game/Blueprint/Equipment/CubeWeapon/Utilities/S_CubeIndexWithDirectIndex` (`|GetArrayItem` _keys_4 _array_index_2)))
                        (`/Game/Blueprint/Equipment/CubeWeapon/BP_CubeWeaponUnit.AddStateToTile` _array_element_2 _cubeindex_4 _directindex_4 "NewEnumerator2"))))))
              (:`Is Not Valid`
                (set `self.SelectedTileIndexAndCubeWeapon` (`|MakeMap`))))
            (else
              ; Comment
              (if (> (`BlueprintMapLibrary.Map_Length` _selectedtileindexandcubeweapon_3) 0)
                (bind _values_6 (`BlueprintMapLibrary.Map_Values` _selectedtileindexandcubeweapon_3))
                (for (_array_element_3 _array_index_3) _values_6
                  (`/Engine/EditorBlueprintResources/StandardMacros.IsValid` _array_element_3
                    (:`Is Valid`
                      (bind _keys_5 (`BlueprintMapLibrary.Map_Keys` (`self.SelectedTileIndexAndCubeWeapon`)))
                      (bind (_cubeindex_5 _directindex_5) (break `/Game/Blueprint/Equipment/CubeWeapon/Utilities/S_CubeIndexWithDirectIndex` (`|GetArrayItem` _keys_5 _array_index_3)))
                      (`/Game/Blueprint/Equipment/CubeWeapon/BP_CubeWeaponUnit.RemoveStateFromTile` _array_element_3 _cubeindex_5 _directindex_5 "NewEnumerator2")))))
              (set `self.SelectedTileIndexAndCubeWeapon` (`|MakeMap`))))
          (else
            (goto _label)))))))

(fn `UserConstructionScript`)