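; Equipment action that adds a weapon at the hovered cube or removes the hovered one, depending on IsAddingWeapon.
; Adding requires the preview weapon to snap to the hovered weapon without overlap, then spawns a BP_CubeWeaponUnit of its type and registers it in EquipmentSystem with horizontal and vertical adjustments.
; Removing checks the passed map's first weapon is valid, then has EquipmentSystem destroy PlayerActionInEquipment's HoveredWeapon.
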(fn `ExecuteAction`
  (params (CubeIndexAndDirectIndex_Weapon :type "Map of /Game/Blueprint/Equipment/CubeWeapon/Utilities/S_CubeIndexWithDirectIndex Structure to /Game/Blueprint/Equipment/CubeWeapon/BP_CubeWeaponUnit Object Reference"))
  (locals (HoveredWeapon :type "/Game/Blueprint/Equipment/CubeWeapon/BP_CubeWeaponUnit Object Reference"))
  (bind _playeractioninequipment (`self.PlayerActionInEquipment`))
  (bind _cubeindexanddirectindex_weapon (`local.CubeIndexAndDirectIndex_Weapon`))
  (bind _cubeindexanddirectindex_weapon_2 (`local.CubeIndexAndDirectIndex_Weapon`))
  (bind _playeractioninequipment_2 (`self.PlayerActionInEquipment`))
  (bind _playeractioninequipment_3 (`self.PlayerActionInEquipment`))
  (bind _previewweapon (`/Game/Blueprint/Equipment/BP_PlayerActionInEquipment.PreviewWeapon` _playeractioninequipment_3))
  (bind (_hascubesnap _hascubeoverlay) (`/Game/Blueprint/Equipment/BP_EquipmentSystem.CheckIsWeaponsSnapTogtherAndNotOverlay` (`/Game/Blueprint/Equipment/BP_PlayerActionInEquipment.EquipmentSystem` _playeractioninequipment_3) (`local.HoveredWeapon`) _previewweapon))
  (if (`self.IsAddingWeapon`)
    ; 悬停的网格有效
    (if (> (`BlueprintMapLibrary.Map_Length` _cubeindexanddirectindex_weapon_2) 0)
      (bind _values (`BlueprintMapLibrary.Map_Values` _cubeindexanddirectindex_weapon_2))
      (bind _output (`|GetArrayItem` _values))
      (`/Engine/EditorBlueprintResources/StandardMacros.IsValid` _output
        (:`Is Valid`
          (set `local.HoveredWeapon` _output)
          ; Comment
          (`/Engine/EditorBlueprintResources/StandardMacros.IsValid` _previewweapon
            (:`Is Valid`
              (if (and _hascubesnap (not _hascubeoverlay))
                ; Comment
                (bind _returnvalue (`|SpawnActorFromClass` "/Game/Blueprint/Equipment/CubeWeapon/BP_CubeWeaponUnit.BP_CubeWeaponUnit_C" (`KismetMathLibrary.MakeTransform` (0.0 0.0 0.0)) "Undefined" "MultiplyWithRoot" null (`/Game/Blueprint/Equipment/CubeWeapon/BP_CubeWeaponUnit.WeaponType` (`/Game/Blueprint/Equipment/BP_PlayerActionInEquipment.PreviewWeapon` (`self.PlayerActionInEquipment`))) false null))
                (`/Game/Blueprint/Equipment/BP_EquipmentSystem.AddWeaponInEquipSystem` (`/Game/Blueprint/Equipment/BP_PlayerActionInEquipment.EquipmentSystem` _playeractioninequipment_2) _returnvalue (`local.CubeIndexAndDirectIndex_Weapon`) (`/Game/Blueprint/Equipment/BP_PlayerActionInEquipment.HorizontalAdjustNum` _playeractioninequipment_2) (`/Game/Blueprint/Equipment/BP_PlayerActionInEquipment.VerticalAdjustNum` _playeractioninequipment_2))))))))
    (else
      ; 悬停的网格有效
      (if (> (`BlueprintMapLibrary.Map_Length` _cubeindexanddirectindex_weapon) 0)
        (bind _values_2 (`BlueprintMapLibrary.Map_Values` _cubeindexanddirectindex_weapon))
        (`/Engine/EditorBlueprintResources/StandardMacros.IsValid` (`|GetArrayItem` _values_2)
          (:`Is Valid`
            (`/Game/Blueprint/Equipment/BP_EquipmentSystem.RemoveWeaponInEquipSystem` (`/Game/Blueprint/Equipment/BP_PlayerActionInEquipment.EquipmentSystem` _playeractioninequipment) (`/Game/Blueprint/Equipment/BP_PlayerActionInEquipment.HoveredWeapon` _playeractioninequipment) true)))))))

(fn `UserConstructionScript`
  (`parent.UserConstructionScript`))