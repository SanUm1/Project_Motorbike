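; BP_SingleTunnel is one tunnel segment that gets recycled to the front of the path as the player advances, with five spawn points ordered left to right.
; A player overlapping Checkpoints fires CallMovingTunnel for BP_TunnelManager to handle the move, guarded by a DoOnce that resets after a short delay against retriggering.
; BoxForRecycling overlaps track Spawn-tagged actors inside the segment for recycling before it moves.
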(event `self.ReceiveBeginPlay`
  ; 存生成点位置（圆球）已从左到右排好顺序
  (set `self.SpawnPoint` (`|MakeArray` (`self.Sphere1`) (`self.Sphere3`) (`self.Sphere`) (`self.Sphere4`) (`self.Sphere2`))))

(event `self.Checkpoints.OnComponentBeginOverlap`
  (params (OverlappedComponent :type "PrimitiveComponent Object Reference") (OtherActor :type "Actor Object Reference") (OtherComp :type "PrimitiveComponent Object Reference") (OtherBodyIndex :type Integer) (bFromSweep :type Boolean) (SweepResult :type "HitResult Structure (by ref)"))
  ; 当玩家走到checkpoints时候，把当前路段移动至最前处（在BP_TunnelManager当中创建）
  (if (`self.ActorHasTag` OtherActor "Player")
    ;; 由于向前移动时候会撞到玩家多触发一次，所以用DoOnce处理。在delay后恢复
    (`/Engine/EditorBlueprintResources/StandardMacros.DoOnce` false :!label _label
      (:`Completed`
        (`self.MovingTunnel` self)
        (`KismetSystemLibrary.PrintString` "Moving")
        (`KismetSystemLibrary.Delay` 0.2)
        ;; 恢复boxcollision
        (`self.ResetCanMove`)))))

(event `ResetCanMove`
  ; 当玩家走到checkpoints时候，把当前路段移动至最前处（在BP_TunnelManager当中创建）
  ;; 由于向前移动时候会撞到玩家多触发一次，所以用DoOnce处理。在delay后恢复
  (goto _label :!via `Reset`))

(event `self.Box for recycling.OnComponentBeginOverlap`
  (params (OverlappedComponent :type "PrimitiveComponent Object Reference") (OtherActor :type "Actor Object Reference") (OtherComp :type "PrimitiveComponent Object Reference") (OtherBodyIndex :type Integer) (bFromSweep :type Boolean) (SweepResult :type "HitResult Structure (by ref)"))
  ; 将处于当前路段的生成物存入数组当中，在路段开始往最前移动之前，先将物品回收
  (if (`self.ActorHasTag` OtherActor "Spawn")
    (`KismetArrayLibrary.Array_AddUnique` (`self.ItemReadyForRecycling`) OtherActor)))

(event `self.Box for recycling.OnComponentEndOverlap`
  (params (OverlappedComponent :type "PrimitiveComponent Object Reference") (OtherActor :type "Actor Object Reference") (OtherComp :type "PrimitiveComponent Object Reference") (OtherBodyIndex :type Integer))
  ; 移除离开当前box collision的actor，一般为会移动的敌人ai
  (if (`self.ActorHasTag` OtherActor "Spawn")
    (`KismetArrayLibrary.Array_RemoveItem` (`self.ItemReadyForRecycling`) OtherActor)))

(fn `UserConstructionScript`)