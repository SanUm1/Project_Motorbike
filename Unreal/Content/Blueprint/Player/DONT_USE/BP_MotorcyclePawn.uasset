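; Motorcycle player pawn, stored under a DONT_USE folder, that switches between third-person and first-person views; its graphs hold no movement logic.
; CheckIsFirstPersonCamera activates the matching camera and shows that view's motorcycle mesh and cube while hiding the other pair.
; BeginPlay selects third person, and Q alternates views through a FlipFlop whose first output also selects third person, so the first press changes nothing.
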(event `self.ReceiveBeginPlay`
  (`self.CheckIsFirstPersonCamera` false))

(event `Key|Q`
  (params (Key :type "Key Structure"))
  ; 视角切换
  (:`Pressed`
    (`/Engine/EditorBlueprintResources/StandardMacros.FlipFlop`
      (:`A`
        (`self.CheckIsFirstPersonCamera` false))
      (:`B`
        (`self.CheckIsFirstPersonCamera` true)))))

(event `CheckIsFirstPersonCamera`
  (params (`CheckIsFirstPerson?` :type Boolean))
  ; 视角切换
  (if `CheckIsFirstPerson?`
    ;; 第一人称
    (`ActorComponent.SetActive` (`self.Camera_FirstPerson`) true false)
    (`SceneComponent.SetVisibility` (`self.MotorcycleMesh_FirstPerson`) true false)
    (`SceneComponent.SetVisibility` (`self.Cube1`) true false)
    (`ActorComponent.SetActive` (`self.Camera`) false false)
    (`SceneComponent.SetVisibility` (`self.MotorcycleMesh`) false false)
    (`SceneComponent.SetVisibility` (`self.Cube`) false false)
    (else
      ;; 第三人称
      (`ActorComponent.SetActive` (`self.Camera_FirstPerson`) false false)
      (`SceneComponent.SetVisibility` (`self.MotorcycleMesh_FirstPerson`) false false)
      (`SceneComponent.SetVisibility` (`self.Cube1`) false false)
      (`ActorComponent.SetActive` (`self.Camera`) true false)
      (`SceneComponent.SetVisibility` (`self.MotorcycleMesh`) true false)
      (`SceneComponent.SetVisibility` (`self.Cube`) true false))))

(fn `UserConstructionScript`)