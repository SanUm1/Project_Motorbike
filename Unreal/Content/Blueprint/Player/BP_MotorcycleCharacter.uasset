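; Player motorcycle character for a forward-driving combat game, handling driving, camera switching, combat, health, scoring and HUD.
; Timelines for acceleration, boost and brake multiply into speed in constant-speed mode, while steering offsets the actor sideways.
; Attacks are timer-looped twin line-trace guns and a draining, recharging shield that damages actors ahead.
; Overlap boxes wake enemies and recycle spawned items; movement, kills and near misses add score until death freezes time.
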(event `Key|One`
  (params (Key :type "Key Structure")))

(event `PlayStartAnim`
  (`SceneComponent.SetVisibility` (`self.StaticMesh`) true false)
  (`|PlayMontage` (`self.SkeletalMesh1`) "/Game/Art/Animation/Character/Character_PlayPhone_Anim_2_Montage.Character_PlayPhone_Anim_2_Montage"
    (:`then`
      (`|PlayMontage` (`self.SkeletalMesh`) "/Game/Art/Animation/Moto/Moto_PlayPhone_Anim_2_Montage.Moto_PlayPhone_Anim_2_Montage"
        (:`then`
          (bind (_direction `_新建轨道_0`) (`Timeline|时间轴` :!via `PlayFromStart`)
            (:`Update`
              (`CameraComponent.SetFieldOfView` (`self.Camera_FirstPerson`) (`KismetMathLibrary.Lerp` 90.0 120.0 `_新建轨道_0`)))))))
    (:`OnNotifyBegin`
      (`SceneComponent.SetVisibility` (`self.StaticMesh`) false false))))

(event `Attack_1 (Keep)`
  ; 左键
)

(event `EnhancedInput|/Game/Input/IA_Attack_1`
  (params (ActionValue :type Boolean) (ElapsedSeconds :type "Float (double-precision)") (TriggeredSeconds :type "Float (double-precision)") (InputAction :type "InputAction Object Reference" :default "/Game/Input/IA_Attack_1.IA_Attack_1"))
  (bind _image_47 (`/Game/UI/W_PlayerScoreUI.Image_47` (`self.ScoreUI`)))
  ; 左键
  (:`Triggered`
    (`self.Attack_1 (Keep)`))
  (:`Started`
    (`self.Attack_1 (Once)`)
    (`self.Weapon_1 Shooting`)
    (`/Game/UI/W_Tutorial.PressAndNext` (`/Game/UI/W_PlayerScoreUI.W_Tutorial` (`self.ScoreUI`)) "LMB")
    (`Image.SetColorAndOpacity` _image_47 (struct :`R` 0.009511 :`B` 0.440972 :`A` 1.0)))
  (:`Canceled`
    (`self.Attack_1 (Completed` :!label _label)
    (`self.Weapon_1 CancelShooting`)
    (`Image.SetColorAndOpacity` _image_47 (struct :`R` 1.0 :`G` 1.0 :`B` 1.0 :`A` 1.0)))
  (:`Completed`
    (goto _label)))

(event `Attack_1 (Once)`
  ; 左键
  (`KismetSystemLibrary.PrintString` "Attack_1"))

(event `self.ReceiveBeginPlay`
  (bind _returnvalue (`GameplayStatics.GetPlayerController` 0))
  (`|ExecutionSequence`
    (:`then_0`
      (`EnhancedInputSubsystemInterface.AddMappingContext` (pcsubsystem `EnhancedInputLocalPlayerSubsystem` (`GameplayStatics.GetPlayerController` 0)) "/Game/Input/IMC_Default.IMC_Default" 0 (struct))
      (`self.UseShield`)
      (`WidgetBlueprintLibrary.SetInputMode_GameOnly` _returnvalue)
      (set `PlayerController.bShowMouseCursor` false _returnvalue))
    (:`then_1`
      (`self.CheckIsFirstPersonCamera` true)
      (`self.CheckMovingAddScore`))
    (:`then_2`
      (bind _returnvalue_2 (`|CreateWidget` "/Game/UI/W_PlayerScoreUI.W_PlayerScoreUI_C"))
      (bind _output_get (set `self.ScoreUI` _returnvalue_2))
      (set `/Game/UI/W_PlayerScoreUI.Player` self _output_get)
      (`UserWidget.AddToViewport` _output_get 0))
    (:`then_3`
      (bind _outrownames (`DataTableFunctionLibrary.GetDataTableRowNames` "/Game/UI/DT_SubList.DT_SubList"))
      (for (_array_element _array_index) _outrownames
        (bind _returnvalue_3 (`|GetDataTableRow` "/Game/UI/DT_SubList.DT_SubList" _array_element)
          (:`then`
            (if (`|EnumEquality` (`.SubType_20_92A8AF69423F1B880EF3F19D33DD3100` (break `/Game/UI/S_SubtitleList` _returnvalue_3)) "NewEnumerator1")
              (`KismetArrayLibrary.Array_Add` (`self.RelaxSubIndexArray`) _array_index))))))
    (:`then_4`
      (for _ (range 2)
        (bind _returnvalue_4 (`|SpawnActorFromClass` "/Game/Blueprint/Player/BP_PlayerBullet.BP_PlayerBullet_C" (`KismetMathLibrary.MakeTransform` (0.0 0.0 5000.0)) "Undefined" "MultiplyWithRoot" null null))
        (`KismetArrayLibrary.Array_Add` (`self.Bullet`) _returnvalue_4))
      (set `self.ShootLocationArray` (`|MakeArray` (`self.Sphere`) (`self.Sphere1`))))
    (:`then_5`
      (`self.AllReady`)
      (`self.PlayStartAnim`))))

(event `Attack_1 (Completed`
  ; 左键
)

(event `Weapon_1 Shooting`
  ; 射击
  (`KismetSystemLibrary.K2_SetTimerDelegate` (delegate `MechinGunShoot`) 0.1 true))

(event `Weapon_1 CancelShooting`
  ; 射击
  (`KismetSystemLibrary.K2_SetTimerDelegate` (delegate `MechinGunShoot`)))

(event `MechinGunShoot`
  ; 射击
  (`self.SimpleShootSystem` (`SceneComponent.K2_GetComponentLocation` (`self.Sphere`)))
  (`self.SimpleShootSystem` (`SceneComponent.K2_GetComponentLocation` (`self.Sphere1`)))
  (`GameplayStatics.PlaySound2D` "/Game/Art/Voice/xm.xm" 1.0 1.0 0.0 null null)
  (for (_array_element _array_index) (`self.Bullet`)
    (`self.K2_SetActorLocation` _array_element (`SceneComponent.K2_GetComponentLocation` (`|GetArrayItem` (`self.ShootLocationArray`) _array_index)) false true)))

(event `Attack_2 (Keep)`
  ; 右键
)

(event `EnhancedInput|/Game/Input/IA_Attack_2`
  (params (ActionValue :type Boolean) (ElapsedSeconds :type "Float (double-precision)") (TriggeredSeconds :type "Float (double-precision)") (InputAction :type "InputAction Object Reference" :default "/Game/Input/IA_Attack_2.IA_Attack_2"))
  (bind _image_2 (`/Game/UI/W_PlayerScoreUI.Image_2` (`self.ScoreUI`)))
  ; 右键
  (:`Triggered`
    (`self.Attack_2 (Keep)`)
    (`self.StartShield`))
  (:`Started`
    (`self.Attack_2 (Once)`)
    (`/Game/UI/W_Tutorial.PressAndNext` (`/Game/UI/W_PlayerScoreUI.W_Tutorial` (`self.ScoreUI`)) "RMB")
    (set `self.UseShield?` true)
    (`Image.SetColorAndOpacity` _image_2 (struct :`R` 0.009511 :`B` 0.440972 :`A` 1.0)))
  (:`Canceled`
    (`self.Attack_2 (Completed` :!label _label_2)
    (set `self.UseShield?` false)
    (`Image.SetColorAndOpacity` _image_2 (struct :`R` 1.0 :`G` 1.0 :`B` 1.0 :`A` 1.0)))
  (:`Completed`
    (goto _label_2)))

(event `Attack_2 (Once)`
  ; 右键
  (`KismetSystemLibrary.PrintString` "Attack_2"))

(event `StartShield`
  (bind _returnvalue (+ (`self.K2_GetActorLocation`) (300.0 0.0 0.0)))
  (if (and (`self.UseShield?`) (not (<= (`self.Shield`) 0.0)))
    (bind _outactors (`KismetSystemLibrary.BoxOverlapActors` _returnvalue (300.0 500.0 500.0) (`|MakeArray` "ObjectTypeQuery3" "ObjectTypeQuery2" "ObjectTypeQuery4" "ObjectTypeQuery1" :!type "EObjectTypeQuery Enum") null (`|MakeArray` self :!type "Actor Object Reference")))
    (`KismetSystemLibrary.DrawDebugBox` _returnvalue (300.0 500.0 500.0) (struct) (struct) 1.0)
    (for _array_element _outactors
      (`GameplayStatics.ApplyDamage` _array_element 100.0))))

(event `PlayerTutorial`
  (if (not (`self.isStartToPlay`))
    (`/Game/UI/W_PlayerScoreUI.SubSystem` (`self.ScoreUI`) 0)))

(event `Attack_2 (Completed`
  ; 右键
)

(event `Space (Keep)`
  ; 空格
)

(event `Key|Q`
  (params (Key :type "Key Structure"))
  ; 切换视角
  (:`Pressed`
    (`/Engine/EditorBlueprintResources/StandardMacros.FlipFlop`
      (:`A`
        (`self.CheckIsFirstPersonCamera` false))
      (:`B`
        (`self.CheckIsFirstPersonCamera` true)))))

(event `EnhancedInput|/Game/Input/IA_KeySpace`
  (params (ActionValue :type Boolean) (ElapsedSeconds :type "Float (double-precision)") (TriggeredSeconds :type "Float (double-precision)") (InputAction :type "InputAction Object Reference" :default "/Game/Input/IA_KeySpace.IA_KeySpace"))
  ; 空格
  (:`Triggered`
    (`self.Space (Keep)`))
  (:`Started`
    (`self.Space (Once`))
  (:`Canceled`
    (`self.Space (Completed` :!label _label_3))
  (:`Completed`
    (goto _label_3)))

(event `Space (Once`
  ; 空格
  (`KismetSystemLibrary.PrintString` "Key Space"))

(event `CheckIsFirstPersonCamera`
  (params (`FIrstPerson?` :type Boolean))
  ; 切换视角
  (if `FIrstPerson?`
    ;; 第一人称
    (`ActorComponent.SetActive` (`self.Camera_FirstPerson`) true false)
    (`SceneComponent.SetVisibility` (`self.MotorcycleMesh_FirstPerson`) true false)
    (`SceneComponent.SetVisibility` (`self.SkeletalMesh`) true false)
    (`ActorComponent.SetActive` (`self.Camera`) false false)
    (`SceneComponent.SetVisibility` (`self.MotorcycleMesh`) false false)
    (`SceneComponent.SetVisibility` (`self.Cube`) false false)
    (else
      ;; 第三人称
      (`ActorComponent.SetActive` (`self.Camera_FirstPerson`) false false)
      (`SceneComponent.SetVisibility` (`self.MotorcycleMesh_FirstPerson`) false false)
      (`SceneComponent.SetVisibility` (`self.SkeletalMesh`) false false)
      (`ActorComponent.SetActive` (`self.Camera`) true false)
      (`SceneComponent.SetVisibility` (`self.MotorcycleMesh`) true false)
      (`SceneComponent.SetVisibility` (`self.Cube`) true false))))

(event `Space (Completed`
  ; 空格
)

(event `UseShield`
  (`KismetSystemLibrary.K2_SetTimerDelegate` (delegate `UseORCancelShield`) 0.1 true))

(event `UseORCancelShield`
  (bind _returnvalue (- (`self.Shield`) 2.0))
  (bind _returnvalue_2 (+ (`self.Shield`) 2.0))
  (if (`self.UseShield?`)
    (if (<= _returnvalue 0.0)
      (set `self.Shield` 0.0)
      (else
        (set `self.Shield` _returnvalue)))
    (elif (>= _returnvalue_2 (`self.MaxShield`))
      (set `self.Shield` (`self.MaxShield`))
      (else
        (set `self.Shield` _returnvalue_2)))))

(event `KeepAddSpeed`
  ; 移动
  ;; 向前
  (bind (_direction `_新建轨道_0`) (`Timeline|AddSpeed` :!label _label_4)
    (:`Update`
      (set `self.SpeedRate (*n)` `_新建轨道_0`)
      (`self.ConstantSpeed`))))

(event `EnhancedInput|/Game/Input/IA_Move`
  (params (ActionValue :type Boolean) (ElapsedSeconds :type "Float (double-precision)") (TriggeredSeconds :type "Float (double-precision)") (InputAction :type "InputAction Object Reference" :default "/Game/Input/IA_Move.IA_Move"))
  (bind _isconstantspeed_ (`self.isConstantSpeed?`))
  (bind _debugmod (`self.DebugMod`))
  ; 移动
  ;; 向前
  (:`Triggered`
    (if _isconstantspeed_
      _
      (elif _debugmod
        (goto _label_4))))
  (:`Completed`
    (if _isconstantspeed_
      _
      (elif _debugmod
        (goto _label_4 :!via `Reverse`)))))

(event `self.ReceiveTick`
  (params (DeltaSeconds :type "Float (single-precision)"))
  (bind _velocity_x (`KismetMathLibrary.BreakVector` (`MovementComponent.Velocity` (`self.CharacterMovement`))))
  ; Tick
  (`|ExecutionSequence`
    (:`then_0`
      ;; 检测是否为恒定速度模式？
      (if (`self.isConstantSpeed?`)
        (`self.KeepAddSpeed`)))
    (:`then_1`
      ;; 计算速度
      (`TextRenderComponent.K2_SetText` (`self.TextRender`) (`KismetTextLibrary.Conv_IntToText` (`KismetMathLibrary.Round` (* _velocity_x 0.036))))
      (`TextRenderComponent.K2_SetText` (`self.TextRender4`) (`KismetTextLibrary.Conv_IntToText` (`KismetMathLibrary.Round` (* _velocity_x 0.036)))))
    (:`then_2`
      (set `self.SmoothTurnValue` (* (`KismetMathLibrary.FInterpTo` (`self.SmoothTurnValue`) (`self.TurnValue`) DeltaSeconds 8.0) (/ (`KismetMathLibrary.FClamp` (`self.Speed`) 0.0 10000.0) 10000.0))))
    (:`then_3`
      ; 平滑镜头转向（转弯
      (if (`self.isStartToPlay`)
        (bind _output_get (set `self.CurrentRotation` (`KismetMathLibrary.FInterpTo` (`self.CurrentRotation`) (* 10.0 (`self.TurnValue`)) (`GameplayStatics.GetWorldDeltaSeconds`) 8.0)))
        (`SceneComponent.K2_SetRelativeRotation` (`self.Camera_FirstPerson`) (`KismetMathLibrary.MakeRotator` _output_get) false false)
        (else
          (set `self.CurrentRotation` 0.0))))
    (:`then_4`
      (`AudioParameterControllerInterface.SetFloatParameter` (`self.Audio`) "EngineState" (`self.Speed`))
      (bind _output_get_2 (set `self.CurrentSpeed` (`KismetMathLibrary.FClamp` (`KismetMathLibrary.FInterpTo` (`self.CurrentSpeed`) (`self.Speed`) (`GameplayStatics.GetWorldDeltaSeconds`) 10.0) 4000.0 20000.0)))
      (`AudioComponent.SetPitchMultiplier` (`self.Audio`) (/ _output_get_2 10000.0)))))

(event `EndConstantSpeed`
  ; 移动
  ;; 向前
  ;;; 防止结束恒定模式瞬间停车，在关闭恒定模式后，立刻进行此事件
  (goto _label_4 :!via `Reverse`))

(event `EnhancedInput|/Game/Input/IA_Turn`
  (params (ActionValue :type "Float (double-precision)") (ElapsedSeconds :type "Float (double-precision)") (TriggeredSeconds :type "Float (double-precision)") (InputAction :type "InputAction Object Reference" :default "/Game/Input/IA_Turn.IA_Turn"))
  (bind _w_tutorial (`/Game/UI/W_PlayerScoreUI.W_Tutorial` (`self.ScoreUI`)))
  ; 移动
  ;; 转弯
  (:`Triggered`
    (`|ExecutionSequence`
      (:`then_0`
        (if (`self.isStartToPlay`)
          (set `self.TurnValue` ActionValue)
          (`self.K2_AddActorWorldOffset` (* (* (* (* (* (* (`KismetMathLibrary.GetRightVector` (`SceneComponent.K2_GetComponentRotation` (`self.CapsuleComponent`))) ActionValue) (`self.SmoothTurnValue`)) 8000.0) (`GameplayStatics.GetWorldDeltaSeconds`)) ActionValue) (`self.SpeedRate (*n)`)) true)))
      (:`then_1`
        (if (< ActionValue 0.0)
          (`/Game/UI/W_Tutorial.PressAndNext` _w_tutorial "A")
          (elif (> ActionValue 0.0)
            (`/Game/UI/W_Tutorial.PressAndNext` _w_tutorial "D"))))))
  (:`Completed`
    (set `self.TurnValue` 0.0)))

(event `self.Box1.OnComponentBeginOverlap`
  (params (OverlappedComponent :type "PrimitiveComponent Object Reference") (OtherActor :type "Actor Object Reference") (OtherComp :type "PrimitiveComponent Object Reference") (OtherBodyIndex :type Integer) (bFromSweep :type Boolean) (SweepResult :type "HitResult Structure (by ref)"))
  ; 当地人碰到玩家前面的碰撞盒子，告知敌人开始行动
  (message `/Game/Blueprint/Enemy/BPI_CallItemState.callEnemyStartMovement` OtherActor))

(event `EnhancedInput|/Game/Input/IA_SpeedUp`
  (params (ActionValue :type Boolean) (ElapsedSeconds :type "Float (double-precision)") (TriggeredSeconds :type "Float (double-precision)") (InputAction :type "InputAction Object Reference" :default "/Game/Input/IA_SpeedUp.IA_SpeedUp"))
  ; 移动
  ;; 加速
  (:`Triggered`
    (if (`self.isStartToPlay`)
      (bind (_direction `_新建轨道_0`) (`Timeline|SpeedUp` :!label _label_5)
        (:`Update`
          (set `self.SpeedUpRate (*n)` (`KismetMathLibrary.FClamp` (* `_新建轨道_0` 1.2) 1.0 1.5))
          (`CameraComponent.SetFieldOfView` (`self.Camera`) (`KismetMathLibrary.Lerp` 100.0 140.0 `_新建轨道_0`))
          (`CameraComponent.SetFieldOfView` (`self.Camera_FirstPerson`) (`KismetMathLibrary.Lerp` 120.0 135.0 `_新建轨道_0`))))
      (else
        (goto _label_5 :!via `Reverse`))))
  (:`Started`
    (`PlayerController.ClientStartCameraShake` :`self` (`GameplayStatics.GetPlayerController` 0) :`Shake` "/Game/Blueprint/Player/CameraShake/BP_SpeedUpCameraShake.BP_SpeedUpCameraShake_C")
    (`/Game/UI/W_Tutorial.PressAndNext` (`/Game/UI/W_PlayerScoreUI.W_Tutorial` (`self.ScoreUI`)) "Shift")
    (`GameplayStatics.PlaySound2D` "/Game/Art/Voice/freesound_community-nitro-activation-48077.freesound_community-nitro-activation-48077" 1.0 1.0 0.0 null null)
    (`AudioComponent.Play` (`self.BootsSound`) 0.0))
  (:`Completed`
    (`AudioComponent.Stop` (`self.BootsSound`))
    (goto _label_5 :!via `Reverse`)))

(event `EndCaculate`
  (`Widget.SetVisibility` (`/Game/UI/W_PlayerScoreUI.W_BossDistination` (`self.ScoreUI`)) "Hidden")
  (`KismetSystemLibrary.K2_PauseTimerHandle` (stale `StartToCaculateDistination` _returnvalue)))

(event `ConstantSpeed`
  ; 恒定速度模式：现版本为，当进入恒定模式，会自动加速到最大速度（非加速），但是当按住刹车，就会降低至行驶最低速度，若松开刹车，则会继续行驶到最高速度
  (bind _output_get (set `self.Speed` (* (* (* (`self.SpeedRate (*n)`) (`self.BaseSpeed`)) (`self.SpeedUpRate (*n)`)) (`self.BrakeRate (*n)`))))
  (set `CharacterMovementComponent.MaxWalkSpeed` _output_get (`self.CharacterMovement`))
  (`self.AddMovementInput` (`SceneComponent.GetForwardVector` (`self.CapsuleComponent`))))

(event `StartToCaculateDistination`
  (params (whichBoss :type "Actor Object Reference"))
  (`Widget.SetVisibility` (`/Game/UI/W_PlayerScoreUI.W_BossDistination` (`self.ScoreUI`)) "Visible")
  (bind _returnvalue (`KismetSystemLibrary.K2_SetTimerDelegate` (delegate `UpdateDistination`) 0.1 true)))

(event `UpdateDistination`
  (set `Slider.Value` (- 1.0 (/ (`KismetMathLibrary.Vector_Distance` (`self.K2_GetActorLocation`) (`self.K2_GetActorLocation` (stale `StartToCaculateDistination` whichBoss))) 20000.0)) (`/Game/UI/W_BossDistination.Slider_39` (`/Game/UI/W_PlayerScoreUI.W_BossDistination` (`self.ScoreUI`)))))

(event `EnhancedInput|/Game/Input/IA_Break`
  (params (ActionValue :type Boolean) (ElapsedSeconds :type "Float (double-precision)") (TriggeredSeconds :type "Float (double-precision)") (InputAction :type "InputAction Object Reference" :default "/Game/Input/IA_Break.IA_Break"))
  (bind _rectlight (`self.RectLight`))
  ; 移动
  ;; 刹车（进入恒定模式的刹车比较特殊，需要单独说明
  (:`Triggered`
    (if (`self.isConstantSpeed?`)
      ;;; 当车进入恒定模式，为防止按住时进入PlayerFromStart时一直维持开头一针使用Do Once，直到松开按钮
      (`/Engine/EditorBlueprintResources/StandardMacros.DoOnce` false :!label _label_6
        (:`Completed`
          (bind (_direction `_新建轨道_0`) (`Timeline|Break` :!via `PlayFromStart` :!label _label_7)
            (:`Update`
              (if (`self.isConstantSpeed?`)
                ;;; 减速速率
                (set `self.BrakeRate (*n)` (`KismetMathLibrary.FClamp` `_新建轨道_0` 0.5))
                (else
                  (set `self.BrakeRate (*n)` `_新建轨道_0`)))))))
      (else
        (goto _label_7))))
  (:`Started`
    (set `self.isBraking` true)
    (`SceneComponent.SetVisibility` _rectlight true false))
  (:`Completed`
    (set `self.isBraking` false)
    (`SceneComponent.SetVisibility` _rectlight false false)
    (`|ExecutionSequence`
      (:`then_0`
        (goto _label_7 :!via `Reverse`))
      (:`then_1`
        (goto _label_6 :!via `Reset`))
      (:`then_2`
        (`/Game/UI/W_Tutorial.PressAndNext` (`/Game/UI/W_PlayerScoreUI.W_Tutorial` (`self.ScoreUI`)) "S")))))

(event `Key|E`
  (params (Key :type "Key Structure"))
  ; 切换恒定速度模式？
  (:`Pressed`
    (`|ExecutionSequence`
      (:`then_0`
        ;; 未经允许，不能控制启动或暂停
        (if (`self.isStartToPlay`)
          (`|ExecutionSequence`
            (:`then_0`
              (if (`self.isConstantSpeed?`)
                _))
            (:`then_1`
              (`/Engine/EditorBlueprintResources/StandardMacros.DoOnce` false :!label _label_8
                (:`Completed`
                  (`self.isStart`)
                  (set `self.isConstantSpeed?` true)
                  (`TextRenderComponent.K2_SetText` (`self.TextRender3`) (`KismetTextLibrary.Conv_StringToText` "On"))
                  (`TextRenderComponent.K2_SetText` (`self.TextRender6`) (`KismetTextLibrary.Conv_StringToText` "On"))))))))
      (:`then_1`
        (`/Game/UI/W_Tutorial.PressAndNext` (`/Game/UI/W_PlayerScoreUI.W_Tutorial` (`self.ScoreUI`)) "E")))))

(event `ReadyToStart`
  ; 切换恒定速度模式？
  (`|ExecutionSequence`
    (:`then_0`
      (goto _label_8 :!via `Reset`))
    (:`then_1`
      (set `self.isConstantSpeed?` false)
      (`self.EndConstantSpeed`)
      (`TextRenderComponent.K2_SetText` (`self.TextRender3`) (`KismetTextLibrary.Conv_StringToText` "Off"))
      (`TextRenderComponent.K2_SetText` (`self.TextRender6`) (`KismetTextLibrary.Conv_StringToText` "Off")))))

(event `self.Box.OnComponentBeginOverlap`
  (params (OverlappedComponent :type "PrimitiveComponent Object Reference") (OtherActor :type "Actor Object Reference") (OtherComp :type "PrimitiveComponent Object Reference") (OtherBodyIndex :type Integer) (bFromSweep :type Boolean) (SweepResult :type "HitResult Structure (by ref)"))
  ;[0.5816 0.4526 0 0.5] 回收场景的物品（重要！！
  (if (`self.ActorHasTag` OtherActor "Spawn")
    (`self.GetSpawnItemAndMoveToStandbyArea` OtherActor (`self.ActorHasTag` OtherActor "Boss"))))

(event `/Game/Blueprint/Player/PlayerScoreSystem/BPI_PlayerGetScore.PlayerBoost`
  ; 弹射（一般在跳台用的上）
  (`self.LaunchCharacter` (* (+ (`SceneComponent.GetForwardVector` (`self.CapsuleComponent`)) (0.0 0.0 2.0)) 3000.0)))

(event `self.ReceiveAnyDamage`
  (params (Damage :type "Float (single-precision)") (DamageType :type "DamageType Object Reference") (InstigatedBy :type "Controller Object Reference") (DamageCauser :type "Actor Object Reference"))
  (bind _returnvalue (- (`self.Health`) Damage))
  ; 受到伤害
  (`|ExecutionSequence`
    (:`then_0`
      (`KismetSystemLibrary.PrintString` (`KismetStringLibrary.Conv_DoubleToString` _returnvalue))
      (if (<= _returnvalue 0.0)
        (set `self.Health` 0.0)
        (`self.PlayerIsDie`)
        (else
          (set `self.Health` _returnvalue))))
    (:`then_1`
      ;; 死亡后，镜头不允许晃动
      (`/Engine/EditorBlueprintResources/StandardMacros.Gate` false :!label _label_9
        (:`Exit`
          (`PlayerController.ClientStartCameraShake` :`self` (`GameplayStatics.GetPlayerController` 0) :`Shake` "/Game/Blueprint/Player/CameraShake/BP_GetHurtCameraShake.BP_GetHurtCameraShake_C"))))))

(event `/Game/Blueprint/Player/PlayerScoreSystem/BPI_PlayerGetScore.PlayerGetScore`
  (params (whichBehavior :type "/Game/Blueprint/Player/PlayerScoreSystem/E_WhichScoreBehavior Enum" :default "NewEnumerator0") (howToAdd :type Text) (howManyScore :type "Float (double-precision)"))
  (bind _slatecolor (make `SlateColor` (struct :`G` 1.0 :`B` 0.023136 :`A` 1.0)))
  (bind _scoreui (`self.ScoreUI`))
  (bind _scoreui_2 (`self.ScoreUI`))
  ; 分数相关
  ;; 技术得分（暂时包括擦肩而过，杀敌
  (switch `/Game/Blueprint/Player/PlayerScoreSystem/E_WhichScoreBehavior` whichBehavior
    (:`NewEnumerator0`
      (`/Game/UI/W_PlayerScoreUI.ScoreInfor` _scoreui howToAdd _slatecolor)
      (`UserWidget.PlayAnimation` _scoreui_2 (`/Game/UI/W_PlayerScoreUI.AddScore` _scoreui_2) 0.0 1 "Forward" 1.0 false :!label _label_10)
      (`self.AddScore` howManyScore))
    (:`NewEnumerator1`
      (if (>= (/ (`self.Speed`) (`self.BaseSpeed`)) 0.5)
        (`/Game/UI/W_PlayerScoreUI.ScoreInfor` _scoreui howToAdd _slatecolor)
        (goto _label_10)))
    (:`NewEnumerator2`
      (`/Game/UI/W_PlayerScoreUI.ScoreInfor` _scoreui howToAdd (make `SlateColor` (struct :`R` 1.0 :`A` 1.0)))
      (`GameplayStatics.PlaySound2D` "/Game/Art/Voice/universfield-error-010-206498.universfield-error-010-206498" 1.0 1.0 0.0 null null))))

(event `CloseBecousePlayerIsDie`
  ; 受到伤害
  ;; 死亡后，镜头不允许晃动
  (goto _label_9 :!via `Close`))

(event `/Game/Blueprint/Player/PlayerScoreSystem/BPI_PlayerGetScore.GameIsOver/Start`
  (params (`Over?` :type Boolean))
  ; 分数相关
  (if `Over?`
    (set `self.isAction` false)
    (else
      (set `self.isAction` true))))

(event `AddScore`
  (params (Score :type "Float (double-precision)"))
  ; 分数相关
  ;; 加分系统（游戏结束时不允许加分
  (set `self.Score` (+ Score (`self.Score`))))

(event `Key|Escape`
  (params (Key :type "Key Structure"))
  (bind _stopui (`self.StopUI`))
  ; 暂停UI
  (:`Pressed`
    (`/Engine/EditorBlueprintResources/StandardMacros.IsValid` (`self.StopUI`) :!label _label_11
      (:`Is Valid`
        _)
      (:`Is Not Valid`
        (bind _returnvalue (`|CreateWidget` "/Game/UI/W_StopUI.W_StopUI_C"))
        (bind _output_get (set `self.StopUI` _returnvalue))
        (`UserWidget.AddToViewport` _output_get 0)))
    (if (`/Game/UI/W_StopUI.isStoping?` _stopui)
      (`/Game/UI/W_StopUI.ControlStopUI` _stopui false)
      (else
        (`/Game/UI/W_StopUI.ControlStopUI` _stopui true)))))

(event `CheckMovingAddScore`
  ; 分数相关
  ;; 开始游戏时，根据速度持续加分
  (`KismetSystemLibrary.K2_SetTimerDelegate` (delegate `MovingAddScore`) 0.1 true))

(event `Key|P`
  (params (Key :type "Key Structure"))
  ; 暂停UI
  (:`Pressed`
    (goto _label_11)))

(event `MovingAddScore`
  (bind _velocity_x (`KismetMathLibrary.BreakVector` (`MovementComponent.Velocity` (`self.CharacterMovement`))))
  ; 分数相关
  ;; 开始游戏时，根据速度持续加分
  (if (`self.isAction`)
    (`self.AddScore` (/ _velocity_x 100.0))))

(event `PlayerIsDie`
  (bind _scoreui (`self.ScoreUI`))
  ; 玩家死亡逻辑
  (`/Engine/EditorBlueprintResources/StandardMacros.DoOnce` false
    (:`Completed`
      (`self.CloseBecousePlayerIsDie`)
      (set `self.isStartToPlay` false)
      (`self.CheckIsFirstPersonCamera` true)
      (`SceneComponent.K2_AttachToComponent` (`self.Camera_FirstPerson`) (`self.SkeletalMesh1`) "head" "KeepWorld" "KeepWorld" "KeepRelative" true)
      (`SkeletalMeshComponent.PlayAnimation` (`self.SkeletalMesh`) "/Game/Art/Animation/Moto/Motor_Die_Anim_5.Motor_Die_Anim_5" false)
      (`|PlayMontage` (`self.SkeletalMesh1`) "/Game/Art/Animation/Character/Character_Die_Anim_2_Montage.Character_Die_Anim_2_Montage"
        (:`OnNotifyBegin`
          (set `TextBlock.Text` (`KismetTextLibrary.Conv_DoubleToText` (`self.Score`) "HalfToEven") (`/Game/UI/W_Die.TextBlock_262` (`/Game/UI/W_PlayerScoreUI.W_Die` _scoreui)))
          (`/Game/UI/W_PlayerScoreUI.ShowDieUI` _scoreui)
          (`AudioComponent.Stop` (`self.Audio`))
          (`GameplayStatics.SetGlobalTimeDilation` 0.0))))))

(event `AskNeedFix?`
  (bind _returnvalue (`GameplayStatics.GetPlayerController` 0))
  (bind _w_fixcar (`/Game/UI/W_PlayerScoreUI.W_FixCar` (`self.ScoreUI`)))
  (bind _button_1 (`/Game/UI/W_FixCar.Button_1` _w_fixcar))
  ; 是否需要修理（UI）
  (set `PlayerController.bShowMouseCursor` true _returnvalue)
  (`WidgetBlueprintLibrary.SetInputMode_GameAndUIEx` _returnvalue null)
  (`Widget.SetVisibility` _w_fixcar "Visible")
  (if (`self.canEscape?`)
    (`Widget.SetVisibility` _button_1 "Visible")
    (else
      (`Widget.SetVisibility` _button_1 "Hidden"))))

(event `PlayBossAnim`
  (bind (_returnvalue_x _returnvalue_y _returnvalue_z) (`KismetMathLibrary.BreakVector` (`self.K2_GetActorLocation`)))
  (`self.K2_SetActorLocation` (`KismetMathLibrary.MakeVector` _returnvalue_x 0.0 _returnvalue_z))
  (`|PlayMontage` (`self.SkeletalMesh1`) "/Game/Art/Animation/Character/Character_P_Anim_Montage.Character_P_Anim_Montage"
    (:`then`
      (`|PlayMontage` (`self.SkeletalMesh`) "/Game/Art/Animation/Moto/Motor_P_Anim_Montage.Motor_P_Anim_Montage"
        (:`then`
          (`PlayerController.ClientStartCameraShake` :`self` (`GameplayStatics.GetPlayerController` 0) :`Shake` "/Game/Blueprint/Player/CameraShake/BP_BossShake.BP_BossShake_C"))))))

(event `AddHealth`
  (params (Health :type "Float (double-precision)"))
  (bind _returnvalue (+ (`self.Health`) Health))
  (if (>= _returnvalue (`self.MaxHealth`))
    (set `self.Health` (`self.MaxHealth`))
    (else
      (set `self.Health` _returnvalue))))

(fn `SimpleShootSystem`
  (params (whichItemLocation :type "Vector Structure"))
  (bind _outhit (`KismetSystemLibrary.LineTraceSingle` whichItemLocation (+ whichItemLocation (* (`SceneComponent.GetForwardVector` (`self.Sphere`)) 100000.0)) "TraceTypeQuery1"))
  (`GameplayStatics.ApplyDamage` (`.HitActor` (`GameplayStatics.BreakHitResult` _outhit)) 30.0))

(fn `UserConstructionScript`)