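; Child motorcycle character that changes its startup behavior depending on the current level.
; BeginPlay compares the level name and runs the parent's BeginPlay only in TestMap.
; In L_Equipment it instead zeroes movement gravity and disables actor tick, leaving the character inert; any other level skips both paths.
; The construction script only calls the parent's.
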(event `self.ReceiveBeginPlay`
  (bind _returnvalue (`GameplayStatics.GetCurrentLevelName` true))
  (if (`KismetStringLibrary.EqualEqual_StrStr` _returnvalue "TestMap")
    (`parent.ReceiveBeginPlay`)
    (elif (`KismetStringLibrary.EqualEqual_StrStr` _returnvalue "L_Equipment")
      (set `CharacterMovementComponent.GravityScale` 0.0 (`self.CharacterMovement`))
      (`self.SetActorTickEnabled` false))))

(fn `UserConstructionScript`
  (`parent.UserConstructionScript`))