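; Moving repair truck that the motorcycle player can ride into, driving forward on Tick at the player's clamped speed, or fixed speed during boarding.
; StartCar opens the door and switches lights; entering Box locks and attaches the player, slides them inside by timeline, and asks about repair on montage notify.
; Box3 awards a skip-repair bonus unless Box2 consumes their shared DoOnce first.
; A looping timeline spins Sphere, and a screen widget receives the player.
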(event `self.ReceiveBeginPlay`
  (`|ExecutionSequence`
    (:`then_0`
      (bind _asbp_motorcycle_character (cast `/Game/Blueprint/Player/BP_MotorcycleCharacter` (`GameplayStatics.GetPlayerPawn` 0)))
      (set `self.Player` _asbp_motorcycle_character)
      (`self.ResetCarDoor`)
      (`SceneComponent.SetVisibility` (`self.SpotLight`) false false)
      (`SceneComponent.SetVisibility` (`self.SpotLight1`) false false)
      (`self.LightRotating`))
    (:`then_1`
      (bind _returnvalue (`|CreateWidget` "/Game/UI/W_BCScreen.W_BCScreen_C"))
      (set `/Game/UI/W_BCScreen.Player` (`self.Player`) _returnvalue)
      (bind _output_get (set `self.BCScreen` _returnvalue))
      (`WidgetComponent.SetWidget` (`self.Widget4`) _output_get))))

(event `LightRotating`
  (bind _sphere (`self.Sphere`))
  (bind (_returnvalue_roll _returnvalue_pitch _returnvalue_yaw) (`KismetMathLibrary.BreakRotator` (`SceneComponent.K2_GetComponentRotation` _sphere)))
  (bind (_direction `_新建轨道_0`) (`Timeline|时间轴_0` :!via `PlayFromStart`)
    (:`Update`
      (`SceneComponent.K2_SetWorldRotation` _sphere (`KismetMathLibrary.MakeRotator` (+ 0.0 (* `_新建轨道_0` 360.0)) _returnvalue_pitch _returnvalue_yaw) false false))
    (:`Finished`
      (`self.LightRotating`))))

(event `PlayerInCarAnim`
  (`|ExecutionSequence`
    (:`then_0`
      (`|PlayMontage` (`self.kache_1`) "/Game/Art/Animation/Truck/Truck_Ainm_CloseDoor_Wait_Montage.Truck_Ainm_CloseDoor_Wait_Montage"
        (:`OnNotifyBegin`
          (`/Game/Blueprint/Player/BP_MotorcycleCharacter.AskNeedFix?` (`self.Player`)))))
    (:`then_1`
      (`SceneComponent.K2_SetWorldLocation` (`self.MotoLocation`) (`SceneComponent.K2_GetComponentLocation` (`self.Sphere2`)) false false)
      (bind (_direction `_新建轨道_0`) (`Timeline|时间轴` :!via `PlayFromStart`)
        (:`Update`
          (`SceneComponent.K2_SetWorldLocation` (`self.MotoLocation`) (`KismetMathLibrary.VLerp` (`SceneComponent.K2_GetComponentLocation` (`self.Sphere2`)) (`SceneComponent.K2_GetComponentLocation` (`self.Sphere1`)) `_新建轨道_0`) false false))))))

(event `self.ReceiveTick`
  (params (DeltaSeconds :type "Float (single-precision)"))
  ; 简单向前移动（速度控制在90码以下）
  (if (`self.isAction`)
    (if (`self.isInAnim`)
      (`self.K2_AddActorWorldOffset` (* (* (`KismetMathLibrary.Vector_Forward`) 5000.0) DeltaSeconds))
      (else
        (`self.K2_AddActorWorldOffset` (* (* (`KismetMathLibrary.Vector_Forward`) (`KismetMathLibrary.FClamp` (`/Game/Blueprint/Player/BP_MotorcycleCharacter.Speed` (`self.Player`)) 0.0 5000.0)) DeltaSeconds))))))

(event `self.Box.OnComponentBeginOverlap`
  (params (OverlappedComponent :type "PrimitiveComponent Object Reference") (OtherActor :type "Actor Object Reference") (OtherComp :type "PrimitiveComponent Object Reference") (OtherBodyIndex :type Integer) (bFromSweep :type Boolean) (SweepResult :type "HitResult Structure (by ref)"))
  (bind _player (`self.Player`))
  (bind _player_2 (`self.Player`))
  (if (== OtherComp (`Character.CapsuleComponent` (`self.Player`)))
    (`KismetSystemLibrary.PrintString` "InInIn" true true (struct :`R` 1.0 :`B` 0.073701 :`A` 1.0))
    (`/Engine/EditorBlueprintResources/StandardMacros.DoOnce` false :!label _label
      (:`Completed`
        (set `self.isInAnim` true)
        (set `/Game/Blueprint/Player/BP_MotorcycleCharacter.isConstantSpeed?` false _player_2)
        (set `/Game/Blueprint/Player/BP_MotorcycleCharacter.isStartToPlay` false _player_2)
        (set `/Game/Blueprint/Player/BP_MotorcycleCharacter.isInVehicle` true _player_2)
        (`CharacterMovementComponent.SetMovementMode` (`Character.CharacterMovement` _player_2) "MOVE_None" 0)
        (`/Game/Blueprint/Player/BP_MotorcycleCharacter.EndConstantSpeed` _player_2)
        (`/Game/Blueprint/Player/BP_MotorcycleCharacter.CheckIsFirstPersonCamera` _player_2 true)
        (`self.K2_SetActorLocation` _player (`SceneComponent.K2_GetComponentLocation` (`self.MotoLocation`)) false false)
        (`self.K2_SetActorRotation` :`self` _player)
        (`self.K2_AttachToComponent` (`self.Player`) (`self.MotoLocation`) "None" "KeepWorld" "KeepWorld" "KeepWorld" true)
        (`self.PlayerInCarAnim`)
        (`SceneComponent.SetVisibility` (`self.SpotLight`) false false)
        (`SceneComponent.SetVisibility` (`self.SpotLight1`) false false)))))

(event `ResetCarDoor`
  (goto _label :!via `Reset`))

(event `StartCar`
  (`|PlayMontage` (`self.kache_1`) "/Game/Art/Animation/Truck/Truck_Ainm_OpenFrontDoor_Montage.Truck_Ainm_OpenFrontDoor_Montage" 0.5
    (:`then`
      (`SceneComponent.SetVisibility` (`self.RectLight`) false false)
      (`SceneComponent.SetVisibility` (`self.SpotLight`) true false)
      (`SceneComponent.SetVisibility` (`self.SpotLight1`) true false))))

(event `self.Box3.OnComponentBeginOverlap`
  (params (OverlappedComponent :type "PrimitiveComponent Object Reference") (OtherActor :type "Actor Object Reference") (OtherComp :type "PrimitiveComponent Object Reference") (OtherBodyIndex :type Integer) (bFromSweep :type Boolean) (SweepResult :type "HitResult Structure (by ref)"))
  ; 不修车的技术得分
  (if (== OtherComp (`Character.CapsuleComponent` (`self.Player`)))
    (`/Engine/EditorBlueprintResources/StandardMacros.DoOnce` false :!label _label_2
      (:`Completed`
        (message `/Game/Blueprint/Player/PlayerScoreSystem/BPI_PlayerGetScore.PlayerGetScore` (`self.Player`) "NewEnumerator0" "很酷，不修车，奖励你5000分！" 5000.0)))))

(event `self.Box2.OnComponentBeginOverlap`
  (params (OverlappedComponent :type "PrimitiveComponent Object Reference") (OtherActor :type "Actor Object Reference") (OtherComp :type "PrimitiveComponent Object Reference") (OtherBodyIndex :type Integer) (bFromSweep :type Boolean) (SweepResult :type "HitResult Structure (by ref)"))
  ; 不修车的技术得分
  (if (== OtherComp (`Character.CapsuleComponent` (`self.Player`)))
    (goto _label_2)))

(event `ResetPlayerGetScore`
  ; 不修车的技术得分
  (goto _label_2 :!via `Reset`))

(fn `UserConstructionScript`)